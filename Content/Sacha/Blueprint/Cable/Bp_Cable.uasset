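; Cable actor that tethers four cable components to the skeletal mesh of a referenced NPC (PNJ1Ref).
; On BeginPlay it pairs a cable array with a socket-name array, creates dynamic materials, and attaches cable ends to both wrists and, for two cables, the root bone.
; A PlaySound event plays a given sound on its audio component, and InteractBetweenItem stops it.
; Tick is empty, and distance-based tiling and an alternative target setup are left unconnected.
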(event `self.ReceiveTick`
  (params (DeltaSeconds :type "Float (single-precision)")))

(event `self.ReceiveBeginPlay`
  (`KismetArrayLibrary.Array_Set` (`self.CableArray`) 0 (`self.Cable`) true)
  (`KismetArrayLibrary.Array_Set` (`self.CableArray`) 1 (`self.Cable1`) true)
  (`KismetArrayLibrary.Array_Set` (`self.CableArray`) 2 (`self.Cable2`) true)
  (`KismetArrayLibrary.Array_Set` (`self.CableArray`) 3 (`self.Cable3`) true)
  (`KismetArrayLibrary.Array_Set` (`self.Socket Name`) 0 "PoignetGauche" true)
  (`KismetArrayLibrary.Array_Set` (`self.Socket Name`) 1 "PoignetDroit" true)
  (`KismetArrayLibrary.Array_Set` (`self.Socket Name`) 2 "RL_BoneRoot" true)
  (`KismetArrayLibrary.Array_Set` (`self.Socket Name`) 3 "RL_BoneRoot" true)
  (for (_array_element _array_index) (`self.CableArray`)
    (`PrimitiveComponent.CreateDynamicMaterialInstance` _array_element _array_index (`PrimitiveComponent.GetMaterial` _array_element 0) "None"))
  (for (_array_element_2 _array_index_2) (`self.Socket Name`)
    (`CableComponent.SetAttachEndToComponent` (`|GetArrayItem` (`self.CableArray`) _array_index_2) (`/Game/Sacha/Blueprint/PNJ/BP_PNJ1.SkeletalMesh` (`self.PNJ1_Ref`)) _array_element_2)))

(event `/Game/Sacha/Interface/BPI_Interact.PlaySound`
  (params (SoundToPlay :type "SoundBase Object Reference") (StartTime :type "Float (double-precision)"))
  (bind _audio (`self.audio`))
  (`AudioComponent.SetSound` _audio SoundToPlay)
  (`AudioComponent.Play` _audio 0.0))

(event `/Game/Sacha/Interface/BPI_Interact.InteractBetweenItem`
  (`AudioComponent.Stop` (`self.audio`)))

(fn `UserConstructionScript`)