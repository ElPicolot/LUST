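; BP_StartSequense is a trigger actor that plays a level sequence once while locking player input.
; The first overlap with its Box passes a DoOnce, then casts to BP_FirstPersonCharacterSacha, so any other overlapping actor also uses up the trigger.
; For that character, it disables input, plays LevelSequenseActor's sequence, and re-enables input after a Delay derived from the sequence's end time.
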(event `self.Box.OnComponentBeginOverlap`
  (params (OverlappedComponent :type "PrimitiveComponent Object Reference") (OtherActor :type "Actor Object Reference") (OtherComp :type "PrimitiveComponent Object Reference") (OtherBodyIndex :type Integer) (bFromSweep :type Boolean) (SweepResult :type "HitResult Structure (by ref)"))
  (bind _levelsequenseactor (`self.LevelSequenseActor`))
  (`/Engine/EditorBlueprintResources/StandardMacros.DoOnce` false
    (:`Completed`
      (bind _asbp_first_person_character_sacha (cast `/Game/Sacha/Blueprint/BP_FirstPersonCharacterSacha` OtherActor))
      (`self.DisableInput` _asbp_first_person_character_sacha (`GameplayStatics.GetPlayerController` 0))
      (`MovieSceneSequencePlayer.Play` (`LevelSequenceActor.SequencePlayer` _levelsequenseactor))
      (`KismetSystemLibrary.Delay` (`TimeManagementBlueprintLibrary.Conv_QualifiedFrameTimeToSeconds` (`MovieSceneSequencePlayer.GetEndTime` (`LevelSequenceActor.SequencePlayer` _levelsequenseactor))))
      (`self.EnableInput` _asbp_first_person_character_sacha (`GameplayStatics.GetPlayerController` 0)))))

(fn `UserConstructionScript`)