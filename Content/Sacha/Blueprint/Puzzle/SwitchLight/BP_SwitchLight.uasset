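; BP_SwitchLight is a puzzle trigger that flickers a point light and reveals Picto planes while the light is off.
; The first box overlap by BP_FirstPersonCharacterSacha starts a looping timer whose FlipFlop alternates light intensity and plane visibility.
; A counter, incremented per Picto on each lit phase, clears the timer at TimeRepeat.
; SetTimer is an uncalled random-interval test; Tick debug-prints its Time value.
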(event `self.ReceiveTick`
  (params (DeltaSeconds :type "Float (single-precision)"))
  (`KismetSystemLibrary.PrintString` (`KismetStringLibrary.Conv_DoubleToString` (`self.Time`))))

(event `self.Box.OnComponentBeginOverlap`
  (params (OverlappedComponent :type "PrimitiveComponent Object Reference") (OtherActor :type "Actor Object Reference") (OtherComp :type "PrimitiveComponent Object Reference") (OtherBodyIndex :type Integer) (bFromSweep :type Boolean) (SweepResult :type "HitResult Structure (by ref)"))
  (cast `/Game/Sacha/Blueprint/BP_FirstPersonCharacterSacha` OtherActor)
  (`/Engine/EditorBlueprintResources/StandardMacros.DoOnce` false
    (:`Completed`
      (bind _returnvalue (`KismetSystemLibrary.K2_SetTimerDelegate` (delegate `SwitchLight`) 0.3 true))
      (set `self.LightHandle` _returnvalue))))

(event `SwitchLight`
  (`/Engine/EditorBlueprintResources/StandardMacros.FlipFlop`
    (:`A`
      (`LightComponent.SetIntensity` (`self.PointLight`) 1000.0)
      (for _array_element (`self.Picto`)
        (`SceneComponent.SetVisibility` (`/Game/Sacha/Blueprint/Puzzle/BP_Picto.Plane` _array_element) false false)
        (`/Engine/EditorBlueprintResources/StandardMacros.IncrementInt` (`self.CounterTimer`)
          (:`  `
            (if (>= (`self.CounterTimer`) (`self.TimeRepeat`))
              (`KismetSystemLibrary.K2_ClearAndInvalidateTimerHandle` (`self.LightHandle`)))))))
    (:`B`
      (`LightComponent.SetIntensity` (`self.PointLight`) 0.0)
      (for _array_element_2 (`self.Picto`)
        (`SceneComponent.SetVisibility` (`/Game/Sacha/Blueprint/Puzzle/BP_Picto.Plane` _array_element_2) true false)))))

(event `SetTimer`
  ;[1 1 1] test modiif time
  (if (not (< (`self.MinTime`) 0.0))
    (set `self.MinTime` (- (`self.MinTime`) 0.01)))
  (set `self.MaxTime` (- (`self.MaxTime`) 0.01))
  (set `self.Time` (`KismetMathLibrary.RandomFloatInRange` (`self.MinTime`) (`self.MaxTime`))))

(fn `UserConstructionScript`)