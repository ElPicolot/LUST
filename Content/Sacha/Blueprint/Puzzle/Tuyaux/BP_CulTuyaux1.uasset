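; BP_CulTuyaux1 is an interactable pipe-puzzle piece that rotates one group of pipes when used.
; On InteractWorking it stores the player reference, then its CulNumber selects the R, Y or B rotate event on BPTuyauAll.
; A FlipFlop then alternates SpawnScarfDecal between the relative locations of TargetObject1 and TargetObject2.
; A leftover branch that sets CanInteractWith maps is not wired to any event.
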(event `self.Interact Working`
  (params (ItemInHand :type "/Game/Sacha/Blueprint/Items/E_MainItemType Enum" :default "NewEnumerator0") (ItemInHandforAnim :type "/Game/Sacha/Blueprint/Items/BP_Item Object Reference") (PlayrRef :type "/Game/Sacha/Blueprint/BP_FirstPersonCharacterSacha Object Reference"))
  (bind _bptuyauall (`self.BPTuyauAll`))
  (set `self.Playr Ref_0` PlayrRef)
  (switch `int` (`self.CulNumber`)
    (:`1`
      (`/Game/Sacha/Blueprint/Puzzle/Tuyaux/BP_AllTuyaux.EventRotateTuyauxR` _bptuyauall))
    (:`2`
      (`/Game/Sacha/Blueprint/Puzzle/Tuyaux/BP_AllTuyaux.EventRotateTuyauxY` _bptuyauall))
    (:`3`
      (`/Game/Sacha/Blueprint/Puzzle/Tuyaux/BP_AllTuyaux.EventRotateTuyauxB` _bptuyauall)))
  (`/Engine/EditorBlueprintResources/StandardMacros.FlipFlop`
    (:`A`
      (`self.SpawnScarfDecal` false (`SceneComponent.RelativeLocation` (`self.TargetObject1`))))
    (:`B`
      (`self.SpawnScarfDecal` false (`SceneComponent.RelativeLocation` (`self.TargetObject2`))))))

(fn `UserConstructionScript`
  (`parent.UserConstructionScript`))