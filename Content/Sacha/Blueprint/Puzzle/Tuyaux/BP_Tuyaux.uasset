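; BP_Tuyaux is a rotatable pipe piece in a puzzle linked to BP_Bath.
; EventRotateTuyaux runs a timeline that lerps the pipe's roll by minus 90 degrees, then re-enables player input.
; It then flags whether the roll nearly matches either of two accepted angles, printing a debug "Win" on a match.
; Finally, it asks the BP_Bath found at BeginPlay to check whether the pipe puzzle is finished.
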(event `self.ReceiveBeginPlay`
  (set `self.PlayerRef` (cast `/Game/Sacha/Blueprint/BP_FirstPersonCharacterSacha` (`GameplayStatics.GetPlayerCharacter` 0) :!pure true))
  (bind _returnvalue (`GameplayStatics.GetActorOfClass` "/Game/Sacha/Blueprint/Items/ItemOnlyInteract/Bathtub/BP_Bath.BP_Bath_C"))
  (set `self.BP_Bath` _returnvalue))

(event `self.ReceiveTick`
  (params (DeltaSeconds :type "Float (single-precision)")))

(event `EventCheckRotation`
  (bind _relativerotation_roll (`KismetMathLibrary.BreakRotator` (`SceneComponent.RelativeRotation` (`self.Tuyau`))))
  (bind _relativerotation_roll_2 (`KismetMathLibrary.BreakRotator` (`SceneComponent.RelativeRotation` (`self.Tuyau`))))
  (if (or (`KismetMathLibrary.NearlyEqual_FloatFloat` _relativerotation_roll (`self.GoodRotation2`) 0.1) (`KismetMathLibrary.NearlyEqual_FloatFloat` _relativerotation_roll_2 (`self.GoodRotation`) 0.1))
    (set `self.IsInGoodPosition` true)
    (`KismetSystemLibrary.PrintString` (`KismetStringLibrary.Concat_StrStr` (`KismetSystemLibrary.GetDisplayName` self) "Win") true true (struct :`R` 1.0 :`B` 0.399914 :`A` 1.0))
    (else
      (set `self.IsInGoodPosition` false))))

(event `EventRotateTuyaux`
  (bind _relativerotation_roll (`KismetMathLibrary.BreakRotator` (`SceneComponent.RelativeRotation` (`self.Tuyau`))))
  (set `self.InitialRotation` _relativerotation_roll)
  (bind (_direction _newtrack_0) (`Timeline|Timeline` :!via `PlayFromStart`)
    (:`Update`
      (`SceneComponent.K2_SetWorldRotation` (`self.Tuyau`) (`KismetMathLibrary.MakeRotator` (`KismetMathLibrary.Lerp` (`self.InitialRotation`) (- (`self.InitialRotation`) 90.0) _newtrack_0)) false false))
    (:`Finished`
      (`self.EnableInput` (`self.PlayerRef`) (`GameplayStatics.GetPlayerController` 0))
      (`self.EventCheckRotation`)
      (`/Game/Sacha/Blueprint/Items/ItemOnlyInteract/Bathtub/BP_Bath.EventCheckIfTuyauxIsFinish` (`self.BP_Bath`)))))

(fn `UserConstructionScript`)