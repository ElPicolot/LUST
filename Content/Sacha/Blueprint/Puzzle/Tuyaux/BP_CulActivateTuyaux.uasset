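; Interactable pipe puzzle actor that, when activated, enables interaction on linked pipe actors and starts a water leak effect.
; InteractWorking stores the player and reveals a scar decal, then loops over CulTuyau, setting each element's CanInteractWith map.
; Inside that loop it also plays whip-hit and flowing-water sounds and shows two small waterfall meshes, so these repeat per element.
; Afterwards it sets its own CanInteractWith entry to false.
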(event `self.Interact Working`
  (params (ItemInHand :type "/Game/Sacha/Blueprint/Items/E_MainItemType Enum" :default "NewEnumerator0") (ItemInHandforAnim :type "/Game/Sacha/Blueprint/Items/BP_Item Object Reference") (PlayrRef :type "/Game/Sacha/Blueprint/BP_FirstPersonCharacterSacha Object Reference"))
  (set `self.Playr Ref_0` PlayrRef)
  (`SceneComponent.SetVisibility` (`self.Decal_Scars`) true false)
  (for _array_element (`self.CulTuyau`)
    (set `/Game/Sacha/Blueprint/Items/BP_Interaction.CanInteractWith?` (`|MakeMap` "NewEnumerator1" true :!type "/Game/Sacha/Blueprint/Items/E_MainItemType Enum") _array_element)
    (`GameplayStatics.PlaySoundAtLocation` "/Game/Sounds/SFX/Fouet_Coup.Fouet_Coup" (`SceneComponent.K2_GetComponentLocation` (`self.Audio_Fouet`)) (struct) 1.0 1.0 0.0 null null null null)
    (`SceneComponent.SetVisibility` (`self.SM_LittleWaterfall`) true false)
    (`GameplayStatics.PlaySoundAtLocation` "/Game/Sounds/SFX/Water_Flowing_Ambience.Water_Flowing_Ambience" (`SceneComponent.K2_GetComponentLocation` (`self.Audio_Eau`)) (struct) 1.0 1.0 0.0 null null null null)
    (`SceneComponent.SetVisibility` (`self.SM_LittleWaterfall1`) true false)
    (`GameplayStatics.PlaySoundAtLocation` "/Game/Sounds/SFX/Water_Flowing_Ambience.Water_Flowing_Ambience" (`SceneComponent.K2_GetComponentLocation` (`self.Audio_Eau`)) (struct) 1.0 1.0 0.0 null null null null))
  (set `self.CanInteractWith?` (`|MakeMap` "NewEnumerator0" :!type "/Game/Sacha/Blueprint/Items/E_MainItemType Enum")))

(fn `UserConstructionScript`
  (`parent.UserConstructionScript`))