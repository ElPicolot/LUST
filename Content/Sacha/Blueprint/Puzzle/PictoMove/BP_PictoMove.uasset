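; Picto shuffle puzzle where three decals blink, hide and swap places over six rounds of increasing speed and shuffle count.
; When the player first stands in the box with the whip, timelines align position and view to the puzzle.
; Watching it starts a round: a looping timer shuffles target positions for per-decal timelines, ending on the initial slots.
; The three CUL actors then snap to their decals and receive CallMonsterMessage.
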(event `self.ReceiveBeginPlay`
  (bind _speedcharalocationrotation (`self.SpeedCharaLocationRotation`))
  (bind (_returnvalue_x _returnvalue_y _returnvalue_z) (`KismetMathLibrary.BreakVector` (`SceneComponent.K2_GetComponentLocation` (`self.Decal_descendre`))))
  (bind (_returnvalue_x_2 _returnvalue_y_2 _returnvalue_z_2) (`KismetMathLibrary.BreakVector` (`SceneComponent.K2_GetComponentLocation` (`self.decalEcarteler`))))
  (bind (_returnvalue_x_3 _returnvalue_y_3 _returnvalue_z_3) (`KismetMathLibrary.BreakVector` (`SceneComponent.K2_GetComponentLocation` (`self.DecalLose`))))
  (set `self.TargetPoseArray` (`|MakeArray` (`SceneComponent.RelativeLocation` (`self.Target1`)) (`SceneComponent.RelativeLocation` (`self.Target2`)) (`SceneComponent.RelativeLocation` (`self.Target3`)) (`SceneComponent.RelativeLocation` (`self.Target4`)) (`SceneComponent.RelativeLocation` (`self.Target5`))))
  (bind _returnvalue (`DecalComponent.CreateDynamicMaterialInstance` (`self.Decal_descendre`)))
  (bind _output_get (set `self.MatDecalDescendreInst` _returnvalue))
  (bind _returnvalue_2 (`DecalComponent.CreateDynamicMaterialInstance` (`self.decalEcarteler`)))
  (bind _output_get_2 (set `self.MatDecalEcartelerInst` _returnvalue_2))
  (bind _returnvalue_3 (`DecalComponent.CreateDynamicMaterialInstance` (`self.DecalLose`)))
  (bind _output_get_3 (set `self.MatDecalLoseInst` _returnvalue_3))
  (set `self.MatInstArray` (`|MakeArray` _output_get _output_get_2 _output_get_3))
  (set `self.Pictos` (`|MakeArray` (`self.DecalLose`) (`self.decalEcarteler`) (`self.Decal_descendre`)))
  (bind _output_get_4 (set `self.TimelineArray` (`|MakeArray` (`self.MoveDacalLose`) (`self.MoveDecalEcarteler`) (`self.MoveDecalDesendre`))))
  (for _array_element _output_get_4
    (`TimelineComponent.SetPlayRate` _array_element (/ 1.0 (`self.Speed`)))
    (`TimelineComponent.SetPlayRate` (`self.PictoBlink`) (/ 1.0 (`self.SpeedBink`)))
    (`TimelineComponent.SetPlayRate` (`self.CharaLocation`) (/ 1.0 _speedcharalocationrotation))
    (`TimelineComponent.SetPlayRate` (`self.CharaRotation`) (/ 1.0 _speedcharalocationrotation))
    (`self.K2_SetActorLocation` (`self.CUL1`) (`KismetMathLibrary.MakeVector` _returnvalue_x _returnvalue_y (+ _returnvalue_z (`self.CulOffset`))) false false)
    (`self.K2_SetActorLocation` (`self.CUL2`) (`KismetMathLibrary.MakeVector` _returnvalue_x_2 _returnvalue_y_2 (+ _returnvalue_z_2 (`self.CulOffset`))) false false)
    (`self.K2_SetActorLocation` (`self.CUL3`) (`KismetMathLibrary.MakeVector` _returnvalue_x_3 _returnvalue_y_3 (+ _returnvalue_z_3 (`self.CulOffset`))) false false)))

(event `self.ReceiveTick`
  (params (DeltaSeconds :type "Float (single-precision)"))
  (bind _playerref (`self.PlayerRef`))
  (bind _playerref_2 (`self.PlayerRef`))
  (bind _numberofpuzzle (`self.NumberOfPuzzle`))
  (bind (_returnvalue_x _returnvalue_y _returnvalue_z) (`KismetMathLibrary.BreakVector` (`self.K2_GetActorLocation` _playerref_2)))
  (bind (_returnvalue_roll _returnvalue_pitch _returnvalue_yaw) (`KismetMathLibrary.BreakRotator` (`KismetMathLibrary.FindLookAtRotation` (`self.K2_GetActorLocation` _playerref) (`SceneComponent.K2_GetComponentLocation` (`self.TargetCam`)))))
  (bind (_returnvalue_roll_2 _returnvalue_pitch_2 _returnvalue_yaw_2) (`KismetMathLibrary.BreakRotator` (`SceneComponent.K2_GetComponentRotation` (`Actor.RootComponent` _playerref))))
  (`|ExecutionSequence`
    (:`then_0`
      (if (and (`self.HasWhip`) (`self.IsInTheBox`))
        (`/Engine/EditorBlueprintResources/StandardMacros.DoOnce` false
          (:`Completed`
            (set `self.IsPuzzeling` true)
            (bind _asbp_first_person_character_sacha (cast `/Game/Sacha/Blueprint/BP_FirstPersonCharacterSacha` (`self.Player`)))
            (set `self.PlayerRef` _asbp_first_person_character_sacha)
            (`/Engine/EditorBlueprintResources/StandardMacros.DoOnce` false
              (:`Completed`
                (`|ExecutionSequence`
                  (:`then_0`
                    (`self.DisableInput` (`self.PlayerRef`) (`GameplayStatics.GetPlayerController` 0))
                    (set `/Game/Sacha/Blueprint/BP_FirstPersonCharacterSacha.IsMoving` false (`self.PlayerRef`))
                    (bind (_direction _location) (`Timeline|CharaLocation` :!via `PlayFromStart`)
                      (:`Update`
                        (bind (_returnvalue_x_2 _returnvalue_y_2) (`KismetMathLibrary.BreakVector` (+ (`self.K2_GetActorLocation` _playerref_2) (* _location (- (`SceneComponent.K2_GetComponentLocation` (`self.CameraTarget`)) (`self.K2_GetActorLocation` _playerref_2))))))
                        (`self.K2_SetActorLocation` (`self.PlayerRef`) (`KismetMathLibrary.MakeVector` _returnvalue_x_2 _returnvalue_y_2 _returnvalue_z) false false))
                      (:`Finished`
                        (`self.EnableInput` (`self.PlayerRef`) (`GameplayStatics.GetPlayerController` 0))
                        (message `/Game/Sacha/Interface/BPI_InteractWorking.CallMonster` (`self.CUL3`))
                        (message `/Game/Sacha/Interface/BPI_InteractWorking.CallMonster` (`self.CUL2`))
                        (message `/Game/Sacha/Interface/BPI_InteractWorking.CallMonster` (`self.CUL1`)))))
                  (:`then_1`
                    (bind (_direction_2 _newtrack_0) (`Timeline|CharaRotation` :!via `PlayFromStart`)
                      (:`Update`
                        (`Controller.SetControlRotation` (`GameplayStatics.GetPlayerController` 0) (`KismetMathLibrary.RLerp` (`KismetMathLibrary.MakeRotator` _returnvalue_roll_2 _returnvalue_pitch_2 _returnvalue_yaw_2) (`KismetMathLibrary.MakeRotator` _returnvalue_roll _returnvalue_pitch _returnvalue_yaw) _newtrack_0))))))))))))
    (:`then_1`
      (if (and (`self.HasWhip`) (`self.IsWachingPuzzle`) (`self.IsInTheBox`) (not (`self.IsPuzzeling`)))
        (set `self.IsPuzzeling` true)
        (`KismetSystemLibrary.Delay` (`self.TimeWaitBlink`))
        (`/Engine/EditorBlueprintResources/StandardMacros.IncrementInt` _numberofpuzzle
          (:`  `
            (switch `int` _numberofpuzzle
              (:`1`
                ;[1 1 1] MODIIF DE LA DIFICULT
                (set `self.Speed` 4.0)
                (set `self.NumberOfShuffle` 3))
              (:`2`
                (set `self.Speed` 3.0)
                (set `self.NumberOfShuffle` 5))
              (:`3`
                (set `self.Speed` 2.0)
                (set `self.NumberOfShuffle` 7))
              (:`4`
                (set `self.Speed` 1.5)
                (set `self.NumberOfShuffle` 9))
              (:`5`
                (set `self.Speed` 1.2)
                (set `self.NumberOfShuffle` 12))
              (:`6`
                (set `self.Speed` 1.0)
                (set `self.NumberOfShuffle` 15)))
            (for _array_element (`self.MatInstArray`)
              (`MaterialInstanceDynamic.SetScalarParameterValue` _array_element "IsHide" 0.0)
              (`MaterialInstanceDynamic.SetScalarParameterValue` _array_element "Speed" 1.0))
            (`Timeline|PictoBlink` :!via `PlayFromStart`
              (:`Finished`
                (for _array_element_2 (`self.MatInstArray`)
                  (`MaterialInstanceDynamic.SetScalarParameterValue` _array_element_2 "Speed" 0.0)
                  (`MaterialInstanceDynamic.SetScalarParameterValue` _array_element_2 "IsHide" 1.0)
                  (for _array_element_3 _
                    (`TimelineComponent.SetPlayRate` _array_element_3 (/ (`self.Speed`) 2.0)))
                  (`KismetArrayLibrary.Array_Clear` (`self.TargetPoseArray`))
                  (set `self.TargetPoseArray` (`|MakeArray` (`SceneComponent.RelativeLocation` (`self.Target1`)) (`SceneComponent.RelativeLocation` (`self.Target2`)) (`SceneComponent.RelativeLocation` (`self.Target3`)) (`SceneComponent.RelativeLocation` (`self.Target4`)) (`SceneComponent.RelativeLocation` (`self.Target5`))))
                  (`KismetArrayLibrary.Array_Shuffle` (`self.TargetPoseArray`))
                  (for _array_element_4 (`self.TimelineArray`)
                    (`TimelineComponent.SetPlayRate` _array_element_4 (/ 1.0 (`self.Speed`))))
                  (bind _returnvalue (`KismetSystemLibrary.K2_SetTimerDelegate` (delegate `MoveAllPictoEvent`) (/ 1.0 (`self.Speed`)) true))
                  (set `self.MovePictoHandle` _returnvalue))))))))))

(event `self.Box.OnComponentBeginOverlap`
  (params (OverlappedComponent :type "PrimitiveComponent Object Reference") (OtherActor :type "Actor Object Reference") (OtherComp :type "PrimitiveComponent Object Reference") (OtherBodyIndex :type Integer) (bFromSweep :type Boolean) (SweepResult :type "HitResult Structure (by ref)"))
  (set `self.IsInTheBox` true)
  (`/Engine/EditorBlueprintResources/StandardMacros.DoOnce` false
    (:`Completed`
      (set `self.Player` OtherActor))))

(event `self.Box.OnComponentEndOverlap`
  (params (OverlappedComponent :type "PrimitiveComponent Object Reference") (OtherActor :type "Actor Object Reference") (OtherComp :type "PrimitiveComponent Object Reference") (OtherBodyIndex :type Integer))
  (set `self.IsInTheBox` false))

(event `/Game/Sacha/Interface/BPI_InteractWorking.InteractBetweenItem`
  (set `self.IsPuzzeling` false))

(event `MoveAllPictoEvent`
  (bind (_returnvalue_x _returnvalue_y _returnvalue_z) (`KismetMathLibrary.BreakVector` (`SceneComponent.K2_GetComponentLocation` (`self.Decal_descendre`))))
  (bind (_returnvalue_x_2 _returnvalue_y_2 _returnvalue_z_2) (`KismetMathLibrary.BreakVector` (`SceneComponent.K2_GetComponentLocation` (`self.decalEcarteler`))))
  (bind (_returnvalue_x_3 _returnvalue_y_3 _returnvalue_z_3) (`KismetMathLibrary.BreakVector` (`SceneComponent.K2_GetComponentLocation` (`self.DecalLose`))))
  (if (not (> (`self.counterMove`) (`self.NumberOfShuffle`)))
    (`KismetArrayLibrary.Array_Shuffle` (`self.TargetPoseArray`))
    (`self.MovePicto1Event`)
    (`self.MovePicto2Event`)
    (`self.MovePicto3Event`)
    (`/Engine/EditorBlueprintResources/StandardMacros.IncrementInt` (`self.counterMove`)
      (:`  `
        (if (> (`self.counterMove`) (`self.NumberOfShuffle`))
          (`KismetArrayLibrary.Array_Clear` (`self.TargetPoseArray`))
          (set `self.TargetPoseArray` (`|MakeArray` (`SceneComponent.RelativeLocation` (`self.InitialPose1`)) (`SceneComponent.RelativeLocation` (`self.InitialPose2`)) (`SceneComponent.RelativeLocation` (`self.InitialPose3`))))
          (`KismetArrayLibrary.Array_Shuffle` (`self.TargetPoseArray`))
          (`KismetArrayLibrary.Array_Shuffle` (`self.TargetPoseArray`))
          (`KismetArrayLibrary.Array_Shuffle` (`self.TargetPoseArray`))
          (`self.MovePicto1Event`)
          (`self.MovePicto2Event`)
          (`self.MovePicto3Event`)
          (`KismetSystemLibrary.Delay` 0.2)
          (if (> (`self.counterMove`) (`self.NumberOfShuffle`))
            (`KismetSystemLibrary.Delay` (`self.Speed`))
            (`self.K2_SetActorLocation` (`self.CUL1`) (`KismetMathLibrary.MakeVector` _returnvalue_x _returnvalue_y (+ _returnvalue_z (`self.CulOffset`))) false false)
            (`self.K2_SetActorLocation` (`self.CUL2`) (`KismetMathLibrary.MakeVector` _returnvalue_x_2 _returnvalue_y_2 (+ _returnvalue_z_2 (`self.CulOffset`))) false false)
            (`self.K2_SetActorLocation` (`self.CUL3`) (`KismetMathLibrary.MakeVector` _returnvalue_x_3 _returnvalue_y_3 (+ _returnvalue_z_3 (`self.CulOffset`))) false false)
            (message `/Game/Sacha/Interface/BPI_InteractWorking.CallMonster` (`self.CUL3`))
            (message `/Game/Sacha/Interface/BPI_InteractWorking.CallMonster` (`self.CUL2`))
            (message `/Game/Sacha/Interface/BPI_InteractWorking.CallMonster` (`self.CUL1`))
            (set `self.counterMove` 0)
            (`KismetSystemLibrary.K2_ClearAndInvalidateTimerHandle` (`self.MovePictoHandle`))))))))

(event `MovePicto1Event`
  (bind (_direction _newtrack_0) (`Timeline|MoveDacalLose` :!via `PlayFromStart`)
    (:`Update`
      (`SceneComponent.K2_SetRelativeLocation` (`self.DecalLose`) (+ (`SceneComponent.RelativeLocation` (`self.DecalLose`)) (* _newtrack_0 (- (`|GetArrayItem` (`self.TargetPoseArray`)) (`SceneComponent.RelativeLocation` (`self.DecalLose`))))) false false))))

(event `MovePicto2Event`
  (bind (_direction _newtrack_0) (`Timeline|MoveDecalEcarteler` :!via `PlayFromStart`)
    (:`Update`
      (`SceneComponent.K2_SetRelativeLocation` (`self.decalEcarteler`) (+ (`SceneComponent.RelativeLocation` (`self.decalEcarteler`)) (* _newtrack_0 (- (`|GetArrayItem` (`self.TargetPoseArray`) 1) (`SceneComponent.RelativeLocation` (`self.decalEcarteler`))))) false false))))

(event `MovePicto3Event`
  (bind (_direction _newtrack_0) (`Timeline|MoveDecalDesendre` :!via `PlayFromStart`)
    (:`Update`
      (`SceneComponent.K2_SetRelativeLocation` (`self.Decal_descendre`) (+ (`SceneComponent.RelativeLocation` (`self.Decal_descendre`)) (* _newtrack_0 (- (`|GetArrayItem` (`self.TargetPoseArray`) 2) (`SceneComponent.RelativeLocation` (`self.Decal_descendre`))))) false false))))

(event `EventMaterialCul1`
  (bind _cul1 (`self.CUL1`))
  (bind _staticmesh (`/Game/Sacha/Blueprint/Items/BP_Interaction.StaticMesh` _cul1))
  (bind _returnvalue_x (`KismetMathLibrary.BreakVector` (`SceneComponent.K2_GetComponentLocation` (`Actor.RootComponent` (`self.CUL1`)))))
  ;[1 1 1] Test changement de materials
  (if (`KismetMathLibrary.NearlyEqual_FloatFloat` _returnvalue_x 0.0 10.0)
    (`PrimitiveComponent.SetMaterial` (`/Game/Sacha/Blueprint/Items/BP_Interaction.StaticMesh` _cul1) 1 "/Game/3D/RA_Ass/MI_Cheeks/MI_Cheeks_Scars.MI_Cheeks_Scars")
    (elif (`KismetMathLibrary.NearlyEqual_FloatFloat` _returnvalue_x 0.0 10.0)
      (`PrimitiveComponent.SetMaterial` _staticmesh 1 "/Game/3D/RA_Ass/MI_Cheeks/MI_Cheeks_Scotch.MI_Cheeks_Scotch")
      (else
        (`PrimitiveComponent.SetMaterial` _staticmesh 1 "/Game/3D/RA_Ass/MI_Cheeks/MI_Cheeks_2.MI_Cheeks_2")))))

(event `EventMaterialCul2`
  (bind _cul2 (`self.CUL2`))
  (bind _returnvalue_x (`KismetMathLibrary.BreakVector` (`SceneComponent.K2_GetComponentLocation` (`self.InitialPose1`))))
  (bind _returnvalue_x_2 (`KismetMathLibrary.BreakVector` (`SceneComponent.K2_GetComponentLocation` (`self.InitialPose3`))))
  (bind _returnvalue_x_3 (`KismetMathLibrary.BreakVector` (`SceneComponent.K2_GetComponentLocation` (`Actor.RootComponent` (`self.CUL2`)))))
  ;[1 1 1] Test changement de materials
  (if (`KismetMathLibrary.NearlyEqual_FloatFloat` _returnvalue_x_3 _returnvalue_x 10.0)
    (`PrimitiveComponent.SetMaterial` (`/Game/Sacha/Blueprint/Items/BP_Interaction.StaticMesh` _cul2) 1 "/Game/3D/RA_Ass/MI_Cheeks/MI_Cheeks_Scars.MI_Cheeks_Scars")
    (elif (`KismetMathLibrary.NearlyEqual_FloatFloat` _returnvalue_x_3 _returnvalue_x_2 10.0)
      (`PrimitiveComponent.SetMaterial` (`/Game/Sacha/Blueprint/Items/BP_Interaction.StaticMesh` _cul2) 1 "/Game/3D/RA_Ass/MI_Cheeks/MI_Cheeks_Scotch.MI_Cheeks_Scotch")
      (else
        (`PrimitiveComponent.SetMaterial` (`/Game/Sacha/Blueprint/Items/BP_Interaction.StaticMesh` _cul2) 1 "/Game/3D/RA_Ass/MI_Cheeks/MI_Cheeks_2.MI_Cheeks_2")))))

(event `EventMaterialCul3`
  (bind _cul3 (`self.CUL3`))
  (bind _returnvalue_x (`KismetMathLibrary.BreakVector` (`SceneComponent.K2_GetComponentLocation` (`self.InitialPose1`))))
  (bind _returnvalue_x_2 (`KismetMathLibrary.BreakVector` (`SceneComponent.K2_GetComponentLocation` (`self.InitialPose3`))))
  (bind _returnvalue_x_3 (`KismetMathLibrary.BreakVector` (`SceneComponent.K2_GetComponentLocation` (`Actor.RootComponent` (`self.CUL3`)))))
  ;[1 1 1] Test changement de materials
  (if (`KismetMathLibrary.NearlyEqual_FloatFloat` _returnvalue_x_3 _returnvalue_x 10.0)
    (`PrimitiveComponent.SetMaterial` (`/Game/Sacha/Blueprint/Items/BP_Interaction.StaticMesh` _cul3) 1 "/Game/3D/RA_Ass/MI_Cheeks/MI_Cheeks_Scars.MI_Cheeks_Scars")
    (elif (`KismetMathLibrary.NearlyEqual_FloatFloat` _returnvalue_x_3 _returnvalue_x_2 10.0)
      (`PrimitiveComponent.SetMaterial` (`/Game/Sacha/Blueprint/Items/BP_Interaction.StaticMesh` _cul3) 1 "/Game/3D/RA_Ass/MI_Cheeks/MI_Cheeks_Scotch.MI_Cheeks_Scotch")
      (else
        (`PrimitiveComponent.SetMaterial` (`/Game/Sacha/Blueprint/Items/BP_Interaction.StaticMesh` _cul3) 1 "/Game/3D/RA_Ass/MI_Cheeks/MI_Cheeks_2.MI_Cheeks_2")))))

(fn `UserConstructionScript`
  (bind (_returnvalue_x _returnvalue_y _returnvalue_z) (`KismetMathLibrary.BreakVector` (`SceneComponent.K2_GetComponentLocation` (`self.Decal_descendre`))))
  (bind (_returnvalue_x_2 _returnvalue_y_2 _returnvalue_z_2) (`KismetMathLibrary.BreakVector` (`SceneComponent.K2_GetComponentLocation` (`self.decalEcarteler`))))
  (bind (_returnvalue_x_3 _returnvalue_y_3 _returnvalue_z_3) (`KismetMathLibrary.BreakVector` (`SceneComponent.K2_GetComponentLocation` (`self.DecalLose`))))
  (`self.K2_SetActorLocation` (`self.CUL1`) (`KismetMathLibrary.MakeVector` _returnvalue_x _returnvalue_y (+ _returnvalue_z (`self.CulOffset`))) false false)
  (`self.K2_SetActorLocation` (`self.CUL2`) (`KismetMathLibrary.MakeVector` _returnvalue_x_2 _returnvalue_y_2 (+ _returnvalue_z_2 (`self.CulOffset`))) false false)
  (`self.K2_SetActorLocation` (`self.CUL3`) (`KismetMathLibrary.MakeVector` _returnvalue_x_3 _returnvalue_y_3 (+ _returnvalue_z_3 (`self.CulOffset`))) false false))