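; BP_CulPicto is an interactable puzzle pictogram that triggers a reaction on a linked NPC (PNJ1).
; InteractWorking starts puzzling on BPPictoMove, plays the CulFouet animation, and alternates scarf decals between two target locations via FlipFlop.
; ECulType selects the NPC event: descend, quartering or falling.
; Meanwhile a timeline turns the camera toward the offset NPC position with input disabled, then restores input and clears IsPuzzeling.
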(event `/Game/Sacha/Interface/BPI_Interact.Interact Working`
  (params (ItemInHand :type "/Game/Sacha/Blueprint/Items/E_MainItemType Enum" :default "NewEnumerator0") (ItemInHandforAnim :type "/Game/Sacha/Blueprint/Items/BP_Item Object Reference") (PlayrRef :type "/Game/Sacha/Blueprint/BP_FirstPersonCharacterSacha Object Reference"))
  (set `self.Playr Ref` PlayrRef)
  (`/Game/Sacha/Blueprint/Puzzle/PictoMove/BP_PictoMove.EventStartPuzzling` (`self.BPPictoMove`))
  (`KismetSystemLibrary.PrintString` "ass moving")
  (`self.Animations_Cul` (`self.Cul_fouet`))
  (`self.RotateCameraOnPNJ` (`self.Playr Ref`) (`self.PNJ1`))
  (`/Engine/EditorBlueprintResources/StandardMacros.FlipFlop`
    (:`A`
      (`self.SpawnScarfDecal` false (`SceneComponent.RelativeLocation` (`self.TargetObject1`))))
    (:`B`
      (`self.SpawnScarfDecal` false (`SceneComponent.RelativeLocation` (`self.TargetObject2`)))))
  (switch `/Game/Sacha/Blueprint/Puzzle/PictoMove/CULPicto/Enum_CulPicto` (`self.E_CulType`)
    (:`NewEnumerator0`
      (`/Game/Sacha/Blueprint/PNJ/BP_PNJ1.EventPNJDecendre` (`self.PNJ1`)))
    (:`NewEnumerator1`
      (`/Game/Sacha/Blueprint/PNJ/BP_PNJ1.EventPnjEcartelement` (`self.PNJ1`)))
    (:`NewEnumerator2`
      (`/Game/Sacha/Blueprint/PNJ/BP_PNJ1.EventPnjFalling` (`self.PNJ1`)))))

(event `RotateCameraOnPNJ`
  (params (PlayerRef :type "/Game/Sacha/Blueprint/BP_FirstPersonCharacterSacha Object Reference") (ActorToLook :type "Actor Object Reference"))
  (bind (_returnvalue_x _returnvalue_y _returnvalue_z) (`KismetMathLibrary.BreakVector` (`self.K2_GetActorLocation` ActorToLook)))
  (bind (_returnvalue_roll _returnvalue_pitch _returnvalue_yaw) (`KismetMathLibrary.BreakRotator` (`SceneComponent.K2_GetComponentRotation` (`Actor.RootComponent` PlayerRef))))
  (bind (_returnvalue_roll_2 _returnvalue_pitch_2 _returnvalue_yaw_2) (`KismetMathLibrary.BreakRotator` (`KismetMathLibrary.FindLookAtRotation` (`self.K2_GetActorLocation` PlayerRef) (`KismetMathLibrary.MakeVector` (+ _returnvalue_x (`self.OffsetXTargetCamera`)) _returnvalue_y (+ _returnvalue_z (`self.OffsetZTargetCamera`))))))
  (`self.DisableInput` PlayerRef (`GameplayStatics.GetPlayerController` 0))
  (bind (_direction _newtrack_0) (`Timeline|Timeline_1` :!via `PlayFromStart`)
    (:`Update`
      (`Controller.SetControlRotation` (`GameplayStatics.GetPlayerController` 0) (`KismetMathLibrary.RLerp` (`KismetMathLibrary.MakeRotator` _returnvalue_roll _returnvalue_pitch _returnvalue_yaw) (`KismetMathLibrary.MakeRotator` _returnvalue_roll_2 _returnvalue_pitch_2 _returnvalue_yaw_2) _newtrack_0)))
    (:`Finished`
      (`self.EnableInput` PlayerRef (`GameplayStatics.GetPlayerController` 0))
      (set `/Game/Sacha/Blueprint/Puzzle/PictoMove/BP_PictoMove.IsPuzzeling` false (`self.BPPictoMove`)))))

(fn `UserConstructionScript`
  (`parent.UserConstructionScript`))