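; BP_JaugeSouffrance is an actor that displays a pain gauge ("souffrance") through a material on its static mesh.
; BeginPlay creates a dynamic instance of MAT_JaugePain and sets its AlphaJ parameter to the current gauge value.
; Each UpJauge event raises a clamped target by a fixed step and enables movement.
; While moving, Tick eases the value toward that target with FInterpTo, updates AlphaJ and prints the value for debugging.
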(event `self.ReceiveBeginPlay`
  (bind _returnvalue (`KismetMaterialLibrary.CreateDynamicMaterialInstance` "/Game/Sacha/Blueprint/JaugeSoufrance/MAT_JaugePain.MAT_JaugePain"))
  (`PrimitiveComponent.SetMaterial` (`self.StaticMeshComponent0`) 0 _returnvalue)
  (bind _output_get (set `self.MatJaugePain` _returnvalue))
  (`MaterialInstanceDynamic.SetScalarParameterValue` _output_get "AlphaJ" (`self.AplhaJaugePain`)))

(event `UpJauge`
  (bind _output_get (set `self.AlphaJaugePainTarget` (`KismetMathLibrary.FClamp` (+ 0.125 (`self.AlphaJaugePainTarget`)) 0.25 1.25)))
  (`KismetSystemLibrary.PrintString` (`KismetStringLibrary.Conv_DoubleToString` _output_get))
  (set `self.IsMoving` true))

(event `self.ReceiveTick`
  (params (DeltaSeconds :type "Float (single-precision)"))
  (bind _aplhajaugepain (`self.AplhaJaugePain`))
  (if (`self.IsMoving`)
    (if (<= (`self.AplhaJaugePain`) (`self.AlphaJaugePainTarget`))
      (set `self.AplhaJaugePain` (`KismetMathLibrary.FInterpTo` (`self.AplhaJaugePain`) (`self.AlphaJaugePainTarget`) (`GameplayStatics.GetWorldDeltaSeconds`) 1.0))
      (`MaterialInstanceDynamic.SetScalarParameterValue` (`self.MatJaugePain`) "AlphaJ" _aplhajaugepain)
      (`KismetSystemLibrary.PrintString` (`KismetStringLibrary.Conv_DoubleToString` _aplhajaugepain))
      (else
        (set `self.IsMoving` false)))))

(fn `UserConstructionScript`)