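; Interactable ash fire pit puzzle that heats a bathtub with a man in it.
; Placing a log plus paper or fuel unlocks the lighter through the CanInteractWith map.
; Lighting without fuel plays success effects, montage, subtitle and sends pain; with fuel, it plays a death montage, then calls the monster.
; Optionally, the held lighter takes its transform from the arrow nearest the player.
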(event `self.ReceiveBeginPlay`
  (set `self.PlayerRef` (cast `/Game/Sacha/Blueprint/BP_FirstPersonCharacterSacha` (`GameplayStatics.GetPlayerCharacter` 0) :!pure true))
  (set `self.CanInteractWith?` (`|MakeMap` "NewEnumerator6" true "NewEnumerator7" true "NewEnumerator11" true "NewEnumerator10" true :!type "/Game/Sacha/Blueprint/Items/E_MainItemType Enum")))

(event `/Game/Sacha/Interface/BPI_Interact.Interact Working`
  (params (ItemInHand :type "/Game/Sacha/Blueprint/Items/E_MainItemType Enum" :default "NewEnumerator0") (ItemInHandforAnim :type "/Game/Sacha/Blueprint/Items/BP_Item Object Reference") (PlayrRef :type "/Game/Sacha/Blueprint/BP_FirstPersonCharacterSacha Object Reference"))
  (bind _returnvalue (`SceneComponent.GetRelativeTransform` (`self.TargetObject3`)))
  (switch `/Game/Sacha/Blueprint/Items/E_MainItemType` ItemInHand
    (:`NewEnumerator2`
      (if (not (`self.FuelIsPlaced`))
        (message `/Game/Sacha/Interface/BPI_Interact.UpPain` (`self.BPPain`) 30.0)
        (`SceneComponent.SetHiddenInGame` (`/Game/Sacha/Blueprint/Items/ItemOnlyInteract/Bathtub/BP_Bath.NS_SmokeBubbleBath` (`self.BP_Bath`)) false false)
        (`GameplayStatics.PlaySoundAtLocation` "/Game/Sounds/SFX/Fire.Fire" (`SceneComponent.K2_GetComponentLocation` (`self.Audio`)) (struct) 1.0 1.0 0.0 null null null null)
        (`GameplayStatics.PlaySoundAtLocation` "/Game/Sounds/Antagonist_Dialogue_Final/20_Asmodeus_Proud.20_Asmodeus_Proud" (`self.K2_GetActorLocation`) (struct) 1.0 1.0 0.0 null null null null)
        (`/Game/Sacha/Winget/WB_SousTitre.EventSousTitrewinget` (`/Game/Sacha/Blueprint/BP_FirstPersonCharacterSacha.WingetSousTitre` (`self.PlayerRef`)) "Asmodeus would be proud")
        (`ActorComponent.SetActive` (`self.FIreWIn`) true false)
        (`|PlayMontage` (`/Game/Sacha/Blueprint/Items/ItemOnlyInteract/Bathtub/BP_Bath.Homme` (`self.BP_Bath`)) "/Game/Animation/Baignoire/baignoire_chauffe_Montage.baignoire_chauffe_Montage"
          (:`then`
            (if (`self.UseLighterTransform`)
              (bind _asbp_first_person_character_sacha (cast `/Game/Sacha/Blueprint/BP_FirstPersonCharacterSacha` (`GameplayStatics.GetPlayerCharacter` 0)))
              (set `/Game/Sacha/Blueprint/Items/BP_Item.Use_Interaction_Loc?` true (`/Game/Sacha/Blueprint/BP_FirstPersonCharacterSacha.ItemInHand` _asbp_first_person_character_sacha)))
            (set `self.CanInteractWith?` (`|MakeMap` "NewEnumerator0" :!type "/Game/Sacha/Blueprint/Items/E_MainItemType Enum") :!label _label)))
        (else
          (`SceneComponent.SetHiddenInGame` (`/Game/Sacha/Blueprint/Items/ItemOnlyInteract/Bathtub/BP_Bath.NS_SmokeBubbleBathLose` (`self.BP_Bath`)) false false)
          (`GameplayStatics.PlaySoundAtLocation` "/Game/StarterContent/Audio/Fire01.Fire01" (`SceneComponent.K2_GetComponentLocation` (`self.Audio`)) (struct) 1.0 1.0 0.0 null null null null)
          (`ActorComponent.SetActive` (`self.FIreLose`) true false)
          (`|PlayMontage` (`/Game/Sacha/Blueprint/Items/ItemOnlyInteract/Bathtub/BP_Bath.Homme` (`self.BP_Bath`)) "/Game/Animation/Baignoire/Baignoire_mort_essence_Montage.Baignoire_mort_essence_Montage"
            (:`then`
              (goto _label))
            (:`OnCompleted`
              (message `/Game/Sacha/Interface/BPI_Interact.CallMonster` (`self.BPMonster`)))))))
    (:`NewEnumerator6`
      (`AddComponent|NODE_AddStaticMeshComponent-4` :`RelativeTransform` _returnvalue)
      (set `self.LogIsPlaced` true)
      (if (or (`self.CombustibleIsPlaced`) (`self.FuelIsPlaced`))
        (set `self.CanInteractWith?` (`|MakeMap` "NewEnumerator7" true "NewEnumerator11" true "NewEnumerator10" true "NewEnumerator2" true :!type "/Game/Sacha/Blueprint/Items/E_MainItemType Enum") :!label _label_2)))
    (:`NewEnumerator10`
      (set `self.FuelIsPlaced` true)
      (`KismetSystemLibrary.PrintString` "Hello")
      (`self.EventFuel`)
      (`KismetSystemLibrary.PrintString` "Hello")
      (if (`self.LogIsPlaced`)
        (`KismetSystemLibrary.PrintString` "CAN FIRE")
        (goto _label_2)))
    (:`NewEnumerator11`
      (`AddComponent|NODE_AddStaticMeshComponent-0` :`RelativeTransform` _returnvalue)
      (set `self.CombustibleIsPlaced` true)
      (if (`self.LogIsPlaced`)
        (goto _label_2)))))

(event `/Game/Marion/BPI_Set_Position.Set_Item_position`
  (bind _iteminhand (`/Game/Sacha/Blueprint/BP_FirstPersonCharacterSacha.ItemInHand` (cast `/Game/Sacha/Blueprint/BP_FirstPersonCharacterSacha` (`GameplayStatics.GetPlayerCharacter` 0) :!pure true)))
  (if (`self.UseLighterTransform`)
    (if (`|EnumEquality` (`/Game/Sacha/Blueprint/Items/BP_Item.MainItemType` _iteminhand) "NewEnumerator2")
      (set `/Game/Sacha/Blueprint/Items/BP_Item.Use_Interaction_Loc?` false _iteminhand)
      (bind _near_lighter (`self.Search_Near_Lighter`))
      (set `/Game/Sacha/Blueprint/Items/BP_Item.Lighter_transform` (`SceneComponent.K2_GetComponentToWorld` (`/Game/Sacha/Blueprint/Items/BP_Lighter_T.Arrow` _near_lighter)) _iteminhand)
      (set `self.Distance Min` 1500.0))))

(event `EventFuel`)

(fn `Search_Near_Lighter`
  (returns (Near_Lighter :type "/Game/Sacha/Blueprint/Items/BP_Lighter_T Object Reference"))
  (for _array_element (`self.Array Lighter T`)
    (bind _returnvalue (`KismetMathLibrary.Vector_Distance` (`SceneComponent.K2_GetComponentLocation` (`/Game/Sacha/Blueprint/Items/BP_Lighter_T.Arrow` _array_element)) (`SceneComponent.K2_GetComponentLocation` (`Character.Mesh` (`self.PlayerRef`)))))
    (if (< _returnvalue (`self.Distance Min`))
      (set `self.Distance Min` _returnvalue)
      (set `self.Near Lighter` _array_element)))
  (return (`self.Near Lighter`)))

(fn `UserConstructionScript`)