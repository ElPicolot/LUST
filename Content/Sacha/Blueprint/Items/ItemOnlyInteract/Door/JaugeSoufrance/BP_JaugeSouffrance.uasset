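; A pain gauge door that fills as it receives pain and swings open once the gauge passes a threshold.
; UpPain adds scaled pain to a target, then a looping timer eases the displayed level toward it through a scalar on a dynamic material.
; At the threshold, the prison light switches to a green material, an opening sound plays and a one-shot timeline rotates the door's yaw.
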(event `self.ReceiveBeginPlay`
  (bind _returnvalue (`KismetMaterialLibrary.CreateDynamicMaterialInstance` "/Game/Sacha/Blueprint/Items/ItemOnlyInteract/Door/JaugeSoufrance/MAT_JaugePain.MAT_JaugePain"))
  (`PrimitiveComponent.SetMaterial` (`self.DoorAperture`) 1 _returnvalue)
  (bind _output_get (set `self.MatJaugePain` _returnvalue))
  (`MaterialInstanceDynamic.SetScalarParameterValue` _output_get "AlphaJ" (`self.AplhaJaugePain`)))

(event `/Game/Sacha/Interface/BPI_InteractWorking.UpPain`
  (params (PainValue :type "Float (double-precision)"))
  (set `self.AlphaJaugePainTarget` (+ (/ PainValue 200.0) (`self.AlphaJaugePainTarget`)))
  (bind _returnvalue (`KismetSystemLibrary.K2_SetTimerDelegate` (delegate `UpJauge`) 0.02 true))
  (set `self.JaugePainHandle` _returnvalue))

(event `UpJauge`
  (if (>= (`self.AplhaJaugePain`) 0.75)
    (`self.StartMoveDoor`)
    (`PrimitiveComponent.SetMaterial` (`self.Prisonlight`) 1 "/AnimationSharing/AnimSharingGreen.AnimSharingGreen")
    (`KismetSystemLibrary.K2_ClearAndInvalidateTimerHandle` (`self.JaugePainHandle`))
    (else
      (set `self.AplhaJaugePain` (`KismetMathLibrary.FInterpTo` (`self.AplhaJaugePain`) (`self.AlphaJaugePainTarget`) (`GameplayStatics.GetWorldDeltaSeconds`) 2.0))
      (`MaterialInstanceDynamic.SetScalarParameterValue` (`self.MatJaugePain`) "AlphaJ" (`self.AplhaJaugePain`))
      (if (`KismetMathLibrary.NearlyEqual_FloatFloat` (`self.AplhaJaugePain`) (`self.AlphaJaugePainTarget`))
        (`KismetSystemLibrary.K2_ClearAndInvalidateTimerHandle` (`self.JaugePainHandle`))))))

(event `StartMoveDoor`
  (bind _door (`self.Door`))
  (bind (_relativerotation_roll _relativerotation_pitch) (`KismetMathLibrary.BreakRotator` (`SceneComponent.RelativeRotation` _door)))
  (`GameplayStatics.PlaySoundAtLocation` "/Game/Sounds/Audio_Effect/Door_Opening.Door_Opening" (`self.K2_GetActorLocation`) (struct) 1.0 1.0 0.0 null null null null)
  (`/Engine/EditorBlueprintResources/StandardMacros.DoOnce` false
    (:`Completed`
      (bind (_direction _newtrack_0) (`Timeline|Timeline_1`)
        (:`Update`
          (`SceneComponent.K2_SetRelativeRotation` _door (`KismetMathLibrary.MakeRotator` _relativerotation_roll _relativerotation_pitch (`KismetMathLibrary.Lerp` 0.0 110.0 _newtrack_0)) false false)
          (`AudioComponent.SetSound` (`self.Audio`) null)
          (`AudioComponent.Play` (`self.Audio`) 0.0))))))

(fn `UserConstructionScript`)