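; Double door that stages a scripted monster encounter, spawning BP_Monster and forcing the player to watch it.
; CallMonster waits, spawns the monster at the Cube, disables input, shows a subtitle and swings both door meshes open in opposite yaw via a timeline.
; A looping timer, never cleared here, rotates the player's view toward the monster and keeps input disabled.
; OpenDoorEvent separately plays a voice line with subtitle and replays the opening.
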(event `self.ReceiveBeginPlay`
  (set `self.As BP First Person Character Sacha` (cast `/Game/Sacha/Blueprint/BP_FirstPersonCharacterSacha` (`GameplayStatics.GetPlayerCharacter` 0) :!pure true)))

(event `/Game/Sacha/Interface/BPI_Interact.CallMonster`
  (bind _staticmesh1 (`self.StaticMesh1`))
  (bind _staticmesh2 (`self.StaticMesh2`))
  (bind (_relativerotation_roll _relativerotation_pitch) (`KismetMathLibrary.BreakRotator` (`SceneComponent.RelativeRotation` _staticmesh2)))
  (bind (_relativerotation_roll_2 _relativerotation_pitch_2) (`KismetMathLibrary.BreakRotator` (`SceneComponent.RelativeRotation` _staticmesh1)))
  (`KismetSystemLibrary.Delay` 2.0)
  (bind _returnvalue (`|SpawnActorFromClass` "/Game/Sacha/Monster/BP_Monster.BP_Monster_C" (`KismetMathLibrary.MakeTransform` (`SceneComponent.K2_GetComponentLocation` (`self.Cube`))) "AdjustIfPossibleButAlwaysSpawn" "MultiplyWithRoot" null null))
  (set `self.Monster` _returnvalue)
  (`self.DisableInput` (`self.As BP First Person Character Sacha`) (`GameplayStatics.GetPlayerController` 0))
  (`KismetSystemLibrary.K2_SetTimerDelegate` (delegate `EventWatchMonster`) 0.02 true)
  (`/Game/Sacha/Winget/WB_SousTitre.EventSousTitrewinget` (`/Game/Sacha/Blueprint/BP_FirstPersonCharacterSacha.WingetSousTitre` (cast `/Game/Sacha/Blueprint/BP_FirstPersonCharacterSacha` (`GameplayStatics.GetPlayerCharacter` 0) :!pure true)) "Again sinner...")
  (bind (_direction _newtrack_0) (`Timeline|Timeline_1` :!label _label)
    (:`Update`
      (bind _returnvalue_2 (`KismetMathLibrary.Lerp` 0.0 100.0 _newtrack_0))
      (`SceneComponent.K2_SetRelativeRotation` _staticmesh1 (`KismetMathLibrary.MakeRotator` _relativerotation_roll_2 _relativerotation_pitch_2 _returnvalue_2) false false)
      (`SceneComponent.K2_SetRelativeRotation` _staticmesh2 (`KismetMathLibrary.MakeRotator` _relativerotation_roll _relativerotation_pitch (* _returnvalue_2 -1.0)) false false))))

(event `OpenDoorEvent`
  (`/Game/Sacha/Winget/WB_SousTitre.EventSousTitrewinget` (`/Game/Sacha/Blueprint/BP_FirstPersonCharacterSacha.WingetSousTitre` (`self.As BP First Person Character Sacha`)) "Now... Its your turn!")
  (`GameplayStatics.PlaySoundAtLocation` "/Game/Sounds/Antagonist_Dialogue_Final/22_Now_Your_Turn.22_Now_Your_Turn" (`self.K2_GetActorLocation`) (struct) 1.0 1.0 0.0 null null null null)
  (goto _label :!via `PlayFromStart`))

(event `EventWatchMonster`
  (bind _as_bp_first_person_character_sacha (`self.As BP First Person Character Sacha`))
  (bind (_returnvalue_x _returnvalue_y _returnvalue_z) (`KismetMathLibrary.BreakVector` (`self.K2_GetActorLocation` (`self.Monster`))))
  (bind (_returnvalue_x_2 _returnvalue_y_2 _returnvalue_z_2) (`KismetMathLibrary.BreakVector` (`self.K2_GetActorLocation` _as_bp_first_person_character_sacha)))
  (`Controller.SetControlRotation` (`GameplayStatics.GetPlayerController` 0) (`KismetMathLibrary.RInterpTo` (`SceneComponent.K2_GetComponentRotation` (`Character.CapsuleComponent` _as_bp_first_person_character_sacha)) (`KismetMathLibrary.FindLookAtRotation` (`KismetMathLibrary.MakeVector` _returnvalue_x_2 _returnvalue_y_2 _returnvalue_z_2) (`KismetMathLibrary.MakeVector` _returnvalue_x _returnvalue_y _returnvalue_z)) (`GameplayStatics.GetWorldDeltaSeconds`) 1.0))
  (`self.DisableInput` (`self.As BP First Person Character Sacha`) (`GameplayStatics.GetPlayerController` 0)))

(fn `UserConstructionScript`
  (`parent.UserConstructionScript`))