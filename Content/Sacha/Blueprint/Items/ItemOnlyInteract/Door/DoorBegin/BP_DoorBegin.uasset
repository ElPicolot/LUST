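; BP_DoorBegin is a scripted door that swings open, then closes behind the player with a voice line.
; The first overlap of BoxOpen by any actor plays an opening sound and runs the DoorRot timeline to lerp the door's yaw.
; The player's first overlap of BoxClose sends a subtitle to the player's widget, plays the player's audio component and reverses the timeline.
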(event `self.ReceiveBeginPlay`
  (bind _returnvalue (`GameplayStatics.GetActorOfClass` "/Game/Sacha/Blueprint/BP_FirstPersonCharacterSacha.BP_FirstPersonCharacterSacha_C"))
  (set `self.PlayerRef` _returnvalue))

(event `self.BoxOpen.OnComponentBeginOverlap`
  (params (OverlappedComponent :type "PrimitiveComponent Object Reference") (OtherActor :type "Actor Object Reference") (OtherComp :type "PrimitiveComponent Object Reference") (OtherBodyIndex :type Integer) (bFromSweep :type Boolean) (SweepResult :type "HitResult Structure (by ref)"))
  (`/Engine/EditorBlueprintResources/StandardMacros.DoOnce` false
    (:`Completed`
      (`GameplayStatics.PlaySound2D` "/Game/Sounds/Audio_Effect/Door_Opening.Door_Opening" 1.0 1.0 0.0 null null)
      (bind (_direction _newtrack_0) (`Timeline|DoorRot` :!label _label)
        (:`Update`
          (`SceneComponent.K2_SetRelativeRotation` (`self.Door`) (`KismetMathLibrary.MakeRotator` 0.0 0.0 (`KismetMathLibrary.Lerp` 0.0 150.0 _newtrack_0)) false false))
        (:`Finished`
          (`KismetSystemLibrary.Delay` 2.0))))))

(event `self.BoxClose.OnComponentBeginOverlap`
  (params (OverlappedComponent :type "PrimitiveComponent Object Reference") (OtherActor :type "Actor Object Reference") (OtherComp :type "PrimitiveComponent Object Reference") (OtherBodyIndex :type Integer) (bFromSweep :type Boolean) (SweepResult :type "HitResult Structure (by ref)"))
  (bind _playerref (`self.PlayerRef`))
  (if (== OtherActor (`self.PlayerRef`))
    (`/Engine/EditorBlueprintResources/StandardMacros.DoOnce` false
      (:`Completed`
        ;[1 1 1] Son Player
        (`/Game/Sacha/Winget/WB_SousTitre.EventSousTitrewinget` (`/Game/Sacha/Blueprint/BP_FirstPersonCharacterSacha.WingetSousTitre` _playerref) "Are you going to be a good girl?")
        (`AudioComponent.Play` (`/Game/Sacha/Blueprint/BP_FirstPersonCharacterSacha.Audio` _playerref) 0.0)
        (goto _label :!via `Reverse`)))))

(fn `UserConstructionScript`)