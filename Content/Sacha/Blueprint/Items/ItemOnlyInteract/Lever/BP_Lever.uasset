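; BP_Lever is an interact-only lever that makes a linked TerribleMachine interactable.
; InteractWorking fires its effect only once, and only when the item in hand matches a specific enum value.
; It turns a mesh material green, then rewrites both CanInteractWith maps to enable the machine and disable the lever for the same key.
; After a short delay, it swaps two material slots to MI_Ass and MI_Cheek.
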(event `/Game/Sacha/Interface/BPI_Interact.Interact Working`
  (params (ItemInHand :type "/Game/Sacha/Blueprint/Items/E_MainItemType Enum" :default "NewEnumerator0") (ItemInHandforAnim :type "/Game/Sacha/Blueprint/Items/BP_Item Object Reference") (PlayrRef :type "/Game/Sacha/Blueprint/BP_FirstPersonCharacterSacha Object Reference"))
  (if (`|EnumEquality` ItemInHand "NewEnumerator1")
    (`/Engine/EditorBlueprintResources/StandardMacros.DoOnce` false
      (:`Completed`
        (`PrimitiveComponent.SetMaterial` (`self.StaticMesh`) 1 "/AnimationSharing/AnimSharingGreen.AnimSharingGreen")
        (set `/Game/Sacha/Blueprint/Items/BP_Interaction.CanInteractWith?` (`|MakeMap` "NewEnumerator0" true :!type "/Game/Sacha/Blueprint/Items/E_MainItemType Enum") (`self.TerribleMachine`))
        (set `self.CanInteractWith?` (`|MakeMap` "NewEnumerator0" :!type "/Game/Sacha/Blueprint/Items/E_MainItemType Enum"))
        (`KismetSystemLibrary.Delay` 3.0)
        (`PrimitiveComponent.SetMaterial` (`self.StaticMesh`) 0 "/Game/3D/RA_Ass/MI_Ass.MI_Ass")
        (`PrimitiveComponent.SetMaterial` (`self.StaticMesh`) 1 "/Game/3D/RA_Ass/MI_Cheeks/MI_Cheek.MI_Cheek")))))

(fn `UserConstructionScript`
  (`parent.UserConstructionScript`))