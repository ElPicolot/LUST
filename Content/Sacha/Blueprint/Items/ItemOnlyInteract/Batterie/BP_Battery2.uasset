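; BP_Battery2 is an interact-only battery prop that hooks a cable to the player's held item.
; When InteractWorking receives the matching item type, it reveals its Cable component and attaches the cable end to the CableSocket on that item's skeletal mesh.
; It then finds BP_BatterieMachine through GetActorOfClass and replaces its CanInteractWith map, so the machine accepts that same item type.
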(event `self.Interact Working`
  (params (ItemInHand :type "/Game/Sacha/Blueprint/Items/E_MainItemType Enum" :default "NewEnumerator0") (ItemInHandforAnim :type "/Game/Sacha/Blueprint/Items/BP_Item Object Reference") (PlayrRef :type "/Game/Sacha/Blueprint/BP_FirstPersonCharacterSacha Object Reference"))
  (if (`|EnumEquality` ItemInHand "NewEnumerator3")
    (`SceneComponent.SetVisibility` (`self.Cable`) true false)
    (bind _output_get (set `self.Item in Handfor Anim` ItemInHandforAnim))
    (`CableComponent.SetAttachEndToComponent` (`self.Cable`) (`/Game/Sacha/Blueprint/Items/BP_Item.ItemSkeletalMesh` _output_get) "CableSocket")
    (bind _returnvalue (`GameplayStatics.GetActorOfClass` "/Game/Sacha/Blueprint/Items/ItemOnlyInteract/BatterieMachine/BP_BatterieMachine.BP_BatterieMachine_C"))
    (set `/Game/Sacha/Blueprint/Items/BP_Interaction.CanInteractWith?` (`|MakeMap` "NewEnumerator3" true :!type "/Game/Sacha/Blueprint/Items/E_MainItemType Enum") _returnvalue)))

(fn `UserConstructionScript`
  (`parent.UserConstructionScript`))