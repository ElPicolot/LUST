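; Interactable battery that the player hooks up with a held clamp item to power electrocution interactions.
; InteractWorking plays a sound, activates spark effects, snaps the item's clamps to the terminals and runs runtime-created cables to it.
; Batterienumber selects what unlocks (NPC, battery machines or BP_LesTete) and enables CanElectrocute, except that a standing NPC only gets BatterieOn.
; Electricte, not called here, spawns cooldown-limited Niagara arcs at random line-trace hits.
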(event `self.Interact Working`
  (params (ItemInHand :type "/Game/Sacha/Blueprint/Items/E_MainItemType Enum" :default "NewEnumerator0") (ItemInHandforAnim :type "/Game/Sacha/Blueprint/Items/BP_Item Object Reference") (PlayrRef :type "/Game/Sacha/Blueprint/BP_FirstPersonCharacterSacha Object Reference"))
  (bind _item_in_handfor_anim (`self.Item in Handfor Anim`))
  (bind _item_in_handfor_anim_2 (`self.Item in Handfor Anim`))
  (if (`|EnumEquality` ItemInHand "NewEnumerator3")
    (set `self.Item in Handfor Anim` ItemInHandforAnim)
    (`GameplayStatics.PlaySoundAtLocation` "/Game/Sounds/SFX/pliers-155627.pliers-155627" (`SceneComponent.K2_GetComponentLocation` (`self.Audio_Pliers`)) (struct) 1.0 1.0 0.0 null null null null)
    (`ActorComponent.SetActive` (`self.NS_ElecL`) true false)
    (`ActorComponent.SetActive` (`self.NS_ElecR`) true false)
    (`SceneComponent.K2_AttachToComponent` (`/Game/Sacha/Blueprint/Items/BP_Item.ItemSkeletalMesh3` _item_in_handfor_anim) (`self.TargetObject1`) "None" "SnapToTarget" "SnapToTarget" "KeepRelative" true)
    (`SceneComponent.K2_AttachToComponent` (`/Game/Sacha/Blueprint/Items/BP_Item.ItemSkeletalMesh4` _item_in_handfor_anim) (`self.TargetObject2`) "None" "SnapToTarget" "SnapToTarget" "KeepRelative" true)
    (bind _returnvalue (`AddComponent|NODE_AddCableComponent-2`))
    (set `self.Cable1` _returnvalue)
    (bind _returnvalue_2 (`AddComponent|NODE_AddCableComponent-3`))
    (set `self.Cable2` _returnvalue_2)
    (`CableComponent.SetAttachEndToComponent` (`self.Cable1`) (`/Game/Sacha/Blueprint/Items/BP_Item.ItemSkeletalMesh` _item_in_handfor_anim_2) "CableSocket")
    (`CableComponent.SetAttachEndToComponent` (`self.Cable2`) (`/Game/Sacha/Blueprint/Items/BP_Item.ItemSkeletalMesh2` _item_in_handfor_anim_2) "CableSocket")
    (switch `int` (`self.Batterienumber`)
      (:`0`
        (bind _returnvalue_3 (`GameplayStatics.GetActorOfClass` "/Game/Sacha/Blueprint/PNJ/BP_PNJ1.BP_PNJ1_C"))
        (if (`/Game/Sacha/Blueprint/PNJ/BP_PNJ1.PNJIsDown` _returnvalue_3)
          (set `/Game/Sacha/Blueprint/Items/BP_Interaction.CanInteractWith?` (`|MakeMap` "NewEnumerator1" true "NewEnumerator3" true :!type "/Game/Sacha/Blueprint/Items/E_MainItemType Enum") _returnvalue_3)
          (set `/Game/Sacha/Blueprint/Items/BP_Item.CanElectrocute` true (`self.Item in Handfor Anim`) :!label _label)
          (else
            (set `/Game/Sacha/Blueprint/PNJ/BP_PNJ1.BatterieOn` true _returnvalue_3)
            (`KismetSystemLibrary.PrintString` "finirFALSE" true true (struct :`R` 1.0 :`G` 0.544537 :`A` 1.0) 5.0))))
      (:`1`
        (bind _outactors (`GameplayStatics.GetAllActorsOfClass` "/Game/Sacha/Blueprint/Items/ItemOnlyInteract/BatterieMachine/BP_BatterieMachine.BP_BatterieMachine_C"))
        (for _array_element _outactors
          (set `/Game/Sacha/Blueprint/Items/BP_Interaction.CanInteractWith?` (`|MakeMap` "NewEnumerator3" true :!type "/Game/Sacha/Blueprint/Items/E_MainItemType Enum") _array_element)
          (`KismetSystemLibrary.PrintString` "finirTRUE" true true (struct :`R` 1.0 :`G` 0.544537 :`A` 1.0) 5.0 :!label _label_2)
          (goto _label)))
      (:`2`
        (bind _returnvalue_4 (`GameplayStatics.GetActorOfClass` "/Game/Sacha/Blueprint/Items/ItemOnlyInteract/Torse/BP_LesTete.BP_LesTete_C"))
        (set `/Game/Sacha/Blueprint/Items/BP_Interaction.CanInteractWith?` (`|MakeMap` "NewEnumerator3" true :!type "/Game/Sacha/Blueprint/Items/E_MainItemType Enum") _returnvalue_4)
        (goto _label_2)))))

(event `self.ReceiveTick`
  (params (DeltaSeconds :type "Float (single-precision)")))

(fn `Electricte`
  (locals (RandomDirection :type "Vector Structure") (`Impact Offset` :type "Float (double-precision)" :default 1.0))
  (if (>= (- (`GameplayStatics.GetTimeSeconds`) (`self.LastTrace`)) (`self.TraceCoolDown`))
    ;[1 1 1] Trace
    (set `local.RandomDirection` (`KismetMathLibrary.RandomUnitVector`))
    (bind _outhit (`KismetSystemLibrary.LineTraceSingle` :`Start` (`SceneComponent.K2_GetComponentLocation` (`self.Cable1`)) :`End` (+ (`SceneComponent.K2_GetComponentLocation` (`self.StaticMesh`)) (* (`local.RandomDirection`) (`self.MaxRadius`))) :`TraceChannel` "TraceTypeQuery1" :`DrawDebugType` "ForDuration" :`DrawTime` (`self.TraceCoolDown`)))
    (set `self.LastTrace` (`GameplayStatics.GetTimeSeconds`))
    (bind (_bblockinghit _binitialoverlap _time _distance _location _impactpoint _normal _impactnormal) (`GameplayStatics.BreakHitResult` _outhit))
    ;[1 1 1] Spawn Niagara System and set parameters.
    (if _bblockinghit
      (bind _returnvalue (`NiagaraFunctionLibrary.SpawnSystemAttached` "/Game/VFX/Electricity/CourteElec_01.CourteElec_01" null "None" (12.0 -27.0 0.0) (struct) "KeepRelativeOffset" true))
      (`NiagaraComponent.SetVariableVec3` _returnvalue "BeamStartPoint" (`self.impactautre`))
      (`NiagaraComponent.SetVariableVec3` _returnvalue "BeamEndPoint" (+ _impactpoint (* _impactnormal (`local.Impact Offset`))))
      (`NiagaraComponent.SetVariableVec3` _returnvalue "ImpactNormal" _impactnormal))))

(fn `UserConstructionScript`
  (`parent.UserConstructionScript`))