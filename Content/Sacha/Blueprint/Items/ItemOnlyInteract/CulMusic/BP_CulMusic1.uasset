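; BP_CulMusic1 is an interact-only item that toggles a pitch effect on the audio of a referenced BPSoundEttoffe.
; Each interaction flips a FlipFlop and calls SpawnScarfDecal with the relative location of TargetObject2 or TargetObject1.
; The first state plays a sped-up timeline that drives the pitch multiplier; the second stops it and restores normal pitch.
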(event `self.ReceiveBeginPlay`
  (`TimelineComponent.SetPlayRate` (`self.TimelineModifyPitch`) 4.0))

(event `self.Interact Working`
  (params (ItemInHand :type "/Game/Sacha/Blueprint/Items/E_MainItemType Enum" :default "NewEnumerator0") (ItemInHandforAnim :type "/Game/Sacha/Blueprint/Items/BP_Item Object Reference") (PlayrRef :type "/Game/Sacha/Blueprint/BP_FirstPersonCharacterSacha Object Reference"))
  (bind _audiocomponent0 (`/Game/Kilian/Bp_SoundEtouffe.AudioComponent0` (`self.BPSoundEttoffe`)))
  (`/Engine/EditorBlueprintResources/StandardMacros.FlipFlop`
    (:`A`
      (`self.SpawnScarfDecal` false (`SceneComponent.RelativeLocation` (`self.TargetObject2`)))
      (bind (_direction _newtrack_0) (`Timeline|TimelineModifyPitch` :!label _label)
        (:`Update`
          (`AudioComponent.SetPitchMultiplier` _audiocomponent0 _newtrack_0))))
    (:`B`
      (`self.SpawnScarfDecal` false (`SceneComponent.RelativeLocation` (`self.TargetObject1`)))
      (`AudioComponent.SetPitchMultiplier` _audiocomponent0 1.0)
      (goto _label :!via `Stop`))))

(fn `UserConstructionScript`)