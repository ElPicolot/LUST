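; BP_BoxCache is an interact-only item Blueprint for a box, with logic to move it vertically.
; A looping timer is meant to drive MoveBoxEvent, which moves the mesh toward a target Z and clears the timer on arrival.
; The InteractBetweenItem event is empty and the target and timer setup is disconnected, so the movement never starts from this graph.
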(event `InteractBetweenItem_1`)

(event `MoveBoxEvent`
  (bind _stopmovez (`self.GoMeshMoveZ` null (`self.Target Position Z`) 3.0 false (`self.Offset Position`)))
  (if _stopmovez
    (`KismetSystemLibrary.K2_ClearAndInvalidateTimerHandle` (`self.MovBoxHandle`))))

(fn `UserConstructionScript`
  (`parent.UserConstructionScript`))