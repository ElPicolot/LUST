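; Bathtub puzzle actor with an animated man inside, which fills with water once the pipes are finished and the gutter is broken.
; Finishing the pipes changes pipe-end interactions and, if the gutter is intact, starts a drip.
; Filling plays sound, animation and waterfall, raises pain, and fades a dynamic water material via timeline.
; Only when pipes finish last does input lock while the view turns to the bath.
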(event `self.ReceiveBeginPlay`
  (bind (_relativelocation_x _relativelocation_y _relativelocation_z) (`KismetMathLibrary.BreakVector` (`SceneComponent.RelativeLocation` (`self.Water`))))
  (bind _output_get (set `self.InitialLocation` _relativelocation_z))
  (set `self.TargetLocation` (+ _output_get 40.0))
  (bind _outactors (`GameplayStatics.GetAllActorsOfClass` "/Game/Sacha/Blueprint/Puzzle/Tuyaux/BP_Tuyaux.BP_Tuyaux_C"))
  (set `self.BPTuyaux` _outactors)
  (bind _outactors_2 (`GameplayStatics.GetAllActorsOfClass` "/Game/Sacha/Blueprint/Puzzle/Tuyaux/BP_CulTuyaux.BP_CulTuyaux_C"))
  (set `self.BPCulTuyau` _outactors_2)
  (`TimelineComponent.SetPlayRate` (`self.TimelineWaterUp`) 0.08)
  (`SkeletalMeshComponent.PlayAnimation` (`self.Homme`) "/Game/Animation/Baignoire/Idlle_baignoire_Anim.Idlle_baignoire_Anim" true))

(event `EventWaterUp`
  (`GameplayStatics.SpawnSoundAtLocation` "/Game/Sounds/SFX/Shower_Water.Shower_Water" (`self.K2_GetActorLocation`) (struct) 1.0 1.0 0.0 null null)
  (`SkeletalMeshComponent.PlayAnimation` (`self.Homme`) "/Game/Animation/Baignoire/eua_baignoire.eua_baignoire" false)
  (`SceneComponent.SetVisibility` (`self.SM_BigWaterfall`) true false)
  (message `/Game/Sacha/Interface/BPI_Interact.UpPain` (`self.BPPain`) 50.0)
  (bind _returnvalue (`PrimitiveComponent.CreateDynamicMaterialInstance` (`self.WaterV2`) 0 "/Game/LD/MAT_WaterLevelUp/MI_WaterLevelUp.MI_WaterLevelUp" "None"))
  (bind _output_get (set `self.Dynamic_Material_Water` _returnvalue))
  (`MaterialInstanceDynamic.SetScalarParameterValue` _output_get "Fade Amount" 0.0)
  (bind (_direction _newtrack_0) (`Timeline|Timeline_WaterlevelUp`)
    (:`Update`
      (`MaterialInstanceDynamic.SetScalarParameterValue` _output_get "Fade Amount" _newtrack_0))
    (:`Finished`
      (set `self.WaterUp` true)
      (`SceneComponent.SetVisibility` (`self.SM_BigWaterfall`) true false))))

(event `EventTuyauxIsFinish`
  (bind (_returnvalue_x _returnvalue_y _returnvalue_z) (`KismetMathLibrary.BreakVector` (`self.K2_GetActorLocation` self)))
  (bind (_returnvalue_roll _returnvalue_pitch _returnvalue_yaw) (`KismetMathLibrary.BreakRotator` (`KismetMathLibrary.FindLookAtRotation` (`self.K2_GetActorLocation` (`self.Player Ref`)) (`KismetMathLibrary.MakeVector` _returnvalue_x _returnvalue_y _returnvalue_z))))
  (bind (_returnvalue_roll_2 _returnvalue_pitch_2 _returnvalue_yaw_2) (`KismetMathLibrary.BreakRotator` (`SceneComponent.K2_GetComponentRotation` (`Actor.RootComponent` (`self.Player Ref`)))))
  (for _array_element (`self.BPCulTuyau`)
    (set `/Game/Sacha/Blueprint/Items/BP_Interaction.CanInteractWith?` (`|MakeMap` "NewEnumerator1" true :!type "/Game/Sacha/Blueprint/Items/E_MainItemType Enum") _array_element)
    (for _array_element_2 (`self.BPCulTuyau`)
      (set `/Game/Sacha/Blueprint/Items/BP_Interaction.CanInteractWith?` (`|MakeMap` "NewEnumerator0" :!type "/Game/Sacha/Blueprint/Items/E_MainItemType Enum") _array_element_2))
    (set `self.TuyauxFinish` true)
    (if (`self.GoutiereBroken`)
      (`self.EventWaterUp`)
      (`GameplayStatics.PlaySoundAtLocation` "/Game/Sounds/SFX/EauQuiCoule.EauQuiCoule" (`SceneComponent.K2_GetComponentLocation` (`self.Bath`)) (struct) 1.0 1.0 0.0 null null null null)
      (bind _output_get (set `self.Player Ref` (cast `/Game/Sacha/Blueprint/BP_FirstPersonCharacterSacha` (`GameplayStatics.GetPlayerCharacter` 0) :!pure true)))
      (`self.DisableInput` _output_get (`GameplayStatics.GetPlayerController` 0))
      (bind (_direction _newtrack_0) (`Timeline|LookAtBath` :!via `PlayFromStart`)
        (:`Update`
          (`Controller.SetControlRotation` (`GameplayStatics.GetPlayerController` 0) (`KismetMathLibrary.RLerp` (`KismetMathLibrary.MakeRotator` _returnvalue_roll_2 _returnvalue_pitch_2 _returnvalue_yaw_2) (`KismetMathLibrary.MakeRotator` _returnvalue_roll _returnvalue_pitch _returnvalue_yaw) _newtrack_0)))
        (:`Finished`
          (`self.EnableInput` (`self.Player Ref`) (`GameplayStatics.GetPlayerController` 0))))
      (else
        (`ActorComponent.SetActive` (`self.WaterDrop`) true false)
        (`GameplayStatics.PlaySoundAtLocation` "/Game/Sounds/SFX/Goutte_Cue.Goutte_Cue" (`SceneComponent.K2_GetComponentLocation` (`self.Audio`)) (struct) 1.0 1.0 0.0 null null null null)))))

(event `EventGoutiereBroken`
  (set `self.GoutiereBroken` true)
  (`ActorComponent.SetActive` (`self.WaterDrop`) false false)
  (if (`self.TuyauxFinish`)
    (`self.EventWaterUp`)))

(fn `UserConstructionScript`
  (`parent.UserConstructionScript`))