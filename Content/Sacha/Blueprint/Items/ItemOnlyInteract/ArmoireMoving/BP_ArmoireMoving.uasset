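; BP_ArmoireMoving is an armoire that slides sideways along its relative Y axis when its moving event is called.
; BeginPlay caches the root's starting relative location, sets a target a fixed offset along Y, and slows the timeline's play rate.
; EventMovingArmoire plays that timeline, lerping the root toward the target while X and Z keep their starting values.
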(event `self.ReceiveBeginPlay`
  (bind _output_get (set `self.initialLocationV` (`SceneComponent.RelativeLocation` (`self.SharedRoot`))))
  (bind _output_get_2 (set `self.InitialLocation` (.y _output_get)))
  (set `self.TargetLocation` (+ _output_get_2 140.0))
  (`TimelineComponent.SetPlayRate` (`self.TimelineMoveArmoire`) 0.2))

(event `EventMovingArmoire`
  (bind (_initiallocationv_x _initiallocationv_y _initiallocationv_z) (`KismetMathLibrary.BreakVector` (`self.initialLocationV`)))
  (bind (_direction _newtrack_0) (`Timeline|TimelineMoveArmoire`)
    (:`Update`
      (`SceneComponent.K2_SetRelativeLocation` (`self.SharedRoot`) (`KismetMathLibrary.MakeVector` _initiallocationv_x (`KismetMathLibrary.Lerp` (`self.InitialLocation`) (`self.TargetLocation`) _newtrack_0) _initiallocationv_z) false false))))

(fn `UserConstructionScript`)