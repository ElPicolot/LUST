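; Interactable battery machine whose rotary knob the player turns to ramp up power on an NPC (Pnj2).
; Interacting either handles the held item (clamp or lever check) or switches to the machine's Enhanced Input context and camera.
; Each switch input turns the knob one step, scaling timeline-driven mesh vibration and NPC animation speed.
; Higher levels send pain messages with camera cutaways, then voice and subtitle warnings, and finally call the monster.
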(event `self.ReceiveBeginPlay`
  (set `self.TargetPosition` 0.0))

(event `EventBlendCameraTest`
  (`self.DisableInput` (`self.Player Ref`) (`GameplayStatics.GetPlayerController` 0))
  (`PlayerController.SetViewTargetWithBlend` (`GameplayStatics.GetPlayerController` 0) (`self.BPCameraView`) (`self.BlendSpeed`) "VTBlend_Linear" 0.0 false)
  (`KismetSystemLibrary.Delay` 3.0)
  (`PlayerController.SetViewTargetWithBlend` (`GameplayStatics.GetPlayerController` 0) self (`self.BlendSpeed`) "VTBlend_Linear" 0.0 false)
  (`self.EnableInput` (`self.Player Ref`) (`GameplayStatics.GetPlayerController` 0)))

(event `/Game/Sacha/Interface/BPI_Interact.Interact Working`
  (params (ItemInHand :type "/Game/Sacha/Blueprint/Items/E_MainItemType Enum" :default "NewEnumerator0") (ItemInHandforAnim :type "/Game/Sacha/Blueprint/Items/BP_Item Object Reference") (PlayrRef :type "/Game/Sacha/Blueprint/BP_FirstPersonCharacterSacha Object Reference"))
  (bind _returnvalue (pcsubsystem `EnhancedInputLocalPlayerSubsystem` (`GameplayStatics.GetPlayerController` 0)))
  (set `self.Item in Handfor Anim` ItemInHandforAnim)
  (set `self.Player Ref` PlayrRef)
  (if (`|EnumEquality` ItemInHand "NewEnumerator3")
    (if (`/Game/Sacha/Blueprint/Items/ItemOnlyInteract/Lever/BP_Lever.LeverOn` (`self.Lever`))
      (set `self.CanInteractWith?` (`|MakeMap` "NewEnumerator5" true "NewEnumerator1" true "NewEnumerator2" true "NewEnumerator5" true :!type "/Game/Sacha/Blueprint/Items/E_MainItemType Enum"))
      (else
        (set `self.ClampOn` true)))
    (`/Game/Sacha/Blueprint/Items/BP_Item.EventStopTimeline` (`self.Item in Handfor Anim`))
    (else
      (`self.DisableInput` (`self.Player Ref`) (`GameplayStatics.GetPlayerController` 0))
      (`/Engine/EditorBlueprintResources/StandardMacros.IsValid` _returnvalue
        (:`Is Valid`
          (`EnhancedInputSubsystemInterface.RemoveMappingContext` _returnvalue "/Game/Sacha/Input/IMC_Sacha.IMC_Sacha" (struct))
          (`EnhancedInputSubsystemInterface.AddMappingContext` _returnvalue "/Game/Sacha/Input/IMC_Machine.IMC_Machine" 1 (struct))
          (`PlayerController.SetViewTargetWithBlend` (`GameplayStatics.GetPlayerController` 0) self (`self.BlendSpeed`) "VTBlend_Linear" 0.0 false)
          (`KismetSystemLibrary.Delay` (`self.BlendSpeed`))
          (`self.EnableInput` (`self.Player Ref`) (`GameplayStatics.GetPlayerController` 0))
          (`TimelineComponent.SetPlayRate` (`self.rotateButton`) 3.0))
        (:`Is Not Valid`
          (`KismetSystemLibrary.PrintString` "WTFFFFFFFF"))))))

(event `/Game/Sacha/Interface/BPI_Interact.SwitchInput`
  (params (ActionValuex :type "Float (double-precision)"))
  (bind _pnj2 (`self.Pnj2`))
  (bind _pnj2_2 (`self.Pnj2`))
  (bind _pnj2_3 (`self.Pnj2`))
  (bind _timelinevibration (`self.TimelineVibration`))
  (bind _timelinevibration_2 (`self.TimelineVibration`))
  (bind _timelinevibration_3 (`self.TimelineVibration`))
  (bind _timelinevibration_4 (`self.TimelineVibration`))
  (bind _timelinevibration_5 (`self.TimelineVibration`))
  (bind (_relativerotation_roll _relativerotation_pitch) (`KismetMathLibrary.BreakRotator` (`SceneComponent.RelativeRotation` (`self.ButtunBase`))))
  (`KismetSystemLibrary.PrintString` "Hello")
  (if (not (`self.IsSwitching`))
    (set `self.TargetPosition` (`KismetMathLibrary.FClamp` (+ (`self.TargetPosition`) 27.5) 0.0 270.0))
    (if (!= (`self.TargetPosition`) (`self.CurrentPosition`))
      (set `self.IsSwitching` true)
      (set `self.PowerMachine` (+ (`self.PowerMachine`) 1))
      (bind (_direction _newtrack_0) (`Timeline|rotateButton` :!via `PlayFromStart`)
        (:`Update`
          (`SceneComponent.K2_SetRelativeRotation` (`self.ButtunBase`) (`KismetMathLibrary.MakeRotator` _relativerotation_roll _relativerotation_pitch (`KismetMathLibrary.Lerp` (`self.CurrentPosition`) (`self.TargetPosition`) _newtrack_0)) false false))
        (:`Finished`
          (set `self.CurrentPosition` (`self.TargetPosition`))
          (set `self.IsSwitching` false)
          (switch `int` (`self.PowerMachine`)
            (:`1`
              ;[0.8848 1 0] Son
              (`self.EventVibration`)
              (`TimelineComponent.SetPlayRate` _timelinevibration_2 1.0)
              (set `self.OffsetLocation` (0.2 0.2 0.2))
              (set `self.OffsetRotation` (struct :`Pitch` 0.2 :`Yaw` 0.2 :`Roll` 0.2))
              (set `/Game/Sacha/Blueprint/PNJ/BP_PNJ2.MachineisActivated` true _pnj2_2)
              (set `/Game/Sacha/Blueprint/PNJ/BP_PNJ2.SpeedAnimMachine` 0.5 _pnj2_2))
            (:`2`
              (`TimelineComponent.SetPlayRate` _timelinevibration_2 1.5)
              (set `self.OffsetLocation` (0.3 0.3 0.3))
              (set `self.OffsetRotation` (struct :`Pitch` 0.3 :`Yaw` 0.3 :`Roll` 0.3))
              (set `/Game/Sacha/Blueprint/PNJ/BP_PNJ2.SpeedAnimMachine` 0.6 _pnj2_3))
            (:`3`
              (`TimelineComponent.SetPlayRate` _timelinevibration_3 2.0)
              (set `self.OffsetLocation` (0.4 0.4 0.4))
              (set `self.OffsetRotation` (struct :`Pitch` 0.4 :`Yaw` 0.4 :`Roll` 0.4))
              (set `/Game/Sacha/Blueprint/PNJ/BP_PNJ2.SpeedAnimMachine` 0.7 _pnj2_3))
            (:`4`
              (`TimelineComponent.SetPlayRate` _timelinevibration_3 2.5)
              (set `self.OffsetLocation` (0.5 0.5 0.5))
              (set `self.OffsetRotation` (struct :`Pitch` 0.5 :`Yaw` 0.5 :`Roll` 0.5))
              (set `/Game/Sacha/Blueprint/PNJ/BP_PNJ2.SpeedAnimMachine` 0.8 _pnj2_3))
            (:`5`
              (`TimelineComponent.SetPlayRate` _timelinevibration_4 3.0)
              (set `self.OffsetLocation` (0.6 0.6 0.6))
              (set `self.OffsetRotation` (struct :`Pitch` 0.6 :`Yaw` 0.6 :`Roll` 0.6))
              (set `/Game/Sacha/Blueprint/PNJ/BP_PNJ2.SpeedAnimMachine` 0.9 _pnj2_3))
            (:`6`
              (`TimelineComponent.SetPlayRate` _timelinevibration_4 3.5)
              (set `self.OffsetLocation` (0.7 0.7 0.7))
              (set `self.OffsetRotation` (struct :`Pitch` 0.7 :`Yaw` 0.7 :`Roll` 0.7))
              (set `/Game/Sacha/Blueprint/PNJ/BP_PNJ2.SpeedAnimMachine` 1.0 _pnj2)
              (message `/Game/Sacha/Interface/BPI_Interact.UpPain` (`self.BPPain`) (`self.Pain Value`) :!label _label)
              (`self.EventBlendCameraTest`)
              (`KismetSystemLibrary.PrintString` "Hello" true true (struct :`R` 0.775092 :`G` 1.0 :`B` 0.209088 :`A` 1.0)))
            (:`7`
              (`TimelineComponent.SetPlayRate` _timelinevibration_5 4.0)
              (set `self.OffsetLocation` (0.8 0.8 0.8))
              (set `self.OffsetRotation` (struct :`Pitch` 0.8 :`Yaw` 0.8 :`Roll` 0.8))
              (set `/Game/Sacha/Blueprint/PNJ/BP_PNJ2.SpeedAnimMachine` 1.1 _pnj2)
              (goto _label))
            (:`8`
              (`TimelineComponent.SetPlayRate` _timelinevibration_5 4.5)
              (set `self.OffsetLocation` (0.9 0.9 0.9))
              (set `self.OffsetRotation` (struct :`Pitch` 0.9 :`Yaw` 0.9 :`Roll` 0.9))
              (set `/Game/Sacha/Blueprint/PNJ/BP_PNJ2.SpeedAnimMachine` 1.2 _pnj2)
              (goto _label))
            (:`9`
              (`TimelineComponent.SetPlayRate` _timelinevibration 5.0)
              (set `self.OffsetLocation` (1.0 1.0 1.0))
              (set `self.OffsetRotation` (struct :`Pitch` 1.0 :`Yaw` 1.0 :`Roll` 1.0))
              (set `/Game/Sacha/Blueprint/PNJ/BP_PNJ2.SpeedAnimMachine` 1.3 _pnj2)
              (`/Game/Sacha/Winget/WB_SousTitre.EventSousTitrewinget` (`/Game/Sacha/Blueprint/BP_FirstPersonCharacterSacha.WingetSousTitre` (`self.Player Ref`)) "STOP !")
              (message `/Game/Sacha/Interface/BPI_Interact.PlaySound` (`self.Speaker`) null 0.0))
            (:`10`
              (`TimelineComponent.SetPlayRate` _timelinevibration 8.0)
              (set `self.OffsetLocation` (1.5 1.5 0.0))
              (set `self.OffsetRotation` (struct :`Pitch` 1.5 :`Yaw` 1.5 :`Roll` 1.5))
              (set `/Game/Sacha/Blueprint/PNJ/BP_PNJ2.SpeedAnimMachine` 1.4 _pnj2)
              (`/Game/Sacha/Winget/WB_SousTitre.EventSousTitrewinget` (`/Game/Sacha/Blueprint/BP_FirstPersonCharacterSacha.WingetSousTitre` (`self.Player Ref`)) "There's no pleasure without pain!")
              (message `/Game/Sacha/Interface/BPI_Interact.PlaySound` (`self.Speaker`) "/Game/Sounds/Antagonist_Dialogue_Final/17_NoPassion_Without_Pain.17_NoPassion_Without_Pain" 0.0)
              (message `/Game/Sacha/Interface/BPI_Interact.CallMonster` (`self.BPMonster`))
              (`self.DisableInput` (`self.Player Ref`) (`GameplayStatics.GetPlayerController` 0))
              (`PlayerController.SetViewTargetWithBlend` (`GameplayStatics.GetPlayerController` 0) (`self.BPCameraViewMonster`) (`self.BlendSpeed`) "VTBlend_Linear" 0.0 false))))))))

(event `EventVibration`
  (bind _staticmesh (`self.StaticMesh`))
  (bind _initiallocation (`self.InitialLocation`))
  (bind (_initialrotation_roll _initialrotation_pitch _initialrotation_yaw) (`KismetMathLibrary.BreakRotator` (`self.InitialRotation`)))
  (bind (_offsetrotation_roll _offsetrotation_pitch _offsetrotation_yaw) (`KismetMathLibrary.BreakRotator` (`self.OffsetRotation`)))
  (set `self.InitialLocation` (`SceneComponent.RelativeLocation` _staticmesh))
  (set `self.InitialRotation` (`SceneComponent.RelativeRotation` _staticmesh))
  (bind (_direction _newtrack_0) (`Timeline|TimelineVibration`)
    (:`Update`
      (bind (_returnvalue_location _returnvalue_rotation) (`KismetMathLibrary.BreakTransform` (`KismetMathLibrary.TLerp` (`KismetMathLibrary.MakeTransform` _initiallocation) (`KismetMathLibrary.MakeTransform` (+ _initiallocation (`self.OffsetLocation`)) (`KismetMathLibrary.MakeRotator` (+ _initialrotation_roll _offsetrotation_roll) (+ _initialrotation_pitch _offsetrotation_pitch) (+ _initialrotation_yaw _offsetrotation_yaw))) _newtrack_0)))
      (`SceneComponent.K2_SetRelativeLocationAndRotation` (`self.StaticMesh`) _returnvalue_location _returnvalue_rotation false false))))

(event `EventBlendCamera`
  (bind (_returnvalue_x _returnvalue_y) (`KismetMathLibrary.BreakVector` (`self.K2_GetActorLocation` (`self.BPPain`))))
  (bind (_returnvalue_roll _returnvalue_pitch _returnvalue_yaw) (`KismetMathLibrary.BreakRotator` (`KismetMathLibrary.FindLookAtRotation` (`self.K2_GetActorLocation`) (`KismetMathLibrary.MakeVector` 0.0 _returnvalue_y))))
  (bind (_returnvalue_roll_2 _returnvalue_pitch_2 _returnvalue_yaw_2) (`KismetMathLibrary.BreakRotator` (`SceneComponent.K2_GetComponentRotation` (`/Game/Sacha/Blueprint/BP_FirstPersonCharacterSacha.FirstPersonCamera` (`self.Player Ref`)))))
  (`self.DisableInput` (`self.Player Ref`) (`GameplayStatics.GetPlayerController` 0))
  (bind (_direction _newtrack_0) (`Timeline|Timeline` :!via `PlayFromStart`)
    (:`Update`
      (`Controller.SetControlRotation` (`GameplayStatics.GetPlayerController` 0) (`KismetMathLibrary.RLerp` (`KismetMathLibrary.MakeRotator` _returnvalue_roll_2 _returnvalue_pitch_2 _returnvalue_yaw_2) (`KismetMathLibrary.MakeRotator` _returnvalue_roll _returnvalue_pitch _returnvalue_yaw) _newtrack_0)))
    (:`Finished`
      (`self.EnableInput` (`GameplayStatics.GetPlayerController` 0)))))

(fn `UserConstructionScript`
  (`parent.UserConstructionScript`))