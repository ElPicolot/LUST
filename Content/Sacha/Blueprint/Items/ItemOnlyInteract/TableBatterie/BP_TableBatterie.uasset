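; BP_TableBatterie is an interactable table that receives a battery item from the player.
; When InteractWorking gets the matching item type, it removes the item from the player's pocket, destroys the held actor and resets the pocket index.
; It spawns a collision-free BP_Batterie at the TargetBatterie transform and sets BatterieOn on Pnj1.
; Disconnected attach, collision-response and NPC message nodes remain unused.
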(event `/Game/Sacha/Interface/BPI_InteractWorking.Interact Working`
  (params (ItemInHand :type "/Game/Sacha/Blueprint/Items/E_MainItemType Enum" :default "NewEnumerator0") (ItemInHandforAnim :type "/Game/Sacha/Blueprint/Items/BP_Item Object Reference") (PlayrRef :type "/Game/Sacha/Blueprint/BP_FirstPersonCharacterSacha Object Reference"))
  (bind _playerref (`self.PlayerRef`))
  (set `self.PlayerRef` PlayrRef)
  (set `self.Item in Handfor Anim` ItemInHandforAnim)
  (if (`|EnumEquality` ItemInHand "NewEnumerator8")
    (`KismetArrayLibrary.Array_RemoveItem` (`/Game/Sacha/Blueprint/BP_FirstPersonCharacterSacha.ItemPocket` _playerref) (`/Game/Sacha/Blueprint/BP_FirstPersonCharacterSacha.ItemInHand` _playerref))
    (`self.K2_DestroyActor` (`self.Item in Handfor Anim`))
    (bind _returnvalue (`|SpawnActorFromClass` "/Game/Sacha/Blueprint/Items/ItemInventory/batterie/BP_Batterie.BP_Batterie_C" (`SceneComponent.K2_GetComponentToWorld` (`self.TargetBatterie`)) "Undefined" "MultiplyWithRoot" null null))
    (`self.SetActorEnableCollision` _returnvalue false)
    (set `/Game/Sacha/Blueprint/BP_FirstPersonCharacterSacha.ItemPocketIndex` 0 (`self.PlayerRef`))
    (set `/Game/Sacha/Blueprint/PNJ/BP_PNJ1.BatterieOn` true (`self.pnj1`))))

(fn `UserConstructionScript`)