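; Interactable security monitor that lets the player view and cycle through a set of security cameras on its screen.
; After a startup delay, it builds a dynamic screen material fed by a render target from the first camera's scene capture.
; Interacting swaps the player to camera input mappings and blends the view to the monitor.
; Switching wraps through cameras, with a timeline animating static noise and moving capture to a new render target scaled by camera quality and viewport size.
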(event `self.ReceiveBeginPlay`
  (`KismetSystemLibrary.Delay` 10.0)
  (`/Engine/EditorBlueprintResources/StandardMacros.IsValid` (`|GetArrayItem` (`self.SecurityCameras`)) :!label _label
    (:`Is Valid`
      (`TimelineComponent.SetPlayRate` (`self.SwitchScreen`) 5.0)
      (bind _returnvalue (`KismetMaterialLibrary.CreateDynamicMaterialInstance` "/Game/Sacha/Blueprint/Items/ItemOnlyInteract/Camera/CameraSecurity_Inst.CameraSecurity_Inst"))
      (bind _output_get (set `self.MonitorMat` _returnvalue))
      (`PrimitiveComponent.SetMaterial` (`self.Monitor`) 0 _output_get)
      (bind _returnvalue_2 (`KismetRenderingLibrary.CreateRenderTarget2D` 256))
      (bind _output_get_2 (set `self.CameraRT` _returnvalue_2))
      (bind _output_get_3 (set `SceneCaptureComponent2D.TextureTarget` _output_get_2 (`/Game/Sacha/Blueprint/Items/ItemOnlyInteract/Camera/BP_CameraSecurity.SceneCaptureComponent2D` (`|GetArrayItem` (`self.SecurityCameras`)))))
      (`MaterialInstanceDynamic.SetTextureParameterValue` (`self.MonitorMat`) "Texture" _output_get_3))
    (:`Is Not Valid`
      (`KismetSystemLibrary.DelayUntilNextTick`)
      (goto _label))))

(event `/Game/Sacha/Interface/BPI_Interact.SwitchInput`
  (params (ActionValuex :type "Float (double-precision)"))
  (bind (_returnvalue_x _returnvalue_y) (`KismetMathLibrary.BreakVector2D` (`WidgetLayoutLibrary.GetViewportSize`)))
  (bind _returnvalue (`KismetArrayLibrary.Array_LastIndex` (`self.SecurityCameras`)))
  (bind _returnvalue_2 (+ (`self.CurrentCamera`) (select `bool` (> ActionValuex 0.0) :`false` -1 :`true` 1)))
  (bind _cameralevelquality (`/Game/Sacha/Blueprint/Items/ItemOnlyInteract/Camera/BP_CameraSecurity.CameraLevelQuality` (`|GetArrayItem` (`self.SecurityCameras`) (`self.CurrentCamera`))))
  (if (not (`self.IsSwitchingCam`))
    (set `self.IsSwitchingCam` true)
    (`KismetSystemLibrary.PrintString` "Hello" true true (struct :`R` 1.0 :`G` 0.04246 :`B` 0.533198 :`A` 1.0))
    (set `self.LastCamera` (`self.CurrentCamera`))
    (set `self.CurrentCamera` (select `bool` (> _returnvalue_2 _returnvalue) :`false` (select `bool` (< _returnvalue_2 0) :`false` _returnvalue_2 :`true` _returnvalue)))
    (bind (_direction _newtrack_0) (`Timeline|SwitchScreen` :!via `PlayFromStart`)
      (:`Update`
        (`MaterialInstanceDynamic.SetScalarParameterValue` (`self.MonitorMat`) "NoisOpacity" (+ (* _newtrack_0 0.5) 0.008)))
      (:`Finished`
        (set `self.IsSwitchingCam` false))
      (:`Switch`
        (set `SceneCaptureComponent2D.TextureTarget` null (`/Game/Sacha/Blueprint/Items/ItemOnlyInteract/Camera/BP_CameraSecurity.SceneCaptureComponent2D` (`|GetArrayItem` (`self.SecurityCameras`) (`self.LastCamera`))))
        (bind _returnvalue_3 (`KismetRenderingLibrary.CreateRenderTarget2D` (`KismetMathLibrary.FTrunc` (* _cameralevelquality _returnvalue_x)) (`KismetMathLibrary.FTrunc` (* _returnvalue_y _cameralevelquality))))
        (bind _output_get (set `self.CameraRT` _returnvalue_3))
        (set `SceneCaptureComponent2D.TextureTarget` _output_get (`/Game/Sacha/Blueprint/Items/ItemOnlyInteract/Camera/BP_CameraSecurity.SceneCaptureComponent2D` (`|GetArrayItem` (`self.SecurityCameras`) (`self.CurrentCamera`))))
        (`MaterialInstanceDynamic.SetTextureParameterValue` (`self.MonitorMat`) "Texture" _output_get)))))

(event `/Game/Sacha/Interface/BPI_Interact.Interact Working`
  (params (ItemInHand :type "/Game/Sacha/Blueprint/Items/E_MainItemType Enum" :default "NewEnumerator0") (ItemInHandforAnim :type "/Game/Sacha/Blueprint/Items/BP_Item Object Reference") (PlayrRef :type "/Game/Sacha/Blueprint/BP_FirstPersonCharacterSacha Object Reference"))
  (bind _returnvalue (pcsubsystem `EnhancedInputLocalPlayerSubsystem` (`GameplayStatics.GetPlayerController` 0)))
  (`KismetSystemLibrary.PrintString` "Hello" true true (struct :`R` 0.364498 :`B` 1.0 :`A` 1.0))
  (set `/Game/Sacha/Blueprint/BP_FirstPersonCharacterSacha.OnCam` true PlayrRef)
  (`/Engine/EditorBlueprintResources/StandardMacros.IsValid` _returnvalue
    (:`Is Valid`
      (`EnhancedInputSubsystemInterface.RemoveMappingContext` _returnvalue "/Game/Sacha/Input/IMC_Sacha.IMC_Sacha" (struct))
      (`EnhancedInputSubsystemInterface.AddMappingContext` _returnvalue "/Game/Sacha/Input/IMC_Camera.IMC_Camera" 1 (struct))
      (`PlayerController.SetViewTargetWithBlend` (`GameplayStatics.GetPlayerController` 0) self 1.0 "VTBlend_Linear" 0.0 false)
      (`self.EnableInput` PlayrRef (`GameplayStatics.GetPlayerController` 0)))))

(fn `UserConstructionScript`)