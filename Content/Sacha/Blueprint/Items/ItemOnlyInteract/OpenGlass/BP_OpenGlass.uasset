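; BP_OpenGlass is an interact-only glass display cabinet (vitrine) that opens to give the player access to the whip (Fouet).
; InteractWorking fires once, clearing the player's ShowVitrine flag, enabling CanGrabFouet and playing the opening sound.
; It switches both cabinet meshes to WorldStatic and the whip mesh to a custom collision channel.
; A timeline then swings StaticMesh1 open by interpolating its relative yaw.
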(event `/Game/Sacha/Interface/BPI_InteractWorking.Interact Working`
  (params (ItemInHand :type "/Game/Sacha/Blueprint/Items/E_MainItemType Enum" :default "NewEnumerator0") (ItemInHandforAnim :type "/Game/Sacha/Blueprint/Items/BP_Item Object Reference") (PlayrRef :type "/Game/Sacha/Blueprint/BP_FirstPersonCharacterSacha Object Reference"))
  (`/Engine/EditorBlueprintResources/StandardMacros.DoOnce` false
    (:`Completed`
      (set `/Game/Sacha/Blueprint/BP_FirstPersonCharacterSacha.ShowVitrine` false PlayrRef)
      (`PrimitiveComponent.SetCollisionObjectType` (`self.StaticMesh`) "ECC_WorldStatic")
      (`PrimitiveComponent.SetCollisionObjectType` (`self.StaticMesh1`) "ECC_WorldStatic")
      (`GameplayStatics.PlaySoundAtLocation` "/Game/Sounds/Audio_Effect/Cabinet_Open.Cabinet_Open" (`self.K2_GetActorLocation`) (struct) 1.0 1.0 0.0 null null null null)
      (set `/Game/Sacha/Blueprint/BP_FirstPersonCharacterSacha.CanGrabFouet` true PlayrRef)
      (`PrimitiveComponent.SetCollisionObjectType` (`/Game/Sacha/Blueprint/Items/BP_Item.StaticMesh` (`self.fouet`)) "ECC_GameTraceChannel2")
      (bind (_direction _newtrack_0) (`Timeline|Timeline` :!via `PlayFromStart`)
        (:`Update`
          (`SceneComponent.K2_SetRelativeRotation` (`self.StaticMesh1`) (`KismetMathLibrary.MakeRotator` 0.0 0.0 (`KismetMathLibrary.Lerp` 15.0 110.0 _newtrack_0)) false false))))))

(fn `UserConstructionScript`)