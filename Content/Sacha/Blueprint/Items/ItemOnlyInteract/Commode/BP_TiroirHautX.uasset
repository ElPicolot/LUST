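; Interactable commode drawer that slides open or closed along the world X axis when grabbed.
; GrabItem alternates through a FlipFlop, playing a sound and running the MoveTiroir timeline forward or backward to lerp the root's position, with IsOpening blocking input during movement.
; BeginPlay caches the start position and sets the travel direction from Inverse.
; The construction script adds the drawer mesh, raised slightly when TiroirHaut is set.
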(event `self.ReceiveBeginPlay`
  (bind _output_get (set `self.InitialLocationV` (`SceneComponent.K2_GetComponentLocation` (`self.DefaultSceneRoot`))))
  (bind _output_get_2 (set `self.InitialLocation` (.x _output_get)))
  (set `self.TargetLocation` (+ _output_get_2 (select `bool` (`self.Inverse`) :`false` 35.0 :`true` -35.0))))

(event `self.GrabItem`
  (params (PlayerRef :type "/Game/Sacha/Blueprint/BP_FirstPersonCharacterSacha Object Reference"))
  (bind (_initiallocationv_x _initiallocationv_y _initiallocationv_z) (`KismetMathLibrary.BreakVector` (`self.InitialLocationV`)))
  (if (not (`self.IsOpening`))
    (set `self.IsOpening` true)
    (`/Engine/EditorBlueprintResources/StandardMacros.FlipFlop`
      (:`A`
        (`GameplayStatics.PlaySoundAtLocation` "/Game/Sounds/SFX/Drawer_Open.Drawer_Open" (`SceneComponent.K2_GetComponentLocation` (`self.Audio_OpenDrawer`)) (struct) 0.3 1.0 0.0 null null null null)
        (bind (_direction _newtrack_0) (`Timeline|MoveTiroir` :!via `PlayFromStart` :!label _label)
          (:`Update`
            (`SceneComponent.K2_SetWorldLocation` (`self.DefaultSceneRoot`) (`KismetMathLibrary.MakeVector` (`KismetMathLibrary.Lerp` (`self.InitialLocation`) (`self.TargetLocation`) _newtrack_0) _initiallocationv_y _initiallocationv_z) false false))
          (:`Finished`
            (set `self.IsOpening` false))))
      (:`B`
        (`GameplayStatics.PlaySoundAtLocation` "/Game/Sounds/SFX/Drawer_Open.Drawer_Open" (`SceneComponent.K2_GetComponentLocation` (`self.Audio_OpenDrawer`)) (struct) 0.3 1.0 0.0 null null null null)
        (goto _label :!via `ReverseFromEnd`)))))

(fn `UserConstructionScript`
  (if (`self.TiroirHaut?`)
    (bind _returnvalue (`AddComponent|NODE_AddStaticMeshComponent-0` :`RelativeTransform` (`KismetMathLibrary.MakeTransform` (0.0 0.0 4.0) (struct) (1.0 1.5 1.0))))
    (set `self.ItemStaticMesh` _returnvalue)
    (else
      (bind _returnvalue_2 (`AddComponent|NODE_AddStaticMeshComponent-1` :`RelativeTransform` (`KismetMathLibrary.MakeTransform` (0.0 0.0 0.0) (struct) (1.0 1.5 1.0))))
      (set `self.ItemStaticMesh` _returnvalue_2))))