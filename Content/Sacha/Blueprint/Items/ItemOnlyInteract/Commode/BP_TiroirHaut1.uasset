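; Interactive dresser drawer (tiroir) that slides open or closed along its relative X axis when the GrabItem event fires.
; BeginPlay caches the closed position and offset target, then a FlipFlop alternates the MoveTiroir timeline forward and reverse to lerp the root.
; An IsOpening flag blocks retriggering until the timeline finishes.
; The construction script adds a mesh variant chosen by TiroirHaut and five box components forming an open-topped tray.
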(event `self.ReceiveBeginPlay`
  (bind _output_get (set `self.InitialLocationV` (`SceneComponent.RelativeLocation` (`self.DefaultSceneRoot`))))
  (bind _output_get_2 (set `self.InitialLocation` (.x _output_get)))
  (set `self.TargetLocation` (- _output_get_2 -35.0)))

(event `self.GrabItem`
  (params (PlayerRef :type "/Game/Sacha/Blueprint/BP_FirstPersonCharacterSacha Object Reference"))
  (bind (_initiallocationv_x _initiallocationv_y _initiallocationv_z) (`KismetMathLibrary.BreakVector` (`self.InitialLocationV`)))
  (if (not (`self.IsOpening`))
    (set `self.IsOpening` true)
    (`/Engine/EditorBlueprintResources/StandardMacros.FlipFlop`
      (:`A`
        (bind (_direction _newtrack_0) (`Timeline|MoveTiroir` :!via `PlayFromStart` :!label _label)
          (:`Update`
            (`SceneComponent.K2_SetRelativeLocation` (`self.DefaultSceneRoot`) (`KismetMathLibrary.MakeVector` (`KismetMathLibrary.Lerp` (`self.InitialLocation`) (`self.TargetLocation`) _newtrack_0) _initiallocationv_y _initiallocationv_z) false false))
          (:`Finished`
            (set `self.IsOpening` false))))
      (:`B`
        (goto _label :!via `ReverseFromEnd`)))))

(fn `UserConstructionScript`
  (if (`self.TiroirHaut?`)
    (bind _returnvalue (`AddComponent|NODE_AddStaticMeshComponent-0` :`RelativeTransform` (`KismetMathLibrary.MakeTransform` (0.0 0.0 4.0))))
    (set `self.ItemStaticMesh` _returnvalue)
    (else
      (bind _returnvalue_2 (`AddComponent|NODE_AddStaticMeshComponent-1`))
      (set `self.ItemStaticMesh` _returnvalue_2)))
  (`AddComponent|NODE_AddBoxComponent-0` :`RelativeTransform` (`KismetMathLibrary.MakeTransform` (0.0 0.0 6.0) (struct) (1.5 0.05 0.3)))
  (`AddComponent|NODE_AddBoxComponent-1` :`RelativeTransform` (`KismetMathLibrary.MakeTransform` (50.0 20.0 6.0) (struct) (0.05 0.5 0.3)))
  (`AddComponent|NODE_AddBoxComponent-2` :`RelativeTransform` (`KismetMathLibrary.MakeTransform` (-50.0 20.0 6.0) (struct) (0.05 0.5 0.3)))
  (`AddComponent|NODE_AddBoxComponent-3` :`RelativeTransform` (`KismetMathLibrary.MakeTransform` (0.0 42.0 6.0) (struct) (1.5 0.05 0.3)))
  (`AddComponent|NODE_AddBoxComponent-4` :`RelativeTransform` (`KismetMathLibrary.MakeTransform` (0.0 20.0 -5.0) (struct) (1.5 0.5 0.05))))