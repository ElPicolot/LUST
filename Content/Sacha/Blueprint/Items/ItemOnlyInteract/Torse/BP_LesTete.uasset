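; BP_LesTete is an interact-only item, the heads, whose successful interaction triggers a moving armoire.
; InteractWorking stops the timeline on the passed in-hand item, fires the moving event on the referenced armoire and calls UpPainMessage on BPPain.
; It then replaces CanInteractWith with a single false entry, switching off that interaction.
; Other graph events are disabled stubs, and construction only calls the parent.
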(event `/Game/Sacha/Interface/BPI_Interact.Interact Working`
  (params (ItemInHand :type "/Game/Sacha/Blueprint/Items/E_MainItemType Enum" :default "NewEnumerator0") (ItemInHandforAnim :type "/Game/Sacha/Blueprint/Items/BP_Item Object Reference") (PlayrRef :type "/Game/Sacha/Blueprint/BP_FirstPersonCharacterSacha Object Reference"))
  (`/Game/Sacha/Blueprint/Items/BP_Item.EventStopTimeline` ItemInHandforAnim)
  (`/Game/Sacha/Blueprint/Items/ItemOnlyInteract/ArmoireMoving/BP_ArmoireMoving.EventMovingArmoire` (`self.BPArmoireMoving`))
  (message `/Game/Sacha/Interface/BPI_Interact.UpPain` (`self.BPPain`) 21.0)
  (set `self.CanInteractWith?` (`|MakeMap` "NewEnumerator0" :!type "/Game/Sacha/Blueprint/Items/E_MainItemType Enum")))

(fn `UserConstructionScript`
  (`parent.UserConstructionScript`))