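; BP_Goutiere is a gutter item that, on its first whip interaction, releases a waterfall and moves a water mesh vertically.
; The interaction spawns a FS_MasterFieldGoutiere field actor at the static mesh, computes a target height and starts a looping timer.
; The waterfall activates after a short delay.
; The timer steps the water at constant speed, then stops itself and deactivates the waterfall when movement completes.
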(event `self.ReceiveBeginPlay`
  (`parent.ReceiveBeginPlay`)
  (set `self.ItemType` (`self.ItemType`))
  (set `self.CanIteractWith` "NewEnumerator2")
  (`ActorComponent.SetActive` (`self.WaterFall`) false false)
  (`KismetSystemLibrary.PrintString` "waterfall not active"))

(event `self.ReceiveActorBeginOverlap`
  (params (OtherActor :type "Actor Object Reference"))
  (`parent.ReceiveActorBeginOverlap` OtherActor))

(event `self.ReceiveTick`
  (params (DeltaSeconds :type "Float (single-precision)"))
  (`parent.ReceiveTick` DeltaSeconds))

(event `/Game/Sacha/Interface/BPI_Whip.InteractWithWhipe`
  (`/Engine/EditorBlueprintResources/StandardMacros.DoOnce` false
    (:`Completed`
      (`|SpawnActorFromClass` "/Game/Sacha/Blueprint/Items/ItemOnlyInteract/Goutiere/FS_MasterFieldGoutiere.FS_MasterFieldGoutiere_C" (`KismetMathLibrary.MakeTransform` (`SceneComponent.K2_GetComponentLocation` (`self.StaticMesh`))) "Undefined" "MultiplyWithRoot" null null)
      (bind _targetpositionz (`self.Set Mesh Move Z` (`self.Water`) (`self.PositionOffset`)))
      (set `self.TargetLocationZ` _targetpositionz)
      (bind _returnvalue (`KismetSystemLibrary.K2_SetTimerDelegate` (delegate `UP_Water`) 0.02 true))
      (set `self.AvtivateGoutiereHandle` _returnvalue)
      (`KismetSystemLibrary.Delay` 0.2)
      (`ActorComponent.SetActive` (`self.WaterFall`) true false))))

(event `UP_Water`
  (bind _stopmovez (`self.GoMeshMoveZ` (`self.Water`) (`self.TargetLocationZ`) 2.0 true (`self.PositionOffset`)))
  (if _stopmovez
    (`ActorComponent.SetActive` (`self.WaterFall`) false false)
    (`KismetSystemLibrary.K2_ClearAndInvalidateTimerHandle` (`self.AvtivateGoutiereHandle`))))

(fn `UserConstructionScript`)