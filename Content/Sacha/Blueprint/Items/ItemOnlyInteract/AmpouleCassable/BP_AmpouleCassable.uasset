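; Breakable light bulb interactable that can trigger an electrocution failure when it falls while the bath is filled.
; On interaction it enables mesh physics, waits briefly, then checks BPBath's WaterUp flag.
; With water up, it prints LOSE, plays the bath's electrocution animation and sounds, then shows a scolding subtitle with voice and calls BPDoorMonster's monster message.
; Otherwise it switches off the point light and plays a smash sound.
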(event `self.ReceiveBeginPlay`
  (set `self.As BP First Person Character Sacha` (cast `/Game/Sacha/Blueprint/BP_FirstPersonCharacterSacha` (`GameplayStatics.GetPlayerCharacter` 0) :!pure true)))

(event `/Game/Sacha/Interface/BPI_Interact.Interact Working`
  (params (ItemInHand :type "/Game/Sacha/Blueprint/Items/E_MainItemType Enum" :default "NewEnumerator0") (ItemInHandforAnim :type "/Game/Sacha/Blueprint/Items/BP_Item Object Reference") (PlayrRef :type "/Game/Sacha/Blueprint/BP_FirstPersonCharacterSacha Object Reference"))
  (`PrimitiveComponent.SetSimulatePhysics` (`self.StaticMesh`) true)
  (`KismetSystemLibrary.Delay` 0.3)
  (if (`/Game/Sacha/Blueprint/Items/ItemOnlyInteract/Bathtub/BP_Bath.WaterUp` (`self.BPBath`))
    (`GameplayStatics.SpawnSoundAtLocation` "/Game/Sounds/SFX/Plouf.Plouf" (0.0 0.0 0.0) (struct) 1.0 1.0 0.0 null null)
    (`KismetSystemLibrary.PrintString` "LOSE")
    (`SkeletalMeshComponent.PlayAnimation` (`/Game/Sacha/Blueprint/Items/ItemOnlyInteract/Bathtub/BP_Bath.SkeletalMeshBaignoire` (`self.BPBath`)) "/Game/Animation/Baignoire/Electrocution.Electrocution" false)
    (`GameplayStatics.SpawnSoundAtLocation` "/Game/Sounds/SFX/BZZZZ_2.BZZZZ_2" (0.0 0.0 0.0) (struct) 1.0 1.0 0.0 null null)
    (`KismetSystemLibrary.Delay` 2.0)
    (`/Game/Sacha/Winget/WB_SousTitre.EventSousTitrewinget` (`/Game/Sacha/Blueprint/BP_FirstPersonCharacterSacha.WingetSousTitre` (`self.As BP First Person Character Sacha`)) "What did I said ??!  \nNaughty girl get's punish")
    (`GameplayStatics.PlaySoundAtLocation` "/Game/Sounds/Antagonist_Dialogue_Final/21_Naughty_Girl.21_Naughty_Girl" (`self.K2_GetActorLocation`) (struct) 1.0 1.0 0.0 null null null null)
    (message `/Game/Sacha/Interface/BPI_Interact.CallMonster` (`self.BPDoorMonster`))
    (else
      (`LightComponent.SetIntensity` (`self.PointLight`) 0.0)
      (`GameplayStatics.SpawnSoundAtLocation` "/Game/Sounds/SFX/LightBulb_Smash2.LightBulb_Smash2" (0.0 0.0 0.0) (struct) 1.0 1.0 0.0 null null))))

(fn `UserConstructionScript`
  (`parent.UserConstructionScript`))