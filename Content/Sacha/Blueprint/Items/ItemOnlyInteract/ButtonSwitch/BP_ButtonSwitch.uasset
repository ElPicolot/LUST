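; BP_ButtonSwitch is an interact-only item Blueprint whose own graph holds no switch logic, only a camera-turn event and parent calls.
; RotateCameraOnPNJ disables player input, then runs a timeline that turns the control rotation toward a given actor.
; Each update lerps from the player's current root rotation to the look-at rotation, re-reading both rather than caching the start.
; Input is re-enabled when the timeline finishes.
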(event `self.ReceiveBeginPlay`
  (`parent.ReceiveBeginPlay`))

(event `RotateCameraOnPNJ`
  (params (PlayerRef :type "/Game/Sacha/Blueprint/BP_FirstPersonCharacterSacha Object Reference") (ActorToLook :type "Actor Object Reference"))
  (bind (_returnvalue_roll _returnvalue_pitch _returnvalue_yaw) (`KismetMathLibrary.BreakRotator` (`KismetMathLibrary.FindLookAtRotation` (`self.K2_GetActorLocation` PlayerRef) (`self.K2_GetActorLocation` ActorToLook))))
  (bind (_returnvalue_roll_2 _returnvalue_pitch_2 _returnvalue_yaw_2) (`KismetMathLibrary.BreakRotator` (`SceneComponent.K2_GetComponentRotation` (`Actor.RootComponent` PlayerRef))))
  (`self.DisableInput` PlayerRef (`GameplayStatics.GetPlayerController` 0))
  (bind (_direction _newtrack_0) (`Timeline|Timeline` :!via `PlayFromStart`)
    (:`Update`
      (`Controller.SetControlRotation` (`GameplayStatics.GetPlayerController` 0) (`KismetMathLibrary.RLerp` (`KismetMathLibrary.MakeRotator` _returnvalue_roll_2 _returnvalue_pitch_2 _returnvalue_yaw_2) (`KismetMathLibrary.MakeRotator` _returnvalue_roll _returnvalue_pitch _returnvalue_yaw) _newtrack_0)))
    (:`Finished`
      (`self.EnableInput` PlayerRef (`GameplayStatics.GetPlayerController` 0)))))

(fn `UserConstructionScript`
  (`parent.UserConstructionScript`))