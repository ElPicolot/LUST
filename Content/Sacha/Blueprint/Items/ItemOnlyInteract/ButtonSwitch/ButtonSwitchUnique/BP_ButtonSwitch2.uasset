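; One-off puzzle switch, struck with a held item to a whip sound, that escalates over three activations.
; CallMonster arms it and SwitchInput disarms it; each accepted hit disarms it and messages the culprits (Cul1, Cul3).
; The first two hits turn the camera to an NPC, play reactions, move ropes and notify the Puzzle.
; The third summons the door monster, disables input, fades and opens the tutorial level.
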(event `self.ReceiveBeginPlay`
  (`parent.ReceiveBeginPlay`)
  (set `self.OriginalMat` (`PrimitiveComponent.GetMaterial` (`self.StaticMesh`) 0)))

(event `/Game/Sacha/Interface/BPI_InteractWorking.Interact Working`
  (params (ItemInHand :type "/Game/Sacha/Blueprint/Items/E_MainItemType Enum" :default "NewEnumerator0") (ItemInHandforAnim :type "/Game/Sacha/Blueprint/Items/BP_Item Object Reference") (PlayrRef :type "/Game/Sacha/Blueprint/BP_FirstPersonCharacterSacha Object Reference"))
  (if (and (`|EnumEquality` ItemInHand "NewEnumerator1") (`self.CanBeKick`))
    (for _array_element (`/Game/Sacha/Blueprint/Puzzle/PictoMove/BP_PictoMove.MatInstArray` (`self.Puzzle`))
      (`MaterialInstanceDynamic.SetScalarParameterValue` _array_element "IsHide" 0.0))
    (set `self.CanBeKick` false)
    (message `/Game/Sacha/Interface/BPI_InteractWorking.SwitchInput` (`self.Cul1`) 0.0)
    (message `/Game/Sacha/Interface/BPI_InteractWorking.SwitchInput` (`self.Cul3`) 0.0)
    (set `self.Playr Ref` PlayrRef)
    (if (`self.CanBeUse`)
      (if (not (`self.IsMoving`))
        (set `self.IsMoving` true)
        (`/Engine/EditorBlueprintResources/StandardMacros.IncrementInt` (`self.NumberofActivation`)
          (:`  `
            (`self.SetAndPlaySound` "/Game/Sounds/SFX/Fouet_Coup.Fouet_Coup" (`self.Audio1`))
            (switch `int` (`self.NumberofActivation`)
              (:`1`
                (`self.RotateCameraOnPNJ` (`self.Playr Ref`) (`self.PNJ1`))
                (`PrimitiveComponent.SetMaterial` (`self.StaticMesh`) 0 "/AnimationSharing/AnimSharingGreen.AnimSharingGreen")
                (message `/Game/Sacha/Interface/BPI_InteractWorking.UpPain` (`self.BP_Pain`) 5.0)
                (`/Game/Sacha/Winget/WB_SousTitre.EventSousTitrewinget` (`/Game/Sacha/Blueprint/BP_FirstPersonCharacterSacha.WingetSousTitre` (`self.Playr Ref`)) "YES that's it... that's how you do it")
                (message `/Game/Sacha/Interface/BPI_InteractWorking.PlaySound` (`self.PNJ1`) "/Game/Sounds/SFX/Homme_Baillon.Homme_Baillon" 0.0)
                (message `/Game/Sacha/Interface/BPI_InteractWorking.PlaySound` (`self.Chaine`) "/Game/Sounds/SFX/Chain_Cran.Chain_Cran" 0.0)
                (`KismetSystemLibrary.Delay` 1.0)
                (`PrimitiveComponent.SetMaterial` (`self.StaticMesh`) 0 (`self.OriginalMat`))
                (set `self.IsMoving` false :!label _label)
                (for _array_element_2 (`self.BPcordeMove`)
                  (message `/Game/Sacha/Interface/BPI_InteractWorking.SwitchInput` _array_element_2 (`self.Corde Speed`)))
                (message `/Game/Sacha/Interface/BPI_InteractWorking.InteractBetweenItem` (`self.Puzzle`)))
              (:`2`
                (`self.RotateCameraOnPNJ` (`self.Playr Ref`) (`self.PNJ1`))
                (`PrimitiveComponent.SetMaterial` (`self.StaticMesh`) 0 "/AnimationSharing/AnimSharingGreen.AnimSharingGreen")
                (message `/Game/Sacha/Interface/BPI_InteractWorking.PlaySound` (`self.PNJ1`) "/Game/Sounds/SFX/Homme_Baillon_1.Homme_Baillon_1" 0.0)
                (`/Game/Sacha/Winget/WB_SousTitre.EventSousTitrewinget` (`/Game/Sacha/Blueprint/BP_FirstPersonCharacterSacha.WingetSousTitre` (`self.Playr Ref`)) "Careful now darling... Don't be too greedy now...")
                (message `/Game/Sacha/Interface/BPI_InteractWorking.PlaySound` (`self.Speaker`) "/Game/Sounds/SFX/Antago_STOP_02.Antago_STOP_02" 0.0)
                (message `/Game/Sacha/Interface/BPI_InteractWorking.PlaySound` (`self.Chaine`) "/Game/Sounds/SFX/Chain_Cran.Chain_Cran" 0.0)
                (`KismetSystemLibrary.Delay` 1.0)
                (`PrimitiveComponent.SetMaterial` (`self.StaticMesh`) 0 (`self.OriginalMat`))
                (goto _label))
              (:`3`
                (`self.RotateCameraOnPNJ` (`self.Playr Ref`) (`self.BPDoorMonster`))
                (`PrimitiveComponent.SetMaterial` (`self.StaticMesh`) 0 "/AnimationSharing/AnimSharingRed.AnimSharingRed")
                (message `/Game/Sacha/Interface/BPI_InteractWorking.CallMonster` (`self.BPDoorMonster`))
                (`/Game/Sacha/Winget/WB_SousTitre.EventSousTitrewinget` (`/Game/Sacha/Blueprint/BP_FirstPersonCharacterSacha.WingetSousTitre` (`self.Playr Ref`)) "I TOLD YOU TO BE CAREFUL!  BLASPHEMY !")
                ;[1 0.01967 0.7901] Son de Mort a setup
                (message `/Game/Sacha/Interface/BPI_InteractWorking.PlaySound` (`self.Speaker`) "/Game/Sounds/SFX/Antago_STOP_02.Antago_STOP_02" 0.0)
                (message `/Game/Sacha/Interface/BPI_InteractWorking.PlaySound` (`self.PNJ1`) "/Game/Sounds/SFX/Homme_Baillon_1.Homme_Baillon_1" 0.0)
                (message `/Game/Sacha/Interface/BPI_InteractWorking.PlaySound` (`self.Chaine`) "/Game/Sounds/SFX/Chain_Cran.Chain_Cran" 0.0)
                (`KismetSystemLibrary.Delay` 1.0)
                (`PrimitiveComponent.SetMaterial` (`self.StaticMesh`) 0 (`self.OriginalMat`))
                ;[1 1 1] A enlever et reconnecter au set d'en haut / test pour build
                (`self.DisableInput` null)
                (`/Game/Sacha/Winget/WB_Fades.FadeIn` (`self.WBFades`))
                (`KismetSystemLibrary.Delay` 10.0)
                (`GameplayStatics.OpenLevelBySoftObjectPtr` "/Game/LD/Salle_Tutoriel_01.Salle_Tutoriel_01")))))))))

(event `/Game/Sacha/Interface/BPI_InteractWorking.CallMonster`
  (set `self.CanBeKick` true))

(event `/Game/Sacha/Interface/BPI_InteractWorking.SwitchInput`
  (params (ActionValuex :type "Float (double-precision)"))
  (set `self.CanBeKick` false))

(fn `UserConstructionScript`
  (`parent.UserConstructionScript`))