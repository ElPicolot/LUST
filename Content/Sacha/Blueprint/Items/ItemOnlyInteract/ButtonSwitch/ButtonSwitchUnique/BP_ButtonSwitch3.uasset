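; BP_ButtonSwitch3 is a one-off interactable button that triggers a scripted scene involving an NPC and the monster door.
; InteractWorking checks the held item type and fires once, turning the button's material green and rotating the player's camera onto BPDoorMonster.
; It enables physics on PNJ1's mesh, plays a whip sound, then after a short delay plays a gagged-man sound and calls the door's monster message.
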(event `/Game/Sacha/Interface/BPI_InteractWorking.Interact Working`
  (params (ItemInHand :type "/Game/Sacha/Blueprint/Items/E_MainItemType Enum" :default "NewEnumerator0") (ItemInHandforAnim :type "/Game/Sacha/Blueprint/Items/BP_Item Object Reference") (PlayrRef :type "/Game/Sacha/Blueprint/BP_FirstPersonCharacterSacha Object Reference"))
  (if (`|EnumEquality` ItemInHand "NewEnumerator1")
    (`/Engine/EditorBlueprintResources/StandardMacros.DoOnce` false
      (:`Completed`
        (`PrimitiveComponent.SetMaterial` (`self.StaticMesh`) 0 "/AnimationSharing/AnimSharingGreen.AnimSharingGreen")
        (`self.RotateCameraOnPNJ` PlayrRef (`self.BP_DoorMonster`))
        (`PrimitiveComponent.SetSimulatePhysics` (`/Game/Sacha/Blueprint/Items/BP_Interaction.StaticMesh` (`self.PNJ1`)) true)
        (message `/Game/Sacha/Interface/BPI_InteractWorking.PlaySound` (`self.Speaker`) "/Game/Sounds/SFX/Fouet_Coup.Fouet_Coup" 0.0)
        (`KismetSystemLibrary.Delay` 1.0)
        (message `/Game/Sacha/Interface/BPI_InteractWorking.PlaySound` (`self.Speaker`) "/Game/Sounds/SFX/Homme_Baillon_2.Homme_Baillon_2" 0.0)
        (message `/Game/Sacha/Interface/BPI_InteractWorking.CallMonster` (`self.BP_DoorMonster`))))))

(fn `UserConstructionScript`
  (`parent.UserConstructionScript`))