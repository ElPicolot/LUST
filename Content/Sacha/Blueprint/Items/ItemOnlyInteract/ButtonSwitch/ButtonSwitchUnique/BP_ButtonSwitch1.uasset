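; Puzzle switch that, while armed by CallMonster, lowers a linked NPC (PNJ1) one step per interaction and raises the PainDoor's pain level.
; Each use turns the camera to the NPC, plays whip and chain sounds, runs the ropes, and moves the NPC's mesh on a looping timer until it stops and notifies the puzzle.
; Pain is higher if the candle burns; the final activation marks the NPC down and triggers the candle if unlit.
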(event `self.ReceiveBeginPlay`
  (`parent.ReceiveBeginPlay`)
  (set `self.InitialMat` (`PrimitiveComponent.GetMaterial` (`self.StaticMesh`) 0)))

(event `/Game/Sacha/Interface/BPI_InteractWorking.Interact Working`
  (params (ItemInHand :type "/Game/Sacha/Blueprint/Items/E_MainItemType Enum" :default "NewEnumerator0") (ItemInHandforAnim :type "/Game/Sacha/Blueprint/Items/BP_Item Object Reference") (PlayrRef :type "/Game/Sacha/Blueprint/BP_FirstPersonCharacterSacha Object Reference"))
  (if (and (`|EnumEquality` ItemInHand "NewEnumerator1") (`self.CanBeKick`))
    (for _array_element (`/Game/Sacha/Blueprint/Puzzle/PictoMove/BP_PictoMove.MatInstArray` (`self.Puzzle`))
      (`MaterialInstanceDynamic.SetScalarParameterValue` _array_element "IsHide" 0.0))
    (set `self.CanBeKick` false)
    (message `/Game/Sacha/Interface/BPI_InteractWorking.SwitchInput` (`self.Cul2`) 0.0)
    (message `/Game/Sacha/Interface/BPI_InteractWorking.SwitchInput` (`self.Cul3`) 0.0)
    (set `self.Playr Ref` PlayrRef)
    (if (`self.CanBeUse`)
      (if (not (`self.IsMoving`))
        (if (== (`self.Numberof Activation`) 0)
          (`/Game/Sacha/Winget/WB_SousTitre.EventSousTitrewinget` (`/Game/Sacha/Blueprint/BP_FirstPersonCharacterSacha.WingetSousTitre` (`self.Playr Ref`)) "That's it... keep going"))
        (set `self.IsMoving` true)
        (`self.RotateCameraOnPNJ` (`self.Playr Ref`) (`self.PNJ1`))
        (`/Engine/EditorBlueprintResources/StandardMacros.IncrementInt` (`self.Numberof Activation`)
          (:`  `
            (if (<= (`self.Numberof Activation`) (`self.ActivationMax`))
              (`PrimitiveComponent.SetMaterial` (`self.StaticMesh`) 0 "/AnimationSharing/AnimSharingGreen.AnimSharingGreen")
              ;[0 0.25 1] Si on le met , l'autre son se joue trop tard
              (`self.SetAndPlaySound` "/Game/Sounds/SFX/Fouet_Coup.Fouet_Coup" (`self.Audio1`))
              (message `/Game/Sacha/Interface/BPI_InteractWorking.PlaySound` (`self.Chaine`) "/Game/Sounds/SFX/Chaine_Tiree.Chaine_Tiree" 1.0)
              (bind _targetpositionz (`self.Set Mesh Move Z` (`/Game/Sacha/Blueprint/Items/BP_Interaction.StaticMesh` (`self.PNJ1`)) (`self.Offset Position`)))
              (set `self.Target Position Z` _targetpositionz)
              (`self.PainIfCandleBurn`)
              (message `/Game/Sacha/Interface/BPI_InteractWorking.UpPain` (`self.PainDoor`) (`self.Pain P`))
              (bind _returnvalue (`KismetSystemLibrary.K2_SetTimerDelegate` (delegate `DownBody`) 0.05 true))
              (set `self.LocationHandle` _returnvalue)
              (for _array_element_2 (`self.BPcordeMove`)
                (message `/Game/Sacha/Interface/BPI_InteractWorking.SwitchInput` _array_element_2 (`self.CordeSpeed`))))))))))

(event `DownBody`
  (bind _stopmovez (`self.GoMeshMoveZ` (`/Game/Sacha/Blueprint/Items/BP_Interaction.StaticMesh` (`self.PNJ1`)) (`self.Target Position Z`) 30.0 true (`self.Offset Position`)))
  (bind _output_get (set `self.Stop Move Z` _stopmovez))
  (if _output_get
    (for _array_element (`self.BPcordeMove`)
      (message `/Game/Sacha/Interface/BPI_InteractWorking.SwitchInput` _array_element 0.0))
    (message `/Game/Sacha/Interface/BPI_InteractWorking.InteractBetweenItem` (`self.Chaine`))
    (`PrimitiveComponent.SetMaterial` (`self.StaticMesh`) 0 (`self.InitialMat`))
    (set `self.IsMoving` false)
    (message `/Game/Sacha/Interface/BPI_InteractWorking.InteractBetweenItem` (`self.Puzzle`))
    (if (== (`self.Numberof Activation`) (`self.ActivationMax`))
      (set `self.CanBeUse` false)
      (set `/Game/Sacha/Blueprint/PNJ/BP_PNJ1.PNJIsDown` true (`self.PNJ1`))
      (if (`self.CandleBurning`)
        (`KismetSystemLibrary.K2_ClearAndInvalidateTimerHandle` (`self.LocationHandle`))
        (else
          (message `/Game/Sacha/Interface/BPI_InteractWorking.InteractBetweenItem` (`self.BPCandle`))
          (`KismetSystemLibrary.K2_ClearAndInvalidateTimerHandle` (`self.LocationHandle`))))
      (else
        (`KismetSystemLibrary.K2_ClearAndInvalidateTimerHandle` (`self.LocationHandle`))))))

(event `/Game/Sacha/Interface/BPI_InteractWorking.InteractBetweenItem`
  (set `self.CandleBurning` true))

(event `PainIfCandleBurn`
  (if (`self.CandleBurning`)
    (set `self.Pain P` 17.0)
    (else
      (set `self.Pain P` 14.0))))

(event `/Game/Sacha/Interface/BPI_InteractWorking.CallMonster`
  (set `self.CanBeKick` true))

(event `/Game/Sacha/Interface/BPI_InteractWorking.SwitchInput`
  (params (ActionValuex :type "Float (double-precision)"))
  (set `self.CanBeKick` false))

(fn `Pain`
  (params (PainP :type "Float (double-precision)" :default 0.0))
  (returns (Pain :type "Float (double-precision)"))
  (return (/ PainP 50.0)))

(fn `UserConstructionScript`
  (`parent.UserConstructionScript`))