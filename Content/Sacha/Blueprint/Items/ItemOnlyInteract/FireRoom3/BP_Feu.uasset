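; BP_Feu is an interactable fire that the player builds from a Log and a Cloth, then ignites with a Lighter.
; InteractWorking branches on the held item, setting attachment flags and enabling CanBurn after a grab montage once both are present.
; If CanBurn, the lighter montage ends by activating the Niagara effect and calling UpPainMessage.
; Each item disables input until its montage completes, but a Lighter used before CanBurn never re-enables it.
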(event `self.ReceiveBeginPlay`
  (`ActorComponent.SetActive` (`self.Niagara`) false false))

(event `/Game/Sacha/Interface/BPI_InteractWorking.Interact Working`
  (params (ItemInHand :type "/Game/Sacha/Blueprint/Items/E_MainItemType Enum" :default "NewEnumerator0") (ItemInHandforAnim :type "/Game/Sacha/Blueprint/Items/BP_Item Object Reference") (PlayrRef :type "/Game/Sacha/Blueprint/BP_FirstPersonCharacterSacha Object Reference"))
  (switch `/Game/Sacha/Blueprint/Items/E_MainItemType` ItemInHand
    (:`NewEnumerator2`
      (`self.DisableInput` (`GameplayStatics.GetPlayerController` 0))
      (if (`self.CanBurn`)
        (`|PlayMontage` null "/Game/Sacha/FirstPersonArmSacha/Annimation/Ligter_CandleAnimation_Montage.Ligter_CandleAnimation_Montage"
          (:`OnCompleted`
            (`self.EnableInput` (`GameplayStatics.GetPlayerController` 0))
            (`ActorComponent.SetActive` (`self.Niagara`) true false)
            (message `/Game/Sacha/Interface/BPI_InteractWorking.UpPain` (`self.Pain`) 40.0)))))
    (:`NewEnumerator6`
      (`self.DisableInput` (`GameplayStatics.GetPlayerController` 0))
      (set `self.LogAttached` true)
      (`|PlayMontage` null "/Game/Sacha/FirstPersonArmSacha/Annimation/AM_Grab2.AM_Grab2"
        (:`OnCompleted`
          (`self.EnableInput` (`GameplayStatics.GetPlayerController` 0))
          (if (`self.ClothAttached`)
            (set `self.CanBurn` true :!label _label)))))
    (:`NewEnumerator7`
      (`self.DisableInput` (`GameplayStatics.GetPlayerController` 0))
      (set `self.ClothAttached` true)
      (`|PlayMontage` null "/Game/Sacha/FirstPersonArmSacha/Annimation/AM_Grab2.AM_Grab2"
        (:`OnCompleted`
          (`self.EnableInput` (`GameplayStatics.GetPlayerController` 0))
          (if (`self.LogAttached`)
            (goto _label)))))))

(fn `UserConstructionScript`)