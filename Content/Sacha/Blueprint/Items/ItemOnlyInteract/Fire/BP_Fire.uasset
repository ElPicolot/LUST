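; BP_Fire is an interact-only fire item that is lit when the player interacts with a specific held item.
; InteractWorking checks the item in hand, then activates the Niagara effect, plays the fire sound at AudioFire's location and flags IsBurning.
; It also shows a "Hot as hell fire" subtitle with a matching voice line, then replaces CanInteractWith so a different item type is accepted.
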(event `self.ReceiveBeginPlay`
  (`parent.ReceiveBeginPlay`))

(event `/Game/Sacha/Interface/BPI_Interact.Interact Working`
  (params (ItemInHand :type "/Game/Sacha/Blueprint/Items/E_MainItemType Enum" :default "NewEnumerator0") (ItemInHandforAnim :type "/Game/Sacha/Blueprint/Items/BP_Item Object Reference") (PlayrRef :type "/Game/Sacha/Blueprint/BP_FirstPersonCharacterSacha Object Reference"))
  (set `self.Playr Ref_0` PlayrRef)
  (if (`|EnumEquality` ItemInHand "NewEnumerator2")
    (`ActorComponent.SetActive` (`self.Niagara`) true false)
    (`GameplayStatics.PlaySoundAtLocation` "/Game/Sounds/SFX/Fire.Fire" (`SceneComponent.K2_GetComponentLocation` (`self.Audio_Fire`)) (struct) 0.8 1.0 0.0 null null null null)
    (set `self.IsBurning` true)
    (`/Game/Sacha/Winget/WB_SousTitre.EventSousTitrewinget` (`/Game/Sacha/Blueprint/BP_FirstPersonCharacterSacha.WingetSousTitre` (`self.Playr Ref_0`)) "Hot as hell fire")
    (message `/Game/Sacha/Interface/BPI_Interact.PlaySound` (`self.Speaker`) "/Game/Sounds/Antagonist_Dialogue_Final/15_Hot_As_Hell.15_Hot_As_Hell" 0.0)
    (set `self.CanInteractWith?` (`|MakeMap` "NewEnumerator5" true :!type "/Game/Sacha/Blueprint/Items/E_MainItemType Enum"))))

(fn `UserConstructionScript`
  (`parent.UserConstructionScript`))