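; BP_Interaction is an interaction item Blueprint that holds helper functions, with empty events and an empty SetTransformWhenInteract stub.
; Two functions handle vertical mesh movement, computing an offset Z and interpolating toward it at constant or eased speed until StopMove is set.
; Others switch the active camera to the one nearest the player mesh, check the held item for a whip, toggle grab physics and collision, and play sounds.
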(event `self.ReceiveBeginPlay`)

(event `self.ReceiveTick`
  (params (DeltaSeconds :type "Float (single-precision)")))

(fn `Get Closest Camera`
  (params (SKPlayerRef :type "SkeletalMeshComponent Object Reference") (CameraTarget :type "CameraComponent Object Reference") (AllCamera :type "Array of CameraComponent Object Reference"))
  (returns (NewLocalVar_01 :type "CameraComponent Object Reference") (DistanceCamera1 :type "Float (double-precision)"))
  (locals (SKMeshPlayer :type "SkeletalMeshComponent Object Reference") (TargetCam :type "CameraComponent Object Reference") (DistanceCamera :type "Float (double-precision)"))
  (bind _output_get (set `local.SKMeshPlayer` SKPlayerRef))
  (bind _output_get_2 (set `local.TargetCam` CameraTarget))
  (set `local.DistanceCamera` (`KismetMathLibrary.Vector_Distance` (`SceneComponent.K2_GetComponentLocation` _output_get) (`SceneComponent.K2_GetComponentLocation` _output_get_2)))
  ;[1 1 1] get closest camera
  (for _array_element AllCamera
    (bind _returnvalue (`KismetMathLibrary.Vector_Distance` (`SceneComponent.K2_GetComponentLocation` (`local.SKMeshPlayer`)) (`SceneComponent.K2_GetComponentLocation` _array_element)))
    (if (> (`KismetMathLibrary.Vector_Distance` (`SceneComponent.K2_GetComponentLocation` (`local.SKMeshPlayer`)) (`SceneComponent.K2_GetComponentLocation` (`local.TargetCam`))) _returnvalue)
      (`ActorComponent.SetActive` (`local.TargetCam`) false false)
      (bind _output_get_3 (set `local.TargetCam` _array_element))
      (`ActorComponent.SetActive` _output_get_3 true false)
      (set `local.DistanceCamera` _returnvalue)))
  (return (`local.TargetCam`) (`local.DistanceCamera`)))

(fn `GoMeshMoveZ`
  (params (Mesh :type "SceneComponent Object Reference") (TargetLocationZ :type "Float (double-precision)") (Speed :type "Float (double-precision)") (`Constant?` :type Boolean) (offsetPosition :type "Float (double-precision)"))
  (returns (StopMoveZ :type Boolean))
  (locals (StopMove :type Boolean))
  (bind _returnvalue (`GameplayStatics.GetWorldDeltaSeconds`))
  (bind _returnvalue_2 (`SceneComponent.GetRelativeTransform` (`local.Mesh`)))
  (`/Engine/EditorBlueprintResources/StandardMacros.IsValid` Mesh
    (:`Is Valid`
      (if (`local.Constant?`)
        (`SceneComponent.K2_SetRelativeLocation` (`local.Mesh`) (`KismetMathLibrary.MakeVector` (.x (.location _returnvalue_2)) (.y (.location _returnvalue_2)) (`KismetMathLibrary.FInterpTo_Constant` (.z (.location _returnvalue_2)) (`local.TargetLocationZ`) _returnvalue (`local.Speed`))) false false)
        (else
          (`SceneComponent.K2_SetRelativeLocation` (`local.Mesh`) (`KismetMathLibrary.MakeVector` (.x (.location _returnvalue_2)) (.y (.location _returnvalue_2)) (`KismetMathLibrary.FInterpTo` (.z (.location _returnvalue_2)) (`local.TargetLocationZ`) _returnvalue (`local.Speed`))) false false)))
      (`|ExecutionSequence`
        (:`then_0`
          (if (or (and (> (`local.offsetPosition`) 0.0) (>= (.z (.location (`SceneComponent.GetRelativeTransform` (`local.Mesh`)))) (`local.TargetLocationZ`))) (and (< (`local.offsetPosition`) 0.0) (<= (.z (.location (`SceneComponent.GetRelativeTransform` (`local.Mesh`)))) (`local.TargetLocationZ`))))
            (set `local.StopMove` true)))
        (:`then_1`
          (return (`local.StopMove`)))))))

(fn `IsWhip?`
  (params (ItemInHands :type "/Game/Sacha/Blueprint/Items/E_MainItemType Enum" :default "NewEnumerator0"))
  (returns (IsWhip :type Boolean))
  (return (`|EnumEquality` ItemInHands "NewEnumerator1")))

(fn `PhysicsGrab`
  (`PrimitiveComponent.SetCollisionEnabled` (`self.StaticMesh`) "NoCollision")
  (`PrimitiveComponent.SetSimulatePhysics` (`self.StaticMesh`) true))

(fn `Set Mesh Move Z`
  (params (Scenecomponent :type "SceneComponent Object Reference") (OffsetPosition :type "Float (double-precision)"))
  (returns (TargetPositionZ :type "Float (double-precision)"))
  (`/Engine/EditorBlueprintResources/StandardMacros.IsValid` Scenecomponent
    (:`Is Valid`
      (return (+ (.z (.location (`SceneComponent.GetRelativeTransform` Scenecomponent))) OffsetPosition)))))

(fn `SetAndPlaySound`
  (params (NewSound :type "SoundBase Object Reference") (Audio :type "AudioComponent Object Reference"))
  (`AudioComponent.SetSound` Audio NewSound)
  (`AudioComponent.Play` (`self.Audio1`) 0.0))

(fn `SetTransformWhenInteract`)

(fn `UserConstructionScript`)