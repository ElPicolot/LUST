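; BP_Iron is an iron item Blueprint that reacts when it is used in an item-to-item interaction.
; Its Niagara effect is switched off at BeginPlay.
; InteractBetweenItem activates the effect and sets CanBurn on two referenced NPCs, Pnj2 and Pnj3, allowing them to burn.
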(event `self.ReceiveBeginPlay`
  (`parent.ReceiveBeginPlay`)
  (`ActorComponent.SetActive` (`self.Niagara_0`) false false))

(event `/Game/Sacha/Interface/BPI_InteractWorking.InteractBetweenItem`
  (`ActorComponent.SetActive` (`self.Niagara_0`) true false)
  (set `/Game/Sacha/Blueprint/PNJ/BP_PNJ2.CanBurn` true (`self.Pnj2`))
  (set `/Game/Sacha/Blueprint/PNJ/BP_PNJ3.CanBurn` true (`self.Pnj3`)))

(fn `UserConstructionScript`
  (`parent.UserConstructionScript`))