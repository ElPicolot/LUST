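; BP_Lighter is a lighter item that shows or hides its flame through a Niagara component.
; Tick calls ActiveFire every frame to match the Niagara active state to the Active0 boolean, which is not set within this Blueprint.
; A separate LighterFiree function toggles the effect with a FlipFlop and debug prints, but nothing here calls it.
; The IA_Use input event is an empty stub.
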(event `self.ReceiveBeginPlay`)

(event `self.ReceiveTick`
  (params (DeltaSeconds :type "Float (single-precision)"))
  (`self.ActiveFire`))

(event `ActiveFire`
  (if (`self.Active_0`)
    (`ActorComponent.SetActive` (`self.Niagara`) true false)
    (else
      (`ActorComponent.SetActive` (`self.Niagara`) false false))))

(event `EnhancedInput|/Game/Sacha/Input/InputAction/IA_Use`
  (params (ActionValue :type Boolean) (ElapsedSeconds :type "Float (double-precision)") (TriggeredSeconds :type "Float (double-precision)") (InputAction :type "InputAction Object Reference" :default "/Game/Sacha/Input/InputAction/IA_Use.IA_Use")))

(fn `LighterFiree`
  (`/Engine/EditorBlueprintResources/StandardMacros.FlipFlop`
    (:`A`
      (`ActorComponent.SetActive` (`self.Niagara`) true false)
      (`KismetSystemLibrary.PrintString` "Hello"))
    (:`B`
      (`ActorComponent.SetActive` (`self.Niagara`) false false)
      (`KismetSystemLibrary.PrintString` "Hello"))))

(fn `UserConstructionScript`)