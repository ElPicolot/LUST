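; BP_Pinces is a pincers item whose construction script registers its left and right pincer meshes as the item's skeletal meshes.
; Its Electricite function is a cooldown-gated electric arc effect that line-traces in a random direction from between the pincers, with debug drawing.
; On a hit, it spawns an attached Niagara beam fed with start, impact point and normal.
; Nothing in this Blueprint currently runs Electricite, as its only event-graph call is disconnected.
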(event `self.ReceiveTick`
  (params (DeltaSeconds :type "Float (single-precision)")))

(fn `Electricite`
  (locals (`Impact Offset` :type "Float (double-precision)") (RandomDirection :type "Vector Structure"))
  (bind _randomdirection (`local.RandomDirection`))
  (bind _returnvalue (* _randomdirection (`self.MinRadius_0`)))
  (bind _returnvalue_2 (/ (+ (`SceneComponent.K2_GetComponentLocation` (`self.PinceLeft`)) (`SceneComponent.K2_GetComponentLocation` (`self.PinceRight`))) 2.0))
  (if (>= (- (`GameplayStatics.GetTimeSeconds`) (`self.LastTrace_0`)) (`self.TraceCoolDown_0`))
    ;[1 1 1] Trace
    (set `local.RandomDirection` (`KismetMathLibrary.RandomUnitVector`))
    (bind _outhit (`KismetSystemLibrary.LineTraceSingle` :`Start` (+ _returnvalue_2 _returnvalue) :`End` (+ _returnvalue_2 (* _randomdirection (`self.MaxRadius_0_0`))) :`TraceChannel` "TraceTypeQuery1" :`DrawDebugType` "ForDuration" :`DrawTime` (`self.TraceCoolDown_0`)))
    (set `self.LastTrace_0` (`GameplayStatics.GetTimeSeconds`))
    (bind (_bblockinghit _binitialoverlap _time _distance _location _impactpoint _normal _impactnormal) (`GameplayStatics.BreakHitResult` _outhit))
    ;[1 1 1] Spawn Niagara System and set parameters.
    (if _bblockinghit
      (bind _returnvalue_3 (`NiagaraFunctionLibrary.SpawnSystemAttached` "/Game/VFX/Electricity/CourteElec_01.CourteElec_01" (`self.Niagara_0`) "None" (0.0 0.0 0.0) (struct) "KeepRelativeOffset" true))
      (`NiagaraComponent.SetVariableVec3` _returnvalue_3 "BeamStartPoint" _returnvalue)
      (`NiagaraComponent.SetVariableVec3` _returnvalue_3 "BeamEndPoint" (+ _impactpoint (* _impactnormal (`local.Impact Offset`))))
      (`NiagaraComponent.SetVariableVec3` _returnvalue_3 "ImpactNormal" _impactnormal))))

(fn `UserConstructionScript`
  (set `self.ItemSkeletalMesh` (`self.PinceLeft`))
  (set `self.ItemSkeletalMesh2` (`self.PinceRight`)))