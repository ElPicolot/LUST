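; BP_Lighter1 is a lighter item that can be physics-grabbed through the InteractSacha interaction event.
; Every Tick it rotates its Plane from a look-at toward the player's first-person camera X/Y, using only roll and pitch, as a billboard-style effect.
; The Niagara effect is switched off on BeginPlay and ActiveFire is empty, with leftover toggle logic disconnected.
; A PlaySound event plays any supplied sound on its audio component.
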(event `self.ReceiveBeginPlay`
  (`ActorComponent.SetActive` (`self.NiagaraDefault`) false false))

(event `ActiveFire`)

(event `self.ReceiveTick`
  (params (DeltaSeconds :type "Float (single-precision)"))
  (bind _plane (`self.Plane`))
  (bind (_returnvalue_x _returnvalue_y) (`KismetMathLibrary.BreakVector` (`SceneComponent.K2_GetComponentLocation` (`/Game/Sacha/Blueprint/BP_FirstPersonCharacterSacha.FirstPersonCamera` (cast `/Game/Sacha/Blueprint/BP_FirstPersonCharacterSacha` (`GameplayStatics.GetPlayerCharacter` 0) :!pure true)))))
  (bind (_returnvalue_roll _returnvalue_pitch) (`KismetMathLibrary.BreakRotator` (`KismetMathLibrary.FindLookAtRotation` (`SceneComponent.K2_GetComponentLocation` _plane) (`KismetMathLibrary.MakeVector` _returnvalue_x _returnvalue_y))))
  (`SceneComponent.K2_SetRelativeRotation` _plane (`KismetMathLibrary.MakeRotator` _returnvalue_roll _returnvalue_pitch) false false))

(event `self.InteractSacha`
  (`self.PhysicsGrab`))

(event `self.PlaySound`
  (params (SoundToPlay :type "SoundBase Object Reference") (StartTime :type "Float (double-precision)"))
  (`AudioComponent.SetSound` (`self.Audio1`) SoundToPlay)
  (`AudioComponent.Play` (`self.Audio1`) 0.0))

(fn `UserConstructionScript`)