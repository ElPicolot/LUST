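; BP_DoorEnd is a double door actor that swings open when its GrabItem event fires.
; A DoOnce gate lets only the first call start the opening timeline, and the graph has no path to reset or close it.
; The timeline track drives a yaw lerp that rotates DoorR and DoorL a quarter turn in opposite directions.
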(event `/Game/Sacha/Interface/BPI_Item.GrabItem`
  (params (PlayerRef :type "/Game/Sacha/Blueprint/BP_FirstPersonCharacterSacha Object Reference"))
  (`/Engine/EditorBlueprintResources/StandardMacros.DoOnce` false
    (:`Completed`
      (bind (_direction _newtrack_0) (`Timeline|TimelineOpenDoor`)
        (:`Update`
          (`SceneComponent.K2_SetRelativeRotation` (`self.DoorR`) (`KismetMathLibrary.MakeRotator` 0.0 0.0 (`KismetMathLibrary.Lerp` 0.0 -90.0 _newtrack_0)) false false)
          (`SceneComponent.K2_SetRelativeRotation` (`self.DoorL`) (`KismetMathLibrary.MakeRotator` 0.0 0.0 (`KismetMathLibrary.Lerp` 0.0 90.0 _newtrack_0)) false false))))))

(fn `UserConstructionScript`
  (`parent.UserConstructionScript`))