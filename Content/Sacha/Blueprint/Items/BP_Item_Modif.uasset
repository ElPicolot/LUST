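; Multi-type item actor for pickups and held tools (whip, lighter, clamp, iron, consumables), whose construction script builds meshes from MainItemType.
; GrabItem adds the type to the player's inventory, moves to the hand socket, then destroys the actor.
; UseItem checks the target's CanInteractWith map, then runs per-type montages or timelines that trigger InteractWorkingMessage, or a failure dip.
; Clamps draw charge from batteries, losing it beyond a timer-checked distance; consumables are removed after placement.
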(event `self.ReceiveBeginPlay`)

(event `EventRemoveCollision`
  (bind _itemstaticmesh2 (`self.ItemStaticMesh2`)
    (:`then`
      (`PrimitiveComponent.SetCollisionObjectType` _itemstaticmesh2 "ECC_WorldDynamic"))
    (:`else`
      _))
  (bind _itemskeletalmesh (`self.ItemSkeletalMesh`)
    (:`then`
      (`PrimitiveComponent.SetCollisionObjectType` _itemskeletalmesh "ECC_WorldDynamic"))
    (:`else`
      _))
  (bind _itemskeletalmesh2 (`self.ItemSkeletalMesh2`)
    (:`then`
      (`PrimitiveComponent.SetCollisionObjectType` _itemskeletalmesh2 "ECC_WorldDynamic"))
    (:`else`
      _))
  (bind _itemstaticmesh (`self.ItemStaticMesh`)
    (:`then`
      (`PrimitiveComponent.SetCollisionObjectType` _itemstaticmesh "ECC_WorldDynamic"))
    (:`else`)))

(event `self.GrabItem`
  (params (PlayerRef :type "/Game/Sacha/Blueprint/BP_FirstPersonCharacterSacha Object Reference"))
  (bind _playerref (`self.PlayerRef`))
  (bind _playerref_2 (`self.PlayerRef`))
  (bind _weaponsocket1 (`/Game/Sacha/Blueprint/BP_FirstPersonCharacterSacha.WeaponSocket1` _playerref_2))
  (bind _output_get (set `self.PlayerRef` PlayerRef))
  (bind _itemstaticmesh (`self.ItemStaticMesh`)
    (:`then`
      (`PrimitiveComponent.SetSimulatePhysics` _itemstaticmesh false))
    (:`else`
      _))
  (`self.DisableInput` _output_get (`GameplayStatics.GetPlayerController` 0))
  (`self.EventRemoveCollision`)
  (`self.SetActorEnableCollision` false)
  (`KismetSystemLibrary.Delay` 0.2)
  (bind _returnvalue (`KismetArrayLibrary.Array_AddUnique` (`/Game/Sacha/Blueprint/BP_FirstPersonCharacterSacha.Inventory` _output_get) (`self.MainItemType`)))
  (set `/Game/Sacha/Blueprint/BP_FirstPersonCharacterSacha.CurrentItemIndex` _returnvalue (`self.PlayerRef`))
  (`self.SetActorEnableCollision` false)
  (`/Game/Sacha/Blueprint/BP_FirstPersonCharacterSacha.EventSwitchItem` (`self.PlayerRef`))
  (`KismetSystemLibrary.MoveComponentTo` (`self.DefaultSceneRoot`) (+ (- (`SceneComponent.K2_GetComponentLocation` _weaponsocket1) (0.0 0.0 10.0)) (* (`self.GetActorForwardVector` _playerref_2) -30.0)) (`SceneComponent.K2_GetComponentRotation` _weaponsocket1) true true 0.5)
  (`self.EnableInput` (`self.PlayerRef`) (`GameplayStatics.GetPlayerController` 0))
  (`/Game/Sacha/Blueprint/BP_FirstPersonCharacterSacha.BeginHeadbob` (`self.PlayerRef`))
  (if (`|EnumEquality` (`self.MainItemType`) "NewEnumerator1")
    (bind _returnvalue_2 (`GameplayStatics.GetActorOfClass` "/Game/Sacha/Blueprint/Puzzle/PictoMove/BP_PictoMove.BP_PictoMove_C"))
    (set `/Game/Sacha/Blueprint/Puzzle/PictoMove/BP_PictoMove.HasWhip` true _returnvalue_2)
    (set `self.WhipIsInIventory` true))
  (`self.K2_DestroyActor`)
  (`/Engine/EditorBlueprintResources/StandardMacros.DoOnce` false
    (:`Completed`
      (`/Game/Sacha/Winget/WB_PickUp.EventShowMolette` (`/Game/Sacha/Blueprint/BP_FirstPersonCharacterSacha.WingetPickup` _playerref))
      (set `/Game/Sacha/Blueprint/BP_FirstPersonCharacterSacha.ShowMollette` true _playerref))))

(event `EventCheckMaxDistance`
  (bind _returnvalue (`KismetSystemLibrary.K2_SetTimerDelegate` (delegate `EventCheckMaxDistanceTick`) 0.1 true)))

(event `self.UseItem`
  (params (PlayerRef :type "/Game/Sacha/Blueprint/BP_FirstPersonCharacterSacha Object Reference") (ItemInteract :type "Actor Object Reference"))
  (bind _playerref (`self.PlayerRef`))
  (bind _asbp_interaction (cast `/Game/Sacha/Blueprint/Items/BP_Interaction` ItemInteract)
    (:`then`
      (set `self.InteractionRef` _asbp_interaction)
      (set `self.PlayerRef` PlayerRef)
      (`KismetSystemLibrary.Delay` 0.2)
      (if (`BlueprintMapLibrary.Map_Find` (`/Game/Sacha/Blueprint/Items/BP_Interaction.CanInteractWith?` (`self.InteractionRef`)) (`self.MainItemType`))
        (bind _asbp_monitor_security (cast `/Game/Sacha/Blueprint/Items/ItemOnlyInteract/Camera/BP_MonitorSecurity` (`self.InteractionRef`))
          (:`then`
            (set `/Game/Sacha/Blueprint/BP_FirstPersonCharacterSacha.SecurityMonitorRef` _asbp_monitor_security _playerref)
            (message `/Game/Sacha/Interface/BPI_Interact.Interact Working` _asbp_monitor_security (`self.MainItemType`) self _playerref))
          (:`CastFailed`
            (cast `/Game/Sacha/Blueprint/Items/ItemOnlyInteract/BatterieMachine/BP_BatterieMachine` (`self.InteractionRef`)
              (:`then`
                (if (`|EnumEquality` (`self.MainItemType`) "NewEnumerator3")
                  (switch `/Game/Sacha/Blueprint/Items/E_MainItemType` (`self.MainItemType`) :!label _label
                    (:`NewEnumerator1`
                      (`self.PlayFouet`))
                    (:`NewEnumerator2`
                      (`self.PlayLighter`))
                    (:`NewEnumerator3`
                      (bind _asbp_battery (cast `/Game/Sacha/Blueprint/Items/ItemOnlyInteract/Batterie/BP_Battery` (`self.InteractionRef`))
                        (:`then`
                          (if (not (`self.CanElectrocute`))
                            (set `self.BatteryRef` _asbp_battery)
                            (set `self.CanElectrocute` true)
                            (`self.EventCheckMaxDistance`)
                            (`self.ClampSucces`)
                            (else
                              (`self.ItemFail`))))
                        (:`CastFailed`
                          (if (`self.CanElectrocute`)
                            (set `/Game/Sacha/Blueprint/Items/ItemOnlyInteract/Batterie/BP_Battery.ElectricteVFX` false _asbp_battery)
                            (`KismetSystemLibrary.PrintString` "ICI" true true (struct :`R` 0.257024 :`B` 0.276042 :`A` 1.0))
                            (`KismetSystemLibrary.PrintString` "Hello" true true (struct :`R` 0.257024 :`B` 0.276042 :`A` 1.0))
                            (`self.ClampSucces`)
                            (`|PlayMontage` (`self.ItemSkeletalMesh`) "/Game/Kilian/Anims/Pinces/PincesLeft/PinceLeftOpen.PinceLeftOpen"
                              (:`then`
                                (`|PlayMontage` (`self.ItemSkeletalMesh2`) "/Game/Kilian/Anims/Pinces/PinceRight/PinceRightOpen.PinceRightOpen"
                                  (:`then`
                                    (`SceneComponent.SetVisibility` (`self.CourteElec_01`) false false)))))
                            (else
                              (`self.ItemFail`))))))
                    (:`NewEnumerator5`
                      (bind _asbp_fire (cast `/Game/Sacha/Blueprint/Items/ItemOnlyInteract/Fire/BP_Fire` (`self.InteractionRef`))
                        (:`then`
                          (if (`/Game/Sacha/Blueprint/Items/ItemOnlyInteract/Fire/BP_Fire.IsBurning` _asbp_fire)
                            (`self.IronSucces` true)
                            (else
                              (`self.ItemFail`))))
                        (:`CastFailed`
                          (if (`self.Light`)
                            (`self.IronSucces` false)
                            (else
                              (`self.ItemFail`)
                              (`KismetSystemLibrary.PrintString` "bug ?"))))))
                    (:`NewEnumerator6`
                      (`self.DropItemSucces` :!label _label_2))
                    (:`NewEnumerator7`
                      (goto _label_2))
                    (:`NewEnumerator8`
                      (goto _label_2))
                    (:`NewEnumerator10`
                      (goto _label_2))
                    (:`NewEnumerator11`
                      (goto _label_2)))
                  (else
                    (message `/Game/Sacha/Interface/BPI_Interact.Interact Working` (`self.InteractionRef`) (`self.MainItemType`) self (`self.PlayerRef`)))))
              (:`CastFailed`
                (goto _label)))))
        (else
          (`self.ItemFail`))))
    (:`CastFailed`
      (`self.EnableInput` PlayerRef (`GameplayStatics.GetPlayerController` 0)))))

(event `EventCheckMaxDistanceTick`
  (bind _batteryref (`self.BatteryRef`))
  (bind _cable (`/Game/Sacha/Blueprint/Items/ItemOnlyInteract/Batterie/BP_Battery.Cable` _batteryref))
  (bind _cable1 (`/Game/Sacha/Blueprint/Items/ItemOnlyInteract/Batterie/BP_Battery.Cable1` _batteryref))
  (if (> (`KismetMathLibrary.VSizeXY` (- (`self.K2_GetActorLocation`) (`self.K2_GetActorLocation` (`self.BatteryRef`)))) 350.0)
    (`CableComponent.SetAttachEndTo` _cable null "None" "None")
    (`SceneComponent.SetVisibility` _cable false false)
    (`CableComponent.SetAttachEndTo` _cable1 null "None" "None")
    (`SceneComponent.SetVisibility` _cable1 false false)
    (set `self.CanElectrocute` false)
    (`KismetSystemLibrary.K2_ClearAndInvalidateTimerHandle` (stale `EventCheckMaxDistance` _returnvalue))))

(event `ReverseMovement`
  (bind (_direction _newtrack_0) (`Timeline|TimelineLighter` :!via `Reverse` :!label _label_3)
    (:`Update`
      (`SceneComponent.K2_SetWorldTransform` (`self.DefaultSceneRoot`) (`KismetMathLibrary.TLerp` (`self.InitialTrandform`) (`self.TargetTransform`) _newtrack_0) false false))
    (:`Finished`
      (if (`self.reverse`)
        (`self.EnableInput` (`self.PlayerRef`) (`GameplayStatics.GetPlayerController` 0))
        (set `self.reverse` false)
        (`/Game/Sacha/Blueprint/BP_FirstPersonCharacterSacha.BeginHeadbob` (`self.PlayerRef`))
        (else
          (set `self.reverse` true)
          (bind _notifyname (`|PlayMontage` (`self.ItemSkeletalMesh`) "/Game/Kilian/Anims/Briquet/AM_AllumeCandle.AM_AllumeCandle")
            (:`OnCompleted`
              (`self.ReverseMovement`))
            (:`OnNotifyBegin`
              (switch `name` _notifyname
                (:`Flamme`
                  (`/Engine/EditorBlueprintResources/StandardMacros.FlipFlop`
                    (:`A`
                      (`SceneComponent.SetVisibility` (`self.Flamme`) true false))
                    (:`B`
                      (`SceneComponent.SetVisibility` (`self.Flamme`) false false))))
                (:`CandleOn`
                  (message `/Game/Sacha/Interface/BPI_Interact.Interact Working` (`self.InteractionRef`) (`self.MainItemType`) self (`self.PlayerRef`)))))))))))

(event `PlayLighter`
  (`self.DisableInput` (`self.PlayerRef`) (`GameplayStatics.GetPlayerController` 0))
  (set `self.InitialTrandform` (`SceneComponent.K2_GetComponentToWorld` (`self.DefaultSceneRoot`)))
  (set `self.TargetTransform` (`SceneComponent.K2_GetComponentToWorld` (`/Game/Sacha/Blueprint/Items/BP_Interaction.TargetObject1` (`self.InteractionRef`))))
  (goto _label_3 :!via `PlayFromStart`))

(event `ItemFail`
  (bind (_initialitemlocation_x _initialitemlocation_y _initialitemlocation_z) (`KismetMathLibrary.BreakVector` (`self.InitialitemLocation`)))
  ;[1 1 1] Baterrie
  (set `self.InitialitemLocation` (`SceneComponent.K2_GetComponentLocation` (`self.DefaultSceneRoot`)))
  (bind (_direction _newtrack_0) (`Timeline|itemFailTimeline` :!via `PlayFromStart`)
    (:`Update`
      (`SceneComponent.K2_SetWorldLocation` (`self.DefaultSceneRoot`) (`KismetMathLibrary.MakeVector` _initialitemlocation_x _initialitemlocation_y (`KismetMathLibrary.Lerp` _initialitemlocation_z (- _initialitemlocation_z 10.0) _newtrack_0)) false false))
    (:`Finished`
      (`self.EnableInput` (`self.PlayerRef`) (`GameplayStatics.GetPlayerController` 0)))))

(event `DropItemSucces`
  ;[1 1 1] Baterrie
  (set `self.InitialTrandform` (`SceneComponent.K2_GetComponentToWorld` (`self.DefaultSceneRoot`)))
  (set `self.TargetTransform` (`SceneComponent.K2_GetComponentToWorld` (`/Game/Sacha/Blueprint/Items/BP_Interaction.TargetObject1` (`self.InteractionRef`))))
  (bind (_direction _newtrack_0) (`Timeline|MoveBatterieTo` :!via `PlayFromStart`)
    (:`Update`
      (`SceneComponent.K2_SetWorldTransform` (`self.DefaultSceneRoot`) (`KismetMathLibrary.TLerp` (`self.InitialTrandform`) (`self.TargetTransform`) _newtrack_0) false false))
    (:`Finished`
      (message `/Game/Sacha/Interface/BPI_Interact.Interact Working` (`self.InteractionRef`) (`self.MainItemType`) self (`self.PlayerRef`))
      (`KismetArrayLibrary.Array_RemoveItem` (`/Game/Sacha/Blueprint/BP_FirstPersonCharacterSacha.Inventory` (`self.PlayerRef`)) (`self.MainItemType`))
      (set `/Game/Sacha/Blueprint/BP_FirstPersonCharacterSacha.CurrentItemIndex` 0 (`self.PlayerRef`))
      (`self.EnableInput` (`self.PlayerRef`) (`GameplayStatics.GetPlayerController` 0))
      (`/Game/Sacha/Blueprint/BP_FirstPersonCharacterSacha.BeginHeadbob` (`self.PlayerRef`))
      (`self.K2_DestroyActor`))))

(event `EventFinishTimeline`
  (bind _playerref (`self.PlayerRef`))
  (bind _mainitemtype (`self.MainItemType`))
  (bind _interactionref (`self.InteractionRef`))
  (bind (_direction _newtrack_0) (`Timeline|ClampMoveto` :!label _label_4)
    (:`Update`
      (`SceneComponent.K2_SetWorldTransform` (`self.ItemSkeletalMesh`) (`KismetMathLibrary.TLerp` (`self.InitialTrandform`) (`self.TargetTransform`) _newtrack_0) false false)
      (`SceneComponent.K2_SetWorldTransform` (`self.ItemSkeletalMesh2`) (`KismetMathLibrary.TLerp` (`self.InitialTrandform2`) (`self.TargetTransform2`) _newtrack_0) false false))
    (:`Finished`
      (`self.EnableInput` (`self.PlayerRef`) (`GameplayStatics.GetPlayerController` 0))
      (`/Game/Sacha/Blueprint/BP_FirstPersonCharacterSacha.BeginHeadbob` (`self.PlayerRef`)))
    (:`Connect`
      (if (== (`self.InteractionRef`) (`self.BatteryRef`))
        (message `/Game/Sacha/Interface/BPI_Interact.Interact Working` _interactionref _mainitemtype self _playerref)
        (else
          (message `/Game/Sacha/Interface/BPI_Interact.Interact Working` _interactionref _mainitemtype self _playerref)
          (`ActorComponent.SetActive` (`/Game/Sacha/Blueprint/Items/ItemOnlyInteract/Batterie/BP_Battery.NS_SmokeBattery` (`self.BatteryRef`)) true false)
          (set `/Game/Sacha/Blueprint/Items/BP_Interaction.CanInteractWith?` (`|MakeMap` "NewEnumerator0" :!type "/Game/Sacha/Blueprint/Items/E_MainItemType Enum") (`self.BatteryRef`)))))))

(event `ClampSucces`
  (bind _interactionref (`self.InteractionRef`))
  (`self.DisableInput` (`self.PlayerRef`) (`GameplayStatics.GetPlayerController` 0))
  (set `self.InitialTrandform` (`SceneComponent.K2_GetComponentToWorld` (`self.ItemSkeletalMesh`)))
  (set `self.InitialTrandform2` (`SceneComponent.K2_GetComponentToWorld` (`self.ItemSkeletalMesh2`)))
  (set `self.TargetTransform` (`SceneComponent.K2_GetComponentToWorld` (`/Game/Sacha/Blueprint/Items/BP_Interaction.TargetObject1` _interactionref)))
  (set `self.TargetTransform2` (`SceneComponent.K2_GetComponentToWorld` (`/Game/Sacha/Blueprint/Items/BP_Interaction.TargetObject2` _interactionref)))
  (goto _label_4 :!via `PlayFromStart`))

(event `EventStopTimeline`
  (`KismetArrayLibrary.Array_RemoveItem` (`/Game/Sacha/Blueprint/BP_FirstPersonCharacterSacha.Inventory` (`self.PlayerRef`)) "NewEnumerator3")
  (set `/Game/Sacha/Blueprint/BP_FirstPersonCharacterSacha.CurrentItemIndex` 0 (`self.PlayerRef`))
  (set `/Game/Sacha/Blueprint/BP_FirstPersonCharacterSacha.ItemInHand` null (`self.PlayerRef`))
  (`self.K2_DetachFromActor` "KeepWorld" "KeepWorld" "KeepWorld")
  (`self.EnableInput` (`self.PlayerRef`) (`GameplayStatics.GetPlayerController` 0))
  (goto _label_4 :!via `Stop`))

(event `IronSucces`
  (params (light :type Boolean))
  (set `self.Light` light)
  (set `self.InitialTrandform` (`SceneComponent.K2_GetComponentToWorld` (`self.DefaultSceneRoot`)))
  (set `self.TargetTransform` (`SceneComponent.K2_GetComponentToWorld` (`/Game/Sacha/Blueprint/Items/BP_Interaction.TargetObject1` (`self.InteractionRef`))))
  (bind (_direction _newtrack_0) (`Timeline|IronTimeline` :!via `PlayFromStart`)
    (:`Update`
      (`SceneComponent.K2_SetWorldTransform` (`self.DefaultSceneRoot`) (`KismetMathLibrary.TLerp` (`self.InitialTrandform`) (`self.TargetTransform`) _newtrack_0) false false))
    (:`Finished`
      (`self.EnableInput` (`self.PlayerRef`) (`GameplayStatics.GetPlayerController` 0))
      (`/Game/Sacha/Blueprint/BP_FirstPersonCharacterSacha.BeginHeadbob` (`self.PlayerRef`)))
    (:`Burn`
      (if (`self.Light`)
        (bind (_direction_2 _newtrack_0_2) (`Timeline|TimelineEmmisiveIron` :!via `PlayFromStart` :!label _label_5)
          (:`Update`
            (`MaterialInstanceDynamic.SetScalarParameterValue` (`self.ItemDynamiqueMat`) "Emissive" (* _newtrack_0_2 0.4))))
        (else
          (message `/Game/Sacha/Interface/BPI_Interact.Interact Working` (`self.InteractionRef`) (`self.MainItemType`) self null)
          (`MaterialInstanceDynamic.SetScalarParameterValue` (`self.ItemDynamiqueMat`) "Emissive" (`KismetMathLibrary.FInterpTo` 0.4 0.0 (`GameplayStatics.GetWorldDeltaSeconds`) 1.0))
          (goto _label_5 :!via `ReverseFromEnd`))))))

(event `PlayFouet`
  (bind _itemskeletalmesh (`self.ItemSkeletalMesh`))
  (bind (_returnvalue_location _returnvalue_rotation) (`KismetMathLibrary.BreakTransform` (`SceneComponent.GetRelativeTransform` _itemskeletalmesh)))
  (set `self.FouetRotationHorsAnim` _returnvalue_rotation)
  (`SceneComponent.K2_SetRelativeTransform` _itemskeletalmesh (`KismetMathLibrary.MakeTransform` (30.0 0.0 0.0) (struct :`Pitch` -20.0 :`Yaw` -100.0 :`Roll` 20.0)) false false)
  (`|PlayMontage` (`self.ItemSkeletalMesh`) "/Game/Kilian/Anims/Fouet/AM_coupFouet.AM_coupFouet"
    (:`OnCompleted`
      (`self.EnableInput` (`self.PlayerRef`) (`GameplayStatics.GetPlayerController` 0))
      (`/Game/Sacha/Blueprint/BP_FirstPersonCharacterSacha.BeginHeadbob` (`self.PlayerRef`))
      (`SceneComponent.K2_SetRelativeTransform` (`self.ItemSkeletalMesh`) (`KismetMathLibrary.MakeTransform` (0.0 0.0 0.0) (`self.FouetRotationHorsAnim`)) false false))
    (:`OnNotifyBegin`
      (message `/Game/Sacha/Interface/BPI_Interact.Interact Working` (`self.InteractionRef`) (`self.MainItemType`) self (`self.PlayerRef`))
      (`KismetSystemLibrary.PrintString` "Hello"))))

(fn `GoMeshMoveZ`
  (params (Mesh :type "SceneComponent Object Reference") (TargetLocationZ :type "Float (double-precision)") (Speed :type "Float (double-precision)") (`Constant?` :type Boolean) (offsetPosition :type "Float (double-precision)"))
  (returns (StopMoveZ :type Boolean))
  (locals (StopMove :type Boolean))
  (bind _returnvalue (`GameplayStatics.GetWorldDeltaSeconds`))
  (bind _returnvalue_2 (`SceneComponent.GetRelativeTransform` (`local.Mesh`)))
  (`/Engine/EditorBlueprintResources/StandardMacros.IsValid` Mesh
    (:`Is Valid`
      (if (`local.Constant?`)
        (`SceneComponent.K2_SetRelativeLocation` (`local.Mesh`) (`KismetMathLibrary.MakeVector` (.x (.location _returnvalue_2)) (.y (.location _returnvalue_2)) (`KismetMathLibrary.FInterpTo_Constant` (.z (.location _returnvalue_2)) (`local.TargetLocationZ`) _returnvalue (`local.Speed`))) false false)
        (else
          (`SceneComponent.K2_SetRelativeLocation` (`local.Mesh`) (`KismetMathLibrary.MakeVector` (.x (.location _returnvalue_2)) (.y (.location _returnvalue_2)) (`KismetMathLibrary.FInterpTo` (.z (.location _returnvalue_2)) (`local.TargetLocationZ`) _returnvalue (`local.Speed`))) false false)))
      (`|ExecutionSequence`
        (:`then_0`
          (if (or (and (> (`local.offsetPosition`) 0.0) (>= (.z (.location (`SceneComponent.GetRelativeTransform` (`local.Mesh`)))) (`local.TargetLocationZ`))) (and (< (`local.offsetPosition`) 0.0) (<= (.z (.location (`SceneComponent.GetRelativeTransform` (`local.Mesh`)))) (`local.TargetLocationZ`))))
            (set `local.StopMove` true)))
        (:`then_1`
          (return (`local.StopMove`)))))))

(fn `PhysicsGrab`)

(fn `Set Mesh Move Z`
  (params (Scenecomponent :type "SceneComponent Object Reference") (OffsetPosition :type "Float (double-precision)"))
  (returns (TargetPositionZ :type "Float (double-precision)"))
  (`/Engine/EditorBlueprintResources/StandardMacros.IsValid` Scenecomponent
    (:`Is Valid`
      (return (+ (.z (.location (`SceneComponent.GetRelativeTransform` Scenecomponent))) OffsetPosition)))))

(fn `SetPositionWhenInteract`)

(fn `SetSimulateItemOnlyHand`)

(fn `UserConstructionScript`
  (switch `/Game/Sacha/Blueprint/Items/E_MainItemType` (`self.MainItemType`)
    (:`NewEnumerator0`
      (set `self.ItemSkeletalMesh` null))
    (:`NewEnumerator1`
      (bind _returnvalue (`AddComponent|NODE_AddSkeletalMeshComponent-0` :`RelativeTransform` (`KismetMathLibrary.MakeTransform` (0.0 0.0 0.0) (struct :`Pitch` -60.0 :`Yaw` -10.0 :`Roll` -70.0))))
      (bind _output_get (set `self.ItemSkeletalMesh` _returnvalue))
      (`PrimitiveComponent.SetBoundsScale` _output_get 3.0)
      (`SkeletalMeshComponent.SetAllBodiesBelowSimulatePhysics` _output_get "Handle_End" true false))
    (:`NewEnumerator2`
      (bind _returnvalue_2 (`AddComponent|NODE_AddSkeletalMeshComponent-1`))
      (set `self.ItemSkeletalMesh` _returnvalue_2)
      (bind _returnvalue_3 (`AddComponent|NODE_AddStaticMeshComponent-4` :`RelativeTransform` (`KismetMathLibrary.MakeTransform` (0.0 -8.0 0.0) (struct :`Pitch` 180.0 :`Roll` -90.0) (0.3 0.3 0.3))))
      (bind _output_get_2 (set `self.Flamme` _returnvalue_3))
      (`SceneComponent.K2_AttachToComponent` _output_get_2 (`self.ItemSkeletalMesh`) "ROOT" "KeepRelative" "KeepRelative" "KeepRelative" false))
    (:`NewEnumerator3`
      (bind _returnvalue_4 (`AddComponent|NODE_AddSkeletalMeshComponent-2` :`RelativeTransform` (`self.InitialTrandformOffsetPinceLeft`)))
      (set `self.ItemSkeletalMesh` _returnvalue_4)
      (bind _returnvalue_5 (`AddComponent|NODE_AddSkeletalMeshComponent-3` :`RelativeTransform` (`self.InitialTrandformOffsetPinceRight`)))
      (set `self.ItemSkeletalMesh2` _returnvalue_5))
    (:`NewEnumerator5`
      (bind _returnvalue_6 (`AddComponent|NODE_AddStaticMeshComponent-3`))
      (bind _output_get_3 (set `self.ItemStaticMesh` _returnvalue_6))
      (bind _returnvalue_7 (`PrimitiveComponent.CreateDynamicMaterialInstance` _output_get_3 0 "/Game/3D/AU_BarreMetalliqueLUST/MI_Barre_Metaliique_emiss.MI_Barre_Metaliique_emiss" "None"))
      (bind _output_get_4 (set `self.ItemDynamiqueMat` _returnvalue_7))
      (`MaterialInstanceDynamic.SetScalarParameterValue` _output_get_4 "Emissive" 0.0))
    (:`NewEnumerator6`
      (bind _returnvalue_8 (`AddComponent|NODE_AddStaticMeshComponent-2`))
      (set `self.ItemStaticMesh` _returnvalue_8))
    (:`NewEnumerator7`
      (bind _returnvalue_9 (`AddComponent|NODE_AddStaticMeshComponent-1`))
      (set `self.ItemStaticMesh` _returnvalue_9))
    (:`NewEnumerator8`
      (bind _returnvalue_10 (`AddComponent|NODE_AddStaticMeshComponent-0`))
      (set `self.ItemStaticMesh` _returnvalue_10))
    (:`NewEnumerator10`
      (bind _returnvalue_11 (`AddComponent|NODE_AddStaticMeshComponent-7`))
      (set `self.ItemStaticMesh` _returnvalue_11))
    (:`NewEnumerator11`
      (bind _returnvalue_12 (`AddComponent|NODE_AddStaticMeshComponent-8`))
      (set `self.ItemStaticMesh` _returnvalue_12))))