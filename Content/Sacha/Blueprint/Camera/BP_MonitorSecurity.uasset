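; Security monitor actor that shows the live feed of a security camera from its SecurityCameras list on its screen mesh.
; On BeginPlay it creates a dynamic screen material and a render target sized from viewport and camera quality, then links the first camera's scene capture to it.
; SwapCamera detaches the current capture and cycles to the next camera with a new render target; nothing live in this graph calls it.
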(event `self.ReceiveBeginPlay`
  (bind (_returnvalue_x _returnvalue_y) (`KismetMathLibrary.BreakVector2D` (`WidgetLayoutLibrary.GetViewportSize`)))
  (bind _monitormat (`self.MonitorMat`))
  (bind _cameralevelquality (`/Game/Sacha/Blueprint/Camera/BP_CameraSecurity.CameraLevelQuality` (`|GetArrayItem` (`self.SecurityCameras`))))
  (`/Engine/EditorBlueprintResources/StandardMacros.IsValid` (`|GetArrayItem` (`self.SecurityCameras`))
    (:`Is Valid`
      (bind _returnvalue (`KismetMaterialLibrary.CreateDynamicMaterialInstance` "/Game/Sacha/Blueprint/Camera/CameraSecurity.CameraSecurity"))
      (bind _output_get (set `self.MonitorMat` _returnvalue))
      (`PrimitiveComponent.SetMaterial` (`self.Monitor`) 0 _output_get)
      (bind _returnvalue_2 (`KismetRenderingLibrary.CreateRenderTarget2D` (`KismetMathLibrary.FTrunc` (* _cameralevelquality _returnvalue_x)) (`KismetMathLibrary.FTrunc` (* _returnvalue_y _cameralevelquality))))
      (bind _output_get_2 (set `self.CameraRT` _returnvalue_2))
      (bind _output_get_3 (set `SceneCaptureComponent2D.TextureTarget` _output_get_2 (`/Game/Sacha/Blueprint/Camera/BP_CameraSecurity.SceneCaptureComponent2D` (`|GetArrayItem` (`self.SecurityCameras`)))))
      (`MaterialInstanceDynamic.SetTextureParameterValue` _monitormat "Texture" _output_get_3)
      (`MaterialInstanceDynamic.SetScalarParameterValue` _monitormat "ScreenBrighness" 0.5)
      (`KismetSystemLibrary.PrintString` "oui mais non"))))

(event `SwapCamera`
  (bind (_returnvalue_x _returnvalue_y) (`KismetMathLibrary.BreakVector2D` (`WidgetLayoutLibrary.GetViewportSize`)))
  (bind _cameralevelquality (`/Game/Sacha/Blueprint/Camera/BP_CameraSecurity.CameraLevelQuality` (`|GetArrayItem` (`self.SecurityCameras`) (`self.CurrentCamera`))))
  (set `SceneCaptureComponent2D.TextureTarget` null (`/Game/Sacha/Blueprint/Camera/BP_CameraSecurity.SceneCaptureComponent2D` (`|GetArrayItem` (`self.SecurityCameras`) (`self.CurrentCamera`))))
  (bind _result (`/Engine/EditorBlueprintResources/StandardMacros.IncrementInt` (`self.CurrentCamera`))
    (:`  `
      (if (>= _result (`KismetArrayLibrary.Array_Length` (`self.SecurityCameras`)))
        (set `self.CurrentCamera` 0))
      (bind _returnvalue (`KismetRenderingLibrary.CreateRenderTarget2D` (`KismetMathLibrary.FTrunc` (* _cameralevelquality _returnvalue_x)) (`KismetMathLibrary.FTrunc` (* _returnvalue_y _cameralevelquality))))
      (bind _output_get (set `self.CameraRT` _returnvalue))
      (bind _output_get_2 (set `SceneCaptureComponent2D.TextureTarget` _output_get (`/Game/Sacha/Blueprint/Camera/BP_CameraSecurity.SceneCaptureComponent2D` (`|GetArrayItem` (`self.SecurityCameras`) (`self.CurrentCamera`)))))
      (`MaterialInstanceDynamic.SetTextureParameterValue` (`self.MonitorMat`) "Texture" _output_get_2))))

(fn `UserConstructionScript`)