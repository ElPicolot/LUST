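; BP_PNJ2 is an interactable NPC who pleads through voice, subtitle and montage the first time its box is overlapped, and can be branded once with a held iron.
; Interacting with the matching item plays the branding montage, sounds and subtitle, raises pain and updates the interaction map.
; A timeline drives the dynamic material's Burn parameter.
; When it finishes, the detached iron drops with physics and leaves the player's inventory.
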(event `self.ReceiveBeginPlay`
  (bind _perso (`self.Perso`))
  (bind _returnvalue (`PrimitiveComponent.CreateDynamicMaterialInstance` _perso 0 (`PrimitiveComponent.GetMaterial` _perso 0) "None"))
  (set `self.BurnDynamiqueMat` _returnvalue)
  (`TimelineComponent.SetPlayRate` (`self.TimelineBurn`) 1.25))

(event `self.Box.OnComponentBeginOverlap`
  (params (OverlappedComponent :type "PrimitiveComponent Object Reference") (OtherActor :type "Actor Object Reference") (OtherComp :type "PrimitiveComponent Object Reference") (OtherBodyIndex :type Integer) (bFromSweep :type Boolean) (SweepResult :type "HitResult Structure (by ref)"))
  (`/Engine/EditorBlueprintResources/StandardMacros.DoOnce` false
    (:`Completed`
      (if true
        (`GameplayStatics.PlaySoundAtLocation` "/Game/Sounds/SFX/Femme_Please.Femme_Please" (`SceneComponent.K2_GetComponentLocation` (`self.Audio_please`)) (struct) 2.0 1.0 0.0 null null null null)
        (`/Game/Sacha/Winget/WB_SousTitre.EventSousTitrewinget` (`/Game/Sacha/Blueprint/BP_FirstPersonCharacterSacha.WingetSousTitre` (`self.Playr Ref`)) "Please, I can't take this anymore...")
        (`|PlayMontage` (`self.Perso`) "/Game/Kilian/Anims/Cage/AM_Stooop.AM_Stooop")))))

(event `self.Interact Working`
  (params (ItemInHand :type "/Game/Sacha/Blueprint/Items/E_MainItemType Enum" :default "NewEnumerator0") (ItemInHandforAnim :type "/Game/Sacha/Blueprint/Items/BP_Item Object Reference") (PlayrRef :type "/Game/Sacha/Blueprint/BP_FirstPersonCharacterSacha Object Reference"))
  (bind _item_in_handfor_anim (`self.Item in Handfor Anim`))
  (bind _playr_ref (`self.Playr Ref`))
  (bind _itemstaticmesh (`/Game/Sacha/Blueprint/Items/BP_Item.ItemStaticMesh` _item_in_handfor_anim))
  (set `self.Item in Handfor Anim` ItemInHandforAnim)
  (if (`|EnumEquality` ItemInHand "NewEnumerator5")
    (`/Engine/EditorBlueprintResources/StandardMacros.DoOnce` false
      (:`Completed`
        (`|PlayMontage` (`self.Perso`) "/Game/Animation/pnj2/brulure_fer_pnj2_Montage.brulure_fer_pnj2_Montage"
          (:`then`
            ;[1 1 1] Son
            (`/Game/Sacha/Winget/WB_SousTitre.EventSousTitrewinget` (`/Game/Sacha/Blueprint/BP_FirstPersonCharacterSacha.WingetSousTitre` (`self.Playr Ref`)) "Branded into her flesh...  \nThat’s what she deserves!")
            (`GameplayStatics.PlaySoundAtLocation` "/Game/Sounds/Antagonist_Dialogue_Final/16_Flesh.16_Flesh" (`SceneComponent.K2_GetComponentLocation` (`self.Audio_Flesh`)) (struct) 0.4 1.0 0.0 null null null null)
            (`GameplayStatics.PlaySoundAtLocation` "/Game/Sounds/SFX/Flesh_Burning.Flesh_Burning" (`SceneComponent.K2_GetComponentLocation` (`self.Audio_FleshBurning`)) (struct) 1.0 1.0 0.0 null null null null)
            (message `/Game/Sacha/Interface/BPI_Interact.UpPain` (`self.BP_Pain`) 40.0)
            (set `self.CanInteractWith?` (`|MakeMap` "NewEnumerator0" :!type "/Game/Sacha/Blueprint/Items/E_MainItemType Enum"))
            (`self.K2_DetachFromActor` (`self.Item in Handfor Anim`) "KeepWorld" "KeepWorld" "KeepWorld")
            (bind (_direction _newtrack_0) (`Timeline|TimelineBurn` :!via `PlayFromStart`)
              (:`Update`
                (`MaterialInstanceDynamic.SetScalarParameterValue` (`self.BurnDynamiqueMat`) "Burn" (`KismetMathLibrary.Lerp` 0.0 1.0 _newtrack_0)))
              (:`Finished`
                (`PrimitiveComponent.SetSimulatePhysics` _itemstaticmesh true)
                (`PrimitiveComponent.SetCollisionResponseToChannel` _itemstaticmesh "ECC_WorldDynamic" "ECR_Ignore")
                (`PrimitiveComponent.SetCollisionProfileName` _itemstaticmesh "None" true)
                (`ActorComponent.SetActive` (`/Game/Sacha/Blueprint/Items/BP_Item.Niagara` _item_in_handfor_anim) false false)
                (set `/Game/Sacha/Blueprint/BP_FirstPersonCharacterSacha.CurrentItemIndex` 0 _playr_ref)
                (`KismetArrayLibrary.Array_RemoveItem` (`/Game/Sacha/Blueprint/BP_FirstPersonCharacterSacha.Inventory` _playr_ref) ItemInHand)
                (`GameplayStatics.PlaySoundAtLocation` "/Game/Sounds/Fer_Qui_Tombe/Fer_Qui_Tombe.Fer_Qui_Tombe" (`SceneComponent.K2_GetComponentLocation` (`self.Audio_Iron_Dropped`)) (struct) 50.0 1.0 6.0 null null null null)))))))))

(fn `UserConstructionScript`)