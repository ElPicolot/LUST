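; BP_Bras is a prop in the PNJ folder that plays sounds when the player bumps its SM_Foetus mesh.
; A hit passes a DoOnce before the cast to BP_FirstPersonCharacterSacha, then plays Sound and Rope_Balancing at the Audio component's location.
; A short timer then resets the DoOnce as a cooldown.
; Because the gate precedes the cast, a non-player hit closes it without scheduling a reset.
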(event `self.SM_Foetus.OnComponentHit`
  (params (HitComponent :type "PrimitiveComponent Object Reference") (OtherActor :type "Actor Object Reference") (OtherComp :type "PrimitiveComponent Object Reference") (NormalImpulse :type "Vector Structure") (Hit :type "HitResult Structure (by ref)"))
  (bind _returnvalue (`SceneComponent.K2_GetComponentLocation` (`self.Audio`)))
  (`/Engine/EditorBlueprintResources/StandardMacros.DoOnce` false :!label _label
    (:`Completed`
      (cast `/Game/Sacha/Blueprint/BP_FirstPersonCharacterSacha` OtherActor)
      (`GameplayStatics.PlaySoundAtLocation` (`self.Sound`) _returnvalue (struct) 1.0 1.0 0.0 null null null null)
      (`GameplayStatics.PlaySoundAtLocation` "/Game/Sounds/SFX/Rope_Balancing.Rope_Balancing" _returnvalue (struct) 1.0 1.0 0.0 null null null null)
      (`KismetSystemLibrary.K2_SetTimerDelegate` (delegate `ResetSound`) 5.0))))

(event `ResetSound`
  (goto _label :!via `Reset`))

(fn `UserConstructionScript`)