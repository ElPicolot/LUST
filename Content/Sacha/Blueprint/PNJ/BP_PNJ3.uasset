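; Interactable NPC that reacts to a whip strike by hauling its mesh along world X while raising the linked BoxCache cage.
; InteractWorking checks the held item and a busy flag, plays delayed audio, notifies BoxCache, then a Timeline lerps both objects by OffsetPosition.
; Each finished move sends pain to BPPain; reaching ActivationMax resets CanInteractWith to a single disabled entry.
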(event `self.ReceiveBeginPlay`
  (`parent.ReceiveBeginPlay`))

(event `self.Interact Working`
  (params (ItemInHand :type "/Game/Sacha/Blueprint/Items/E_MainItemType Enum" :default "NewEnumerator0") (ItemInHandforAnim :type "/Game/Sacha/Blueprint/Items/BP_Item Object Reference") (PlayrRef :type "/Game/Sacha/Blueprint/BP_FirstPersonCharacterSacha Object Reference"))
  (bind (_returnvalue_x _returnvalue_y _returnvalue_z) (`KismetMathLibrary.BreakVector` (`SceneComponent.K2_GetComponentLocation` (`self.StaticMesh`))))
  (bind _returnvalue_x_2 (`KismetMathLibrary.BreakVector` (`SceneComponent.K2_GetComponentLocation` (`self.StaticMesh`))))
  (bind _defaultsceneroot (`/Game/Sacha/Blueprint/Items/BP_Item.DefaultSceneRoot` (`self.BoxCache`)))
  (bind (_returnvalue_x_3 _returnvalue_y_2 _returnvalue_z_2) (`KismetMathLibrary.BreakVector` (`SceneComponent.K2_GetComponentLocation` (`/Game/Sacha/Blueprint/Items/BP_Item.DefaultSceneRoot` (`self.BoxCache`)))))
  (bind (_returnvalue_x_4 _returnvalue_y_3) (`KismetMathLibrary.BreakVector` (`SceneComponent.K2_GetComponentLocation` _defaultsceneroot)))
  (if (`|EnumEquality` ItemInHand "NewEnumerator1")
    (if (not (`self.IsMoving`))
      (set `self.IsMoving` true)
      (if (< (`self.Numberof Activation`) (`self.Activation Max`))
        (`GameplayStatics.PlaySound2D` "/Game/Sounds/SFX/Fouet_Coup.Fouet_Coup" 1.0 1.0 0.0 null null)
        (`KismetSystemLibrary.Delay` 0.2)
        (`AudioComponent.Play` (`self.Audio1`) 0.0)
        (`KismetSystemLibrary.Delay` 0.5)
        (set `CableComponent.bEnableStiffness` false (`self.Cable`))
        (`GameplayStatics.PlaySound2D` "/Game/Sounds/Audio_Effect/Impact_Brick_Drag_Through_Rock_Salt_04.Impact_Brick_Drag_Through_Rock_Salt_04" 1.0 1.0 0.0 null null)
        (`/Engine/EditorBlueprintResources/StandardMacros.IncrementInt` (`self.Numberof Activation`)
          (:`  `
            (set `self.InitialPositionX` _returnvalue_x_2)
            (set `self.TargetPositionX` (+ (`self.OffsetPosition`) _returnvalue_x_2))
            (set `self.CageInitialLocation` _returnvalue_z_2)
            (set `self.CageTargetLocation` (+ (`self.OffsetPosition`) _returnvalue_z_2))
            (message `/Game/Sacha/Interface/BPI_Interact.InteractBetweenItem` (`self.BoxCache`))
            (bind (_direction _newtrack_0) (`Timeline|Timeline` :!via `PlayFromStart`)
              (:`Update`
                (`SceneComponent.K2_SetWorldLocation` (`self.StaticMesh`) (`KismetMathLibrary.MakeVector` (`KismetMathLibrary.Lerp` (`self.InitialPositionX`) (`self.TargetPositionX`) _newtrack_0) _returnvalue_y _returnvalue_z) false false)
                (`SceneComponent.K2_SetWorldLocation` _defaultsceneroot (`KismetMathLibrary.MakeVector` _returnvalue_x_4 _returnvalue_y_3 (`KismetMathLibrary.Lerp` (`self.CageInitialLocation`) (`self.CageTargetLocation`) _newtrack_0)) false false))
              (:`Finished`
                (message `/Game/Sacha/Interface/BPI_Interact.UpPain` (`self.BP_Pain`) 11.0)
                (set `self.IsMoving` false)
                (set `CableComponent.bEnableStiffness` false (`self.Cable`))
                (if (not (< (`self.Numberof Activation`) (`self.Activation Max`)))
                  (set `self.CanInteractWith?` (`|MakeMap` "NewEnumerator0" :!type "/Game/Sacha/Blueprint/Items/E_MainItemType Enum")))))))))))

(fn `UserConstructionScript`
  (`parent.UserConstructionScript`))