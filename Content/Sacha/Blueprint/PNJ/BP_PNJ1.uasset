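; Gagged NPC victim in a torture puzzle, reacting to the player's items and rig events with montages, sounds, subtitles and pain updates to BPPain.
; Item interaction plays electric shock or whip reactions.
; Counted descent and stretching events drive the ropes, lower it by timeline or play montages, and reset or finish the BPPictoMove puzzle.
; A third stretch or a fall disables player input, plays a looping end animation and calls the monster door.
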(event `self.ReceiveBeginPlay`
  (bind _asbp_first_person_character_sacha (cast `/Game/Sacha/Blueprint/BP_FirstPersonCharacterSacha` (`GameplayStatics.GetPlayerCharacter` 0) :!pure true))
  (`TimelineComponent.SetPlayRate` (`self.TimelinePnjDencente`) 0.2)
  (set `self.Playr Ref` _asbp_first_person_character_sacha)
  (set `self.PlayrRef` _asbp_first_person_character_sacha))

(event `self.ReceiveTick`
  (params (DeltaSeconds :type "Float (single-precision)")))

(event `/Game/Sacha/Interface/BPI_Interact.Interact Working`
  (params (ItemInHand :type "/Game/Sacha/Blueprint/Items/E_MainItemType Enum" :default "NewEnumerator0") (ItemInHandforAnim :type "/Game/Sacha/Blueprint/Items/BP_Item Object Reference") (PlayrRef :type "/Game/Sacha/Blueprint/BP_FirstPersonCharacterSacha Object Reference"))
  (bind _skeletalmesh (`self.SkeletalMesh`))
  (bind _skeletalmesh_2 (`self.SkeletalMesh`))
  (bind (_returnvalue_x _returnvalue_y _returnvalue_z) (`KismetMathLibrary.BreakVector` (`SceneComponent.K2_GetComponentLocation` _skeletalmesh)))
  (bind (_returnvalue_x_2 _returnvalue_y_2 _returnvalue_z_2) (`KismetMathLibrary.BreakVector` (`SceneComponent.K2_GetComponentLocation` _skeletalmesh_2)))
  (set `self.PlayrRef` PlayrRef)
  (set `self.Item in Handfor Anim` ItemInHandforAnim)
  (set `self.isFoueter` true)
  (`KismetSystemLibrary.PrintString` "AnimFouetSurLePnj1")
  (`|ExecutionSequence`
    (:`then_0`
      (if (`|EnumEquality` ItemInHand "NewEnumerator3")
        (set `self.CanInteractWith?` (`|MakeMap` "NewEnumerator1" true :!type "/Game/Sacha/Blueprint/Items/E_MainItemType Enum"))
        (`GameplayStatics.PlaySoundAtLocation` "/Game/Sounds/SFX/BZZZZ.BZZZZ" (`self.K2_GetActorLocation`) (struct) 1.0 1.0 0.0 null null null null)
        (`SceneComponent.K2_SetWorldLocation` _skeletalmesh_2 (`KismetMathLibrary.MakeVector` _returnvalue_x_2 _returnvalue_y_2 (- _returnvalue_z_2 70.0)) false false)
        (`|PlayMontage` (`self.SkeletalMesh`) "/Game/Kilian/Anims/HommeAttach/Homme_X_ELEC_Montage.Homme_X_ELEC_Montage"
          (:`OnBlendOut`
            (`SceneComponent.K2_SetWorldLocation` _skeletalmesh (`KismetMathLibrary.MakeVector` _returnvalue_x _returnvalue_y (+ _returnvalue_z 70.0)) false false)
            (message `/Game/Sacha/Interface/BPI_Interact.UpPain` (`self.BP_Pain`) 46.0)
            (`self.SetAndPlaySound` (`self.SoundToPlay`) (`self.Audio1`))
            (`self.SetAndPlaySound` (`self.SoundToPlay3`))
            (`/Game/Sacha/Blueprint/Items/BP_Item.EventActiveSmoke` (`self.Item in Handfor Anim`))
            (set `self.isFoueter` false)))))
    (:`then_1`
      (if (`|EnumEquality` ItemInHand "NewEnumerator1")
        (`|PlayMontage` (`self.SkeletalMesh`) "/Game/Kilian/Anims/HommeAttach/Homme_X_Fouet_Montage.Homme_X_Fouet_Montage"
          (:`then`
            (`/Engine/EditorBlueprintResources/StandardMacros.DoOnce` false
              (:`Completed`
                (`/Game/Sacha/Winget/WB_SousTitre.EventSousTitrewinget` (`/Game/Sacha/Blueprint/BP_FirstPersonCharacterSacha.WingetSousTitre` (`self.PlayrRef`)) "Ohhh, yeah do it harder...")
                (`GameplayStatics.PlaySoundAtLocation` "/Game/Sounds/Antagonist_Dialogue_Final/03_Do_it_Harder.03_Do_it_Harder" (`SceneComponent.K2_GetComponentLocation` (`self.Audio_DoItHarder`)) (struct) 1.0 1.0 0.0 null null null null))))
          (:`OnCompleted`
            (`/Engine/EditorBlueprintResources/StandardMacros.DoOnce` false
              (:`Completed`
                (message `/Game/Sacha/Interface/BPI_Interact.UpPain` (`self.BP_Pain`) 2.0)))))))))

(event `/Game/Sacha/Interface/BPI_Interact.PlaySound`
  (params (SoundToPlay :type "SoundBase Object Reference") (StartTime :type "Float (double-precision)"))
  (`AudioComponent.SetSound` (`self.Audio1`) SoundToPlay)
  (`AudioComponent.Play` (`self.Audio1`) 0.0))

(event `EventPNJDecendre`
  (bind (_returnvalue_x _returnvalue_y) (`KismetMathLibrary.BreakVector` (`self.K2_GetActorLocation`)))
  (bind (_returnvalue_x_2 _returnvalue_y_2 _returnvalue_z) (`KismetMathLibrary.BreakVector` (`self.K2_GetActorLocation`)))
  (if (== (`self.NumberofActivationDecente`) 0)
    (`/Game/Sacha/Winget/WB_SousTitre.EventSousTitrewinget` (`/Game/Sacha/Blueprint/BP_FirstPersonCharacterSacha.WingetSousTitre` (cast `/Game/Sacha/Blueprint/BP_FirstPersonCharacterSacha` (`GameplayStatics.GetPlayerCharacter` 0) :!pure true)) "Oh yeeaah! Do it harder")
    (`KismetSystemLibrary.Delay` 0.5))
  (`/Engine/EditorBlueprintResources/StandardMacros.IncrementInt` (`self.NumberofActivationDecente`)
    (:`  `
      (bind _output_get (set `self.PnjInitialLoc` _returnvalue_z))
      (set `self.PnjTargetlLoc` (- _output_get (`self.OffsetTargetLocation`)))
      ;[1 1 1] Event when cul desendre is activated
      (if (== (`self.NumberofActivationDecente`) (`self.NumberofActivationDecenteMax`))
        (set `self.PNJIsDown` true)
        (set `/Game/Sacha/Blueprint/Puzzle/PictoMove/BP_PictoMove.IsFinish` true (`self.BP_PictoMove`)))
      (for _array_element (`self.BPCordeMove`)
        (`/Game/Sacha/Blueprint/Cable/BP_CableMove.EventCordeMoving` _array_element (`self.CordeSpeed`)))
      (bind (_direction _newtrack_0) (`Timeline|TimelinePnjDencente` :!via `PlayFromStart`)
        (:`Update`
          (`self.K2_SetActorLocation` (`KismetMathLibrary.MakeVector` _returnvalue_x _returnvalue_y (`KismetMathLibrary.Lerp` (`self.PnjInitialLoc`) (`self.PnjTargetlLoc`) _newtrack_0))))
        (:`Finished`
          (for _array_element_2 (`self.BPCordeMove`)
            (`/Game/Sacha/Blueprint/Cable/BP_CableMove.EventCordeMoving` _array_element_2 0.0))
          (if (== (`self.NumberofActivationDecente`) (`self.NumberofActivationDecenteMax`))
            (message `/Game/Sacha/Interface/BPI_Interact.UpPain` (`self.BP_Pain`) 20.0)
            (else
              (`/Game/Sacha/Blueprint/Puzzle/PictoMove/BP_PictoMove.EventResetPuzzling` (`self.BP_PictoMove`))
              (message `/Game/Sacha/Interface/BPI_Interact.UpPain` (`self.BP_Pain`) 10.0))))))))

(event `EventPnjEcartelement`
  (`/Engine/EditorBlueprintResources/StandardMacros.IncrementInt` (`self.NumberofActivationEcartelement`)
    (:`  `
      (`GameplayStatics.SpawnSoundAtLocation` "/Game/Sounds/SFX/Homme_Baillon.Homme_Baillon" (0.0 0.0 0.0) (struct) 1.0 1.0 0.0 null null)
      (`GameplayStatics.SpawnSoundAtLocation` "/Game/Sounds/SFX/Chain_Cran.Chain_Cran" (0.0 0.0 0.0) (struct) 1.0 1.0 0.0 null null)
      (switch `int` (`self.NumberofActivationEcartelement`)
        (:`1`
          (for _array_element (`self.BPCordeMove`)
            (`/Game/Sacha/Blueprint/Cable/BP_CableMove.EventCordeMoving` _array_element (`self.CordeSpeed`)))
          (`|PlayMontage` (`self.SkeletalMesh`) "/Game/Kilian/Anims/HommeAttach/AN_Ecarteler.AN_Ecarteler"
            (:`OnCompleted`
              (for _array_element_2 (`self.BPCordeMove`)
                (`/Game/Sacha/Blueprint/Cable/BP_CableMove.EventCordeMoving` _array_element_2 0.0))
              (message `/Game/Sacha/Interface/BPI_Interact.PlaySound` (`self.Speaker`) "/Game/Sounds/Antagonist_Dialogue_Final/07_Yeah_thatsit.07_Yeah_thatsit" 0.0)
              (`/Game/Sacha/Winget/WB_SousTitre.EventSousTitrewinget` (`/Game/Sacha/Blueprint/BP_FirstPersonCharacterSacha.WingetSousTitre` (`self.PlayrRef`)) "Yeah... that's it... that's how you do it")
              (message `/Game/Sacha/Interface/BPI_Interact.UpPain` (`self.BP_Pain`) 5.0)
              (`/Game/Sacha/Blueprint/Puzzle/PictoMove/BP_PictoMove.EventResetPuzzling` (`self.BP_PictoMove`)))))
        (:`2`
          (for _array_element_3 (`self.BPCordeMove`)
            (`/Game/Sacha/Blueprint/Cable/BP_CableMove.EventCordeMoving` _array_element_3 (`self.CordeSpeed`)))
          (`|PlayMontage` (`self.SkeletalMesh`) "/Game/Kilian/Anims/HommeAttach/AN_Ecarteler.AN_Ecarteler"
            (:`OnCompleted`
              (for _array_element_4 (`self.BPCordeMove`)
                (`/Game/Sacha/Blueprint/Cable/BP_CableMove.EventCordeMoving` _array_element_4 0.0))
              (message `/Game/Sacha/Interface/BPI_Interact.PlaySound` (`self.Speaker`) "/Game/Sounds/Antagonist_Dialogue_Final/08_CarrefullNow.08_CarrefullNow" 0.0)
              (`/Game/Sacha/Winget/WB_SousTitre.EventSousTitrewinget` (`/Game/Sacha/Blueprint/BP_FirstPersonCharacterSacha.WingetSousTitre` (`self.PlayrRef`)) "Careful now darling... Don't be too greedy now...")
              (`/Game/Sacha/Blueprint/Puzzle/PictoMove/BP_PictoMove.EventResetPuzzling` (`self.BP_PictoMove`)))))
        (:`3`
          (`self.DisableInput` (`self.Playr Ref`) (`GameplayStatics.GetPlayerController` 0))
          (`SkeletalMeshComponent.SetAnimationMode` (`self.SkeletalMesh`) "AnimationBlueprint" false)
          (`SkeletalMeshComponent.PlayAnimation` (`self.SkeletalMesh`) "/Game/Kilian/Anims/HommeAttach/AN_EcartelerDead.AN_EcartelerDead" true)
          (`KismetSystemLibrary.Delay` 3.0)
          (set `self.IsEcarteler` true)
          (message `/Game/Sacha/Interface/BPI_Interact.PlaySound` (`self.Speaker`) "/Game/Sounds/Antagonist_Dialogue_Final/09_ITOLDYOU.09_ITOLDYOU" 0.0)
          (`/Game/Sacha/Winget/WB_SousTitre.EventSousTitrewinget` (`/Game/Sacha/Blueprint/BP_FirstPersonCharacterSacha.WingetSousTitre` (`self.PlayrRef`)) "I TOLD YOU TO BE CAREFUL! \nBLASPHEMY!")
          (message `/Game/Sacha/Interface/BPI_Interact.CallMonster` (`self.BPMonsterDoor`)))))))

(event `EventPnjFalling`
  (bind _bpcable (`self.BpCable`))
  (bind (_returnvalue_x _returnvalue_y _returnvalue_z) (`KismetMathLibrary.BreakVector` (`SceneComponent.K2_GetComponentLocation` (`self.SkeletalMesh`))))
  (set `CableComponent.CableLength` 250.0 (`/Game/Sacha/Blueprint/Cable/Bp_Cable.Cable` _bpcable))
  (set `CableComponent.CableLength` 250.0 (`/Game/Sacha/Blueprint/Cable/Bp_Cable.Cable1` _bpcable))
  (set `CableComponent.CableLength` 250.0 (`/Game/Sacha/Blueprint/Cable/Bp_Cable.Cable2` _bpcable))
  (set `CableComponent.CableLength` 250.0 (`/Game/Sacha/Blueprint/Cable/Bp_Cable.Cable3` _bpcable))
  (`self.DisableInput` (`self.Playr Ref`) (`GameplayStatics.GetPlayerController` 0))
  ;[1 1 1] Set simulate physics
  (`SceneComponent.K2_SetWorldLocation` (`self.SkeletalMesh`) (`KismetMathLibrary.MakeVector` _returnvalue_x _returnvalue_y (- _returnvalue_z 135.0)) false false)
  (`SkeletalMeshComponent.SetAnimationMode` (`self.SkeletalMesh`) "AnimationBlueprint" false)
  (`SkeletalMeshComponent.PlayAnimation` (`self.SkeletalMesh`) "/Game/Kilian/Anims/HommeAttach/Homme_X_PicsiDLE.Homme_X_PicsiDLE" true)
  (`KismetSystemLibrary.Delay` 3.0)
  (message `/Game/Sacha/Interface/BPI_Interact.PlaySound` (`self.Speaker`) "/Game/Sounds/Antagonist_Dialogue_Final/11_How_do_you_expect.11_How_do_you_expect" 0.0)
  (`/Game/Sacha/Winget/WB_SousTitre.EventSousTitrewinget` (`/Game/Sacha/Blueprint/BP_FirstPersonCharacterSacha.WingetSousTitre` (`self.PlayrRef`)) "How do you expect him to feel good now?!!")
  (message `/Game/Sacha/Interface/BPI_Interact.CallMonster` (`self.BPMonsterDoor`))
  (set `/Game/Sacha/Blueprint/Puzzle/PictoMove/BP_PictoMove.IsFinish` true (`self.BP_PictoMove`)))

(fn `UserConstructionScript`
  (`SceneComponent.K2_AttachToComponent` (`self.BallGag`) (`self.SkeletalMesh`) "BallSocket" "SnapToTarget" "SnapToTarget" "KeepRelative" true))