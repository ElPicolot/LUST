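; Bp_Cable is a cable rig Blueprint that ties an NPC's limbs to four cables, much like puppet strings.
; On BeginPlay, it attaches the end of each Cable component to the right foot, left foot, right hand or left hand component of the referenced PNJ1 character.
; The attachments use no socket, and the construction script is empty.
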(event `self.ReceiveBeginPlay`
  (bind _pnj1_ref (`self.PNJ1_Ref`))
  (`CableComponent.SetAttachEndToComponent` (`self.Cable`) (`/Game/Sacha/Blueprint/PNJ/BP_PNJ1.Pied_D` _pnj1_ref) "None")
  (`CableComponent.SetAttachEndToComponent` (`self.Cable1`) (`/Game/Sacha/Blueprint/PNJ/BP_PNJ1.Pied_G` _pnj1_ref) "None")
  (`CableComponent.SetAttachEndToComponent` (`self.Cable2`) (`/Game/Sacha/Blueprint/PNJ/BP_PNJ1.Main_D` _pnj1_ref) "None")
  (`CableComponent.SetAttachEndToComponent` (`self.Cable3`) (`/Game/Sacha/Blueprint/PNJ/BP_PNJ1.Main_G` _pnj1_ref) "None"))

(fn `UserConstructionScript`)