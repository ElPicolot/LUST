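; BP_Monster is a monster enemy that can be activated against the player and performs a melee attack.
; ActiveMonster sets the SeenPlayer key in its AI controller's Blackboard.
; AttackPlayer, gated by an attacking flag and a minimum max walk speed, starts an attack montage and immediately sphere-traces forward from AttackPoint to damage a hit pawn, with debug drawing enabled.
; The flag clears when the montage completes; CallMonster is an empty stub.
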(event `self.ReceiveBeginPlay`)

(event `self.ActiveMonster`
  (`BlackboardComponent.SetValueAsBool` (`AIBlueprintHelperLibrary.GetBlackboard` (`AIBlueprintHelperLibrary.GetAIController` self)) "SeenPlayer" true))

(event `AttackPlayer`
  (bind _attackpoint (`self.AttackPoint`))
  (bind _returnvalue (`SceneComponent.K2_GetComponentLocation` _attackpoint))
  (if (and (not (`self.IsAttacking`)) (> (`CharacterMovementComponent.MaxWalkSpeed` (`self.CharacterMovement`)) 150.0))
    (set `self.IsAttacking` true)
    (`|PlayMontage` (`self.Mesh`) "/Game/Sacha/Monster/annimation/Combo_Attack_04_01_Seq_Montage.Combo_Attack_04_01_Seq_Montage"
      (:`then`
        (bind (_outhit _returnvalue_2) (`KismetSystemLibrary.SphereTraceSingleForObjects` :`Start` _returnvalue :`End` (+ _returnvalue (* (`SceneComponent.GetForwardVector` _attackpoint) 100.0)) :`Radius` 30.0 :`ObjectTypes` (`|MakeArray` "ObjectTypeQuery3" :!type "EObjectTypeQuery Enum") :`DrawDebugType` "ForDuration"))
        (if _returnvalue_2
          (`GameplayStatics.ApplyDamage` (`.HitActor` (`GameplayStatics.BreakHitResult` _outhit)) 10.0)))
      (:`OnCompleted`
        (set `self.IsAttacking` false)))))

(fn `CallMonster`
  (return))

(fn `UserConstructionScript`)