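; Camera actor, named for the antagonist, that takes over player 0's view as soon as it begins play.
; BeginPlay sets it as the view target, then casts the player character to BP_FirstPersonCharacterSacha.
; Its root snaps once to the first point of that character's spline, using the first-person camera's world rotation, with no per-frame update.
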(event `self.ReceiveBeginPlay`
  (`PlayerController.SetViewTargetWithBlend` (`GameplayStatics.GetPlayerController` 0) self 0.0 "VTBlend_Linear" 0.0 false)
  (bind _asbp_first_person_character_sacha (cast `/Game/Sacha/Blueprint/BP_FirstPersonCharacterSacha` (`GameplayStatics.GetPlayerCharacter` 0)))
  (`SceneComponent.K2_SetWorldLocationAndRotation` (`self.DefaultSceneRoot`) (`SplineComponent.GetLocationAtSplinePoint` (`/Game/Sacha/Blueprint/BP_FirstPersonCharacterSacha.Spline` _asbp_first_person_character_sacha) 0 "World") (`SceneComponent.K2_GetComponentRotation` (`/Game/Sacha/Blueprint/BP_FirstPersonCharacterSacha.FirstPersonCamera` _asbp_first_person_character_sacha)) false false))

(fn `UserConstructionScript`)