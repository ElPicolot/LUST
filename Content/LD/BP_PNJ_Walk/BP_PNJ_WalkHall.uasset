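; BP_PNJ_WalkHall is an NPC that walks once along a spline when BP_FirstPersonCharacterSacha overlaps its trigger box.
; A Timeline, with play rate inversely scaled by TimePlayRate, drives a Lerp over spline distance to position the skeletal mesh.
; Mesh rotation comes from a look-at between the spline's local forward vector and the mesh's current forward vector.
; The actor destroys itself when the Timeline finishes.
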(event `Play_spline`
  (`TimelineComponent.SetPlayRate` (`self.Timeline`) (/ 0.7 (`self.Time/PlayRate`)))
  (`self.Follow Spline`))

(event `Follow Spline`
  (bind _spline (`self.Spline`))
  (bind (_direction _newtrack_0) (`Timeline|Timeline`)
    (:`Update`
      (bind _returnvalue (`KismetMathLibrary.Lerp` 0.0 (`SplineComponent.GetDistanceAlongSplineAtSplinePoint` _spline (- (`SplineComponent.GetNumberOfSplinePoints` _spline) 1)) _newtrack_0))
      (`SceneComponent.K2_SetWorldLocationAndRotation` (`self.SkeletalMesh`) (`SplineComponent.GetLocationAtDistanceAlongSpline` _spline _returnvalue "World") (`KismetMathLibrary.FindLookAtRotation` (`KismetMathLibrary.Conv_RotatorToVector` (`SplineComponent.GetRotationAtDistanceAlongSpline` (`self.Spline`) _returnvalue "Local")) (`KismetMathLibrary.Conv_RotatorToVector` (`SceneComponent.K2_GetComponentRotation` (`self.SkeletalMesh`)))) false false))
    (:`Finished`
      (`self.K2_DestroyActor`))))

(event `self.Box.OnComponentBeginOverlap`
  (params (OverlappedComponent :type "PrimitiveComponent Object Reference") (OtherActor :type "Actor Object Reference") (OtherComp :type "PrimitiveComponent Object Reference") (OtherBodyIndex :type Integer) (bFromSweep :type Boolean) (SweepResult :type "HitResult Structure (by ref)"))
  (cast `/Game/Sacha/Blueprint/BP_FirstPersonCharacterSacha` OtherActor)
  (`self.Play_spline`))

(fn `UserConstructionScript`)