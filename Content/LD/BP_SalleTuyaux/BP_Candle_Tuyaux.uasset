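; Interactable candle for the pipe room that the player lights, once only, with a held lighter.
; A valid interaction disables input, then a timeline moves the lighter from its initial transform to a target point, where it plays a lighting montage.
; Montage notifies toggle the lighter's Niagara flame and switch on the candle's fire, light and sound.
; On completion the same timeline reverses to return the lighter, then input is restored.
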(event `self.ReceiveBeginPlay`
  (`parent.ReceiveBeginPlay`)
  (`ActorComponent.SetActive` (`self.Fire`) false false)
  (`TimelineComponent.SetPlayRate` (`self.GoToCandle`) 1.0))

(event `ReverseMovement`
  (bind _niagaradefault (`/Game/Sacha/Blueprint/Items/BP_Item.NiagaraDefault` (`self.ItemInHandRef`)))
  (bind (_direction _newtrack_0) (`Timeline|GoToCandle` :!via `Reverse` :!label _label)
    (:`Update`
      (`SceneComponent.K2_SetWorldTransform` (`Actor.RootComponent` (`self.ItemInHandRef`)) (`KismetMathLibrary.TLerp` (`self.InitialTrandform`) (`SceneComponent.K2_GetComponentToWorld` (`self.BriquetTarget`)) _newtrack_0) false false))
    (:`Finished`
      (if (`self.reverse`)
        (`self.EnableInput` (`self.Playr Ref`) (`GameplayStatics.GetPlayerController` 0))
        (else
          (set `self.reverse` true)
          (bind _notifyname (`|PlayMontage` (`/Game/Sacha/Blueprint/Items/BP_Item.SkeletalMesh` (`self.ItemInHandRef`)) "/Game/Kilian/Anims/Briquet/AM_AllumeCandle.AM_AllumeCandle")
            (:`OnCompleted`
              (`self.ReverseMovement`))
            (:`OnNotifyBegin`
              (switch `name` _notifyname
                (:`Flamme`
                  (`/Engine/EditorBlueprintResources/StandardMacros.FlipFlop`
                    (:`A`
                      (`ActorComponent.SetActive` _niagaradefault true false))
                    (:`B`
                      (`ActorComponent.SetActive` _niagaradefault false false))))
                (:`CandleOn`
                  ;[1 1 1] Son Ok briquet + delay flamme
                  (`self.SetAndPlaySound` (`self.SoundToPlay2`) (`self.Audio1`))
                  (`ActorComponent.SetActive` (`self.Fire`) true false)
                  (`ActorComponent.SetActive` (`self.Fire`) true false)
                  (`SceneComponent.SetVisibility` (`self.PointLight`) true false))))))))))

(event `self.Interact Working`
  (params (ItemInHand :type "/Game/Sacha/Blueprint/Items/E_MainItemType Enum" :default "NewEnumerator0") (ItemInHandforAnim :type "/Game/Sacha/Blueprint/Items/BP_Item Object Reference") (PlayrRef :type "/Game/Sacha/Blueprint/BP_FirstPersonCharacterSacha Object Reference"))
  (set `self.ItemInHandRef` ItemInHandforAnim)
  (if (`|EnumEquality` ItemInHand "NewEnumerator2")
    (`/Engine/EditorBlueprintResources/StandardMacros.DoOnce` false
      (:`Completed`
        (bind _output_get (set `self.Playr Ref` PlayrRef))
        (`self.DisableInput` _output_get (`GameplayStatics.GetPlayerController` 0))
        (set `self.InitialTrandform` (`SceneComponent.K2_GetComponentToWorld` (`Actor.RootComponent` (`self.ItemInHandRef`))))
        (goto _label :!via `PlayFromStart`)))))

(fn `UserConstructionScript`
  (`parent.UserConstructionScript`))